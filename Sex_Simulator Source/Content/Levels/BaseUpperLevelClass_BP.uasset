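; Base actor that pairs a named level with a UI widget through load, hide and unload functions.
; Load binds loaded events via the LLC manager and level object, loads with optional loading screen, opens the widget, then removes the manager binding.
; Hide closes the widget and Unload also destroys the actor; their LLC hide/unload calls are disconnected, leaving the level untouched.
; OnLevelLoaded and the standard events are empty.
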(event EventBeginPlay)

(event Collision|EventActorBeginOverlap
  (params (OtherActor :type Actor%20Object%20Reference)))

(event EventTick
  (params (DeltaSeconds :type Float%20%28single-precision%29)))

(fn ConstructionScript
  (Rendering|SetVisibility (Variables|Default|GetDefaultSceneRoot) false false))

(fn ULCLoad
  (bind _issuccess (CallFunction|SetonLevelLoadedDelegate))
  (if _issuccess
    (bind (_success _levelobject) (CallFunction|LoadLLC (Variables|Default|GetLevelName) true (Variables|Default|GetIsSetLoadingScreenWhileLoading) (Variables|Default|GetLoadingScreenZOrder) (Variables|Default|GetKeepLoadingScreenAfterLevelIsLoaded)))
    (if _success
      (EventDispatchers|BindEventtoOnLevelLoaded _levelobject (EventDispatchers|CreateEvent :!event OnLevelLoaded))
      (bind _widget_reference (CallFunction|OpenWidget (Variables|Default|GetWidget) true (Variables|Default|GetWidgetZOrder)))
      (CallFunction|RemoveonLevelLoadedDelegate)
      (return self _levelobject _widget_reference))))

(fn ULCUnload
  (CallFunction|CloseWidget (Variables|Default|GetWidget))
  (Actor|DestroyActor))

(fn ULCHide
  (CallFunction|CloseWidget (Variables|Default|GetWidget)))

(fn OnLevelLoaded)

(fn SetonLevelLoadedDelegate
  (bind (_isfound _levelmanager) (CallFunction|GetLLCManager))
  (if _isfound
    (EventDispatchers|BindEventtoLLCMonLevelLoadedandVisibleDelegate _levelmanager (EventDispatchers|CreateEvent :!event OnLevelLoaded)))
  (return _isfound))

(fn RemoveonLevelLoadedDelegate
  (bind (_isfound _levelmanager) (CallFunction|GetLLCManager))
  (if _isfound
    (EventDispatchers|UnbindEventfromLLCMonLevelLoadedandVisibleDelegate _levelmanager (EventDispatchers|CreateEvent :!event OnLevelLoaded)))
  (return _isfound))