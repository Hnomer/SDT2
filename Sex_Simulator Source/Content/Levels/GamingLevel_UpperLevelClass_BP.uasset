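; Upper-level class for the gaming level, managing its character selection, pause and in-game HUD menus.
; On load it opens character selection, then applies the chosen save's morphs and body-part colors before showing the HUD.
; Tab, I and Escape toggle alterations, info and pause panels, using visibility flags to coordinate menus, cursor and input mode.
; Hide and unload close the widgets and reset Object Manager actors.
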(event EventBeginPlay
  (|CallParentFunction)
  (CallFunction|EGPlayerControllerBeginPlay)
  (CallFunction|EGUIBeginPlay))

(event Collision|EventActorBeginOverlap
  (params (OtherActor :type Actor%20Object%20Reference))
  (|CallParentFunction OtherActor) ; This node is disabled and will not be called.\nDrag off pins to build functionality.
)

(event EventOnLevelLoaded
  (CallFunction|EGPlayerControlleronLevelLoaded)
  (CallFunction|EGUIonLevelLoaded))

(event EventTick
  (params (DeltaSeconds :type Float%20%28single-precision%29))
  (|CallParentFunction DeltaSeconds) ; This node is disabled and will not be called.\nDrag off pins to build functionality.
)

(event EventULCHide
  (CallFunction|CloseWidget "/Game/Blueprints/HUD/InGameHUD/CharacterSelectionWidget_BP.CharacterSelectionWidget_BP_C")
  (CallFunction|CloseWidget "/Game/Blueprints/HUD/InGameHUD/PauseWidget_BP.PauseWidget_BP_C")
  (CallFunction|CloseWidget "/Game/Blueprints/HUD/InGameHUD/InGameHUD.InGameHUD_C")
  (Input|DisableInput (Game|GetPlayerController 0))
  (bind (_isfound _objectmanager) (CallFunction|GetObjectManager))
  (if _isfound
    (Default|OMResetActors _objectmanager))
  (|CallParentFunction)
  (Actor|DestroyActor))

(event EventULCUnload
  (CallFunction|CloseWidget "/Game/Blueprints/HUD/InGameHUD/CharacterSelectionWidget_BP.CharacterSelectionWidget_BP_C")
  (CallFunction|CloseWidget "/Game/Blueprints/HUD/InGameHUD/InGameHUD.InGameHUD_C")
  (CallFunction|CloseWidget "/Game/Blueprints/HUD/InGameHUD/PauseWidget_BP.PauseWidget_BP_C")
  (bind (_isfound _objectmanager) (CallFunction|GetObjectManager))
  (if _isfound
    (Default|OMResetActors _objectmanager)
    (|CallParentFunction)))

(event Custom|EG_PlayerController_BeginPlay)

(event Custom|EG_PlayerController_OnLevelLoaded
  (Input|EnableInput (Game|GetPlayerController 0)))

(event Input|KeyboardEvents|I
  (params (Key :type Key%20Structure))
  (:Pressed
    (UI|ToggleinGameInfo false false)))

(event Input|KeyboardEvents|Tab
  (params (Key :type Key%20Structure))
  (:Pressed
    (UI|ToggleinGameAlternationsMenu false false)))

(event Input|KeyboardEvents|Escape
  (params (Key :type Key%20Structure))
  (:Pressed
    (if (Variables|UI|GetIsSittingsMenuOpen)
      (CallFunction|CloseWidget "/Game/Blueprints/HUD/Settings/Settings_Widget.Settings_Widget_C")
      (UI|OnCloseSettings)
      (else
        (UI|TogglePauseMenu)))))

(event Custom|EG_UI_OnLevelLoaded
  (UI|OpenCharacterSelectionMenu))

(event Custom|EG_UI_BeginPlay)

(fn ConstructionScript
  (|CallParentFunction))

(fn OpenCharacterSelectionMenu
  (if (Variables|UI|GetIsPauseMenuVisible)
    (UI|TogglePauseMenu)
    (if (Variables|UI|GetIsInGameAlternationsMenuVisible)
      (UI|ToggleinGameAlternationsMenu false true)))
  (Variables|UI|SetIsCharacterSelectionMenuVisible true)
  (bind _widget_reference (CallFunction|OpenWidget "/Game/Blueprints/HUD/InGameHUD/CharacterSelectionWidget_BP.CharacterSelectionWidget_BP_C" true 2))
  (bind _ascharacter_selection_widget_bp (Utilities|Casting|CastToCharacterSelectionWidget_BP _widget_reference))
  (EventDispatchers|BindEventtoCharacterSelectionWidgetonRequestLoadDelegate _ascharacter_selection_widget_bp (EventDispatchers|CreateEvent :!event OnRequestLoad))
  (CallFunction|SetCursorVisibility true)
  (CallFunction|SetInputMode true false false _widget_reference "DoNotLock" false))

(fn OnRequestLoad
  (params (SaveName :type Name))
  (bind (_issuccess _save_object) (CallFunction|GetSave "NewEnumerator0" false SaveName))
  (if _issuccess
    (bind _assamka_character_save_class_bp (Utilities|Casting|CastToSamkaCharacterSaveClass_BP _save_object))
    (bind (_savename _saveversion _savedate _authorname _modifiedbyname _characterthumbnail _morphitemstruct_array _bodypartscolorsstruct) (Default|GetSaveData _assamka_character_save_class_bp))
    (bind _issuccess_2 (CallFunction|SetSamkaMorphs!GamingLevelOnly! _morphitemstruct_array))
    (bind _issuccess_3 (CallFunction|SetSamkaBodyPartsColors!GamingLevelOnly! _bodypartscolorsstruct))
    (if (and _issuccess_3 _issuccess_2)
      (CallFunction|CloseWidget "/Game/Blueprints/HUD/InGameHUD/CharacterSelectionWidget_BP.CharacterSelectionWidget_BP_C")
      (CallFunction|SetInputMode false true false 0 "DoNotLock" false)
      (Variables|UI|SetIsCharacterSelectionMenuVisible false)
      (CallFunction|SetCursorVisibility false)
      (CallFunction|OpenWidget "/Game/Blueprints/HUD/InGameHUD/InGameHUD.InGameHUD_C" true))))

(fn TogglePauseMenu
  (if (not (Variables|UI|GetIsCharacterSelectionMenuVisible))
    (if (Variables|UI|GetIsInGameAlternationsMenuVisible)
      (UI|ToggleinGameAlternationsMenu false true))
    (if (Variables|UI|GetIsInGameInfoMenuVisible)
      (UI|ToggleinGameInfo false false))
    (bind _output_get (Variables|UI|SetIsPauseMenuVisible (not (Variables|UI|GetIsPauseMenuVisible))))
    (if _output_get
      (bind _widget_reference (CallFunction|OpenWidget "/Game/Blueprints/HUD/InGameHUD/PauseWidget_BP.PauseWidget_BP_C" true 1))
      (bind _aspause_widget_bp (Utilities|Casting|CastToPauseWidget_BP _widget_reference))
      (EventDispatchers|BindEventtoPauseWidgetonCloseWidgetDelegate _aspause_widget_bp (EventDispatchers|CreateEvent :!event TogglePauseMenu))
      (EventDispatchers|BindEventtoPauseWidgetonSelectCharacterDelegate _aspause_widget_bp (EventDispatchers|CreateEvent :!event OpenCharacterSelectionMenu))
      (EventDispatchers|BindEventtoPauseWidgetonOpenSettingsDelegate _aspause_widget_bp (EventDispatchers|CreateEvent :!event OnOpenSettings))
      (EventDispatchers|BindEventtoPauseWidgetonCloseSettingsDelegate _aspause_widget_bp (EventDispatchers|CreateEvent :!event OnCloseSettings))
      (CallFunction|SetInputMode true false false _widget_reference "DoNotLock" false)
      (CallFunction|SetCursorVisibility true)
      (else
        (CallFunction|CloseWidget "/Game/Blueprints/HUD/InGameHUD/PauseWidget_BP.PauseWidget_BP_C")
        (CallFunction|SetInputMode false true false 0 "DoNotLock" false)
        (CallFunction|SetCursorVisibility false)))))

(fn ToggleinGameAlternationsMenu
  (params (ForceShow :type Boolean) (ForceHide :type Boolean))
  (bind _widgetobject (CallFunction|GetWidget "/Game/Blueprints/HUD/InGameHUD/InGameHUD.InGameHUD_C"))
  (bind _asin_game_hud (Utilities|Casting|CastToInGameHUD _widgetobject))
  (if ForceShow
    (CallFunction|SetCursorVisibility true :!label _label)
    (CallFunction|SetInputMode true false false 0 "DoNotLock" false)
    (Variables|UI|SetIsInGameAlternationsMenuVisible true)
    (Default|SetShowinGameAlternationsCanvas _asin_game_hud true false 1.0)
    (elif ForceHide
      (CallFunction|SetCursorVisibility false :!label _label_2)
      (CallFunction|SetInputMode false true false 0 "DoNotLock" false)
      (Variables|UI|SetIsInGameAlternationsMenuVisible false)
      (Default|SetShowinGameAlternationsCanvas _asin_game_hud false false 1.0)
      (elif (not (or (Variables|UI|GetIsCharacterSelectionMenuVisible) (Variables|UI|GetIsPauseMenuVisible)))
        (if (not (Variables|UI|GetIsInGameAlternationsMenuVisible))
          (goto _label)
          (else
            (goto _label_2)))))))

(fn ToggleinGameInfo
  (params (ForceShow :type Boolean) (ForceHide :type Boolean))
  (bind _widgetobject (CallFunction|GetWidget "/Game/Blueprints/HUD/InGameHUD/InGameHUD.InGameHUD_C"))
  (bind _asin_game_hud (Utilities|Casting|CastToInGameHUD _widgetobject))
  (if ForceShow
    (Variables|UI|SetIsInGameInfoMenuVisible true :!label _label)
    (Default|SetShowinGameInfoCanvas _asin_game_hud true 1.0)
    (elif ForceHide
      (Variables|UI|SetIsInGameInfoMenuVisible false :!label _label_2)
      (Default|SetShowinGameInfoCanvas _asin_game_hud false 1.0)
      (elif (not (or (Variables|UI|GetIsCharacterSelectionMenuVisible) (Variables|UI|GetIsPauseMenuVisible)))
        (if (not (Variables|UI|GetIsInGameInfoMenuVisible))
          (goto _label)
          (else
            (goto _label_2)))))))

(fn OnOpenSettings
  (Variables|UI|SetIsSittingsMenuOpen true))

(fn OnCloseSettings
  (Variables|UI|SetIsSittingsMenuOpen false))