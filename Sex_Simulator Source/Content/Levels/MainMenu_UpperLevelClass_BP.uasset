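; Main menu upper-level class that handles input and loading-screen state, and dresses the Samka character from a random save.
; On level load it enables input in UI-only mode, then hides the loading screen after a short delay.
; A one-time step then picks a random non-built-in character save, if any exist, and applies its morphs and body-part colors.
; Unloading or hiding the level disables player input.
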(event EventBeginPlay
  (|CallParentFunction) ; This node is disabled and will not be called.\nDrag off pins to build functionality.
)

(event Collision|EventActorBeginOverlap
  (params (OtherActor :type Actor%20Object%20Reference))
  (|CallParentFunction OtherActor) ; This node is disabled and will not be called.\nDrag off pins to build functionality.
)

(event EventOnLevelLoaded
  (|CallParentFunction)
  (Input|EnableInput (Game|GetPlayerController 0))
  (CallFunction|SetInputMode false false true 0 "DoNotLock" false)
  (Utilities|FlowControl|Delay 2.0)
  (CallFunction|SetLoadingScreenEnabled false false)
  (Utilities|FlowControl|DoOnce false
    (:Completed
      (bind _save_objects_array (CallFunction|GetAllSaves "NewEnumerator0" false false))
      (if (> (Utilities|Array|Length _save_objects_array) 0)
        (bind _assamka_character_save_class_bp (Utilities|Casting|CastToSamkaCharacterSaveClass_BP (Utilities|Array|Get(acopy) _save_objects_array (Math|Random|RandomIntegerinRange 0 (- (Utilities|Array|Length _save_objects_array) 1)))))
        (bind (_savename _saveversion _savedate _authorname _modifiedbyname _characterthumbnail _morphitemstruct_array _bodypartscolorsstruct) (Default|GetSaveData _assamka_character_save_class_bp))
        (CallFunction|SetSamkaMorphs!GamingLevelOnly! _morphitemstruct_array)
        (CallFunction|SetSamkaBodyPartsColors!GamingLevelOnly! _bodypartscolorsstruct)))))

(event EventTick
  (params (DeltaSeconds :type Float%20%28single-precision%29))
  (|CallParentFunction DeltaSeconds) ; This node is disabled and will not be called.\nDrag off pins to build functionality.
)

(event EventULCUnload
  (Input|DisableInput (Game|GetPlayerController 0))
  (|CallParentFunction))

(event EventULCHide
  (Input|DisableInput (Game|GetPlayerController 0))
  (|CallParentFunction))

(fn ConstructionScript
  (|CallParentFunction))