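; Upper-level class that runs the character customization level: save/load menu, editing and return to the main menu.
; After polling for the CustomizationManager, it routes widget events, body-part clicks and right-mouse drag into morph, color, camera and rotation changes on the character.
; It creates, loads, renames and deletes character saves with thumbnails, confirming overwrites, deletions and unsaved changes.
; Loading reconciles saved morphs with the current list, offering force or soft fixes on mismatch.
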(event EventTick
  (params (DeltaSeconds :type Float%20%28single-precision%29))
  (|CallParentFunction DeltaSeconds))

(event EventOnLevelLoaded
  (CallFunction|SetLoadingScreenEnabled true false 100)
  (bind _isinitcomplete (CallFunction|Init :!label _label))
  (if _isinitcomplete
    (CallFunction|EGUIonLevelLoaded)
    (UI|SetBackButton false)
    (CallFunction|OpenWidget "/Game/Blueprints/HUD/Customization/CustomizationWidget_BP.CustomizationWidget_BP_C" false 1)
    (CallFunction|SetLoadingScreenEnabled false false 10)
    (else
      (Utilities|FlowControl|Delay 0.2)
      (goto _label))))

(event EventULCUnload
  (CallFunction|CloseWidget "/Game/Blueprints/HUD/Customization/SaveLoadCustomizationWidget_BP.SaveLoadCustomizationWidget_BP_C")
  (CallFunction|CloseWidget "/Game/Blueprints/HUD/Customization/CustomizationWidget_BP.CustomizationWidget_BP_C")
  (Input|DisableInput (Game|GetPlayerController 0))
  (|CallParentFunction))

(event EventULCHide
  (CallFunction|CloseWidget "/Game/Blueprints/HUD/Customization/SaveLoadCustomizationWidget_BP.SaveLoadCustomizationWidget_BP_C")
  (CallFunction|CloseWidget "/Game/Blueprints/HUD/Customization/CustomizationWidget_BP.CustomizationWidget_BP_C")
  (Input|DisableInput (Game|GetPlayerController 0))
  (|CallParentFunction))

(event Custom|EG_UI_OnLevelLoaded
  (UI|OpenCharacterSelectionMenu))

(event Input|MouseEvents|MouseX
  (params (AxisValue :type Float%20%28single-precision%29))
  (bind _customizationmanager (Variables|Default|GetCustomizationManager))
  (bind _samkacustomizationactor (Variables|/Game/Blueprints/Managers/CustomizationManager_BP.CustomizationManager_BP_C|GetSamkaCustomizationActor _customizationmanager))
  (if (and (Variables|Controls|GetIsRMBPressed) (Variables|Customizing|GetIsInCustomizationEnvironment))
    (Default|RotateSamka _samkacustomizationactor (* AxisValue -1.0))
    (else
      (Default|RotateSamka _samkacustomizationactor 0.0))))

(event Input|MouseEvents|MouseY
  (params (AxisValue :type Float%20%28single-precision%29))
  (bind _customizationmanager (Variables|Default|GetCustomizationManager))
  (bind _samkacustomizationactor (Variables|/Game/Blueprints/Managers/CustomizationManager_BP.CustomizationManager_BP_C|GetSamkaCustomizationActor _customizationmanager))
  (if (and (Variables|Controls|GetIsRMBPressed) (Variables|Customizing|GetIsInCustomizationEnvironment))
    (Default|HeadUpDown _samkacustomizationactor (* AxisValue -1.0) false)
    (else
      (Default|HeadUpDown _samkacustomizationactor 0.0 true))))

(event Input|KeyboardEvents|CtrlS
  (params (Key :type Key%20Structure))
  (:Pressed
    (if (Variables|Customizing|GetIsInCustomizationEnvironment)
      (Save/LoadFunctions|SaveProgress))))

(event Input|MouseEvents|RightMouseButton
  (params (Key :type Key%20Structure))
  (:Pressed
    (Variables|Controls|SetIsRMBPressed true))
  (:Released
    (Variables|Controls|SetIsRMBPressed false)))

(fn ConstructionScript
  (|CallParentFunction))

(fn OpenCharacterSelectionMenu
  (bind _widget_reference (CallFunction|OpenWidget "/Game/Blueprints/HUD/Customization/SaveLoadCustomizationWidget_BP.SaveLoadCustomizationWidget_BP_C" true 1))
  (bind _assave_load_customization_widget_bp (Utilities|Casting|CastToSaveLoadCustomizationWidget_BP _widget_reference))
  (Utilities|FlowControl|Sequence
    (:then_0
      (EventDispatchers|BindEventtoOnRequestCloseWidgetSaveLoadCustomizationWidgetDelegate _assave_load_customization_widget_bp (EventDispatchers|CreateEvent :!event OnCloseCharacterSelectionMenuDelegate)))
    (:then_1
      (EventDispatchers|BindEventtoOnRequestLoadSaveSaveLoadCustomizationWidgetDelegate _assave_load_customization_widget_bp (EventDispatchers|CreateEvent :!event OnLoadCharacterDelegate)))
    (:then_2
      (EventDispatchers|BindEventtoOnRequestNewSaveSaveLoadCustomizationWidgetDelegate _assave_load_customization_widget_bp (EventDispatchers|CreateEvent :!event OnNewSaveDelegate)))
    (:then_3
      (EventDispatchers|BindEventtoOnRequestRenameSaveSaveLoadCustomizationWidgetDelegate _assave_load_customization_widget_bp (EventDispatchers|CreateEvent :!event OnRenameSaveDelegate)))
    (:then_4
      (EventDispatchers|BindEventtoOnRequestQuitSaveLoadCustomizationWidgetDelegate _assave_load_customization_widget_bp (EventDispatchers|CreateEvent :!event OnQuitDelegate)))
    (:then_5
      (EventDispatchers|BindEventtoOnRequestDeleteSaveSaveLoadCustomizationWidgetDelegate _assave_load_customization_widget_bp (EventDispatchers|CreateEvent :!event OnDeleteSaveDelegate)))))

(fn OnCloseCharacterSelectionMenuDelegate
  (CallFunction|CloseWidget "/Game/Blueprints/HUD/Customization/SaveLoadCustomizationWidget_BP.SaveLoadCustomizationWidget_BP_C"))

(fn OnLoadCharacterDelegate
  (params (SaveName :type Name))
  (bind _output_get (Variables|Default|SetPendingSaveFileName_BUFFER SaveName))
  (if (Variables|Customizing|GetIsProgressSaved)
    (bind _assamka_character_save_class_bp (Save/LoadFunctions|GetSavefromFile _output_get))
    (Save/LoadFunctions|LoadSave _assamka_character_save_class_bp true false)
    (else
      (bind _widget_reference (CallFunction|OpenWidget "/Game/Blueprints/HUD/Customization/AreYouSureWdiget_BP.AreYouSureWdiget_BP_C" false 10))
      (bind _asare_you_sure_wdiget_bp (Utilities|Casting|CastToAreYouSureWdiget_BP _widget_reference))
      (Default|SetandShowAreYouSure _asare_you_sure_wdiget_bp (Utilities|Text|MakeLiteralText "You progress isn't saved! Do you want to save it before loading?") 10)
      (Utilities|FlowControl|Sequence
        (:then_0
          (EventDispatchers|BindEventtoOnYesAreYouSureWidget _asare_you_sure_wdiget_bp (EventDispatchers|CreateEvent :!event OnLoadSaveAskProgressIsNotSavedYes)))
        (:then_1
          (EventDispatchers|BindEventtoOnNoAreYouSureWidget _asare_you_sure_wdiget_bp (EventDispatchers|CreateEvent :!event OnLoadSaveAskProgressIsNotSavedNo)))
        (:then_2
          (EventDispatchers|BindEventtoOnCancelAreYouSureWidget _asare_you_sure_wdiget_bp (EventDispatchers|CreateEvent :!event OnLoadSaveAskProgressIsNotSavedCancel)))))))

(fn OnNewSaveDelegate
  (params (SaveName :type Name))
  (Variables|Default|SetPendingSaveFileName_BUFFER SaveName)
  (bind _isexists (CallFunction|IsSaveExists "NewEnumerator0" SaveName))
  (if _isexists
    (bind _widget_reference (CallFunction|OpenWidget "/Game/Blueprints/HUD/Customization/AreYouSureWdiget_BP.AreYouSureWdiget_BP_C" false 10))
    (bind _asare_you_sure_wdiget_bp (Utilities|Casting|CastToAreYouSureWdiget_BP _widget_reference))
    (Default|SetandShowAreYouSure _asare_you_sure_wdiget_bp (Utilities|Text|ToText(String) (Utilities|String|Append "The save with this name: \"" (Utilities|String|ToString(Name) SaveName) "\" already exists. " "Do you want to override it?")) 10)
    (Utilities|FlowControl|Sequence
      (:then_0
        (EventDispatchers|BindEventtoOnYesAreYouSureWidget _asare_you_sure_wdiget_bp (EventDispatchers|CreateEvent :!event OnNewSaveAskOverrideSaveYesDelegate)))
      (:then_1
        (EventDispatchers|BindEventtoOnNoAreYouSureWidget _asare_you_sure_wdiget_bp (EventDispatchers|CreateEvent :!event OnNewSaveAskOverrideSaveNoDelegate)))
      (:then_2
        (EventDispatchers|BindEventtoOnCancelAreYouSureWidget _asare_you_sure_wdiget_bp (EventDispatchers|CreateEvent :!event OnNewSaveAskOverrideSaveCancelDelegate))))
    (else
      (Save/LoadFunctions|CreateNewSave SaveName))))

(fn OnRenameSaveDelegate
  (params (SaveName :type Name) (NewSaveName :type Name))
  (Save/LoadFunctions|RenameSave SaveName NewSaveName))

(fn OnQuitDelegate
  (CallFunction|Quit false))

(fn OnDeleteSaveDelegate
  (params (SaveName :type Name))
  (Variables|Default|SetPendingSaveFileName_BUFFER SaveName)
  (bind _widget_reference (CallFunction|OpenWidget "/Game/Blueprints/HUD/Customization/AreYouSureWdiget_BP.AreYouSureWdiget_BP_C" false 10))
  (bind _asare_you_sure_wdiget_bp (Utilities|Casting|CastToAreYouSureWdiget_BP _widget_reference))
  (Default|SetandShowAreYouSure _asare_you_sure_wdiget_bp (Utilities|Text|ToText(String) (Utilities|String|Append "Are you sure you want to delete the save: \"" (Utilities|String|ToString(Name) SaveName) "\" ?")) 10)
  (Utilities|FlowControl|Sequence
    (:then_0
      (EventDispatchers|BindEventtoOnYesAreYouSureWidget _asare_you_sure_wdiget_bp (EventDispatchers|CreateEvent :!event OnDeleteSaveAskDeleteSaveYes)))
    (:then_1
      (EventDispatchers|BindEventtoOnNoAreYouSureWidget _asare_you_sure_wdiget_bp (EventDispatchers|CreateEvent :!event OnDeleteSaveAskDeleteSaveNo)))
    (:then_2
      (EventDispatchers|BindEventtoOnCancelAreYouSureWidget _asare_you_sure_wdiget_bp (EventDispatchers|CreateEvent :!event OnDeleteSaveAskDeleteSaveCancel)))))

(fn OnNewSaveAskOverrideSaveYesDelegate
  (UIAreYouSureWidget|UnbindAllfromAreYouSureWidget)
  (if (Variables|Customizing|GetIsProgressSaved)
    (Save/LoadFunctions|CreateNewSave (Variables|Default|GetPendingSaveFileName_BUFFER))
    (CallFunction|CloseWidget "/Game/Blueprints/HUD/Customization/AreYouSureWdiget_BP.AreYouSureWdiget_BP_C")
    (else
      (bind _widget_reference (CallFunction|OpenWidget "/Game/Blueprints/HUD/Customization/AreYouSureWdiget_BP.AreYouSureWdiget_BP_C" false))
      (bind _asare_you_sure_wdiget_bp (Utilities|Casting|CastToAreYouSureWdiget_BP _widget_reference))
      (Default|SetandShowAreYouSure _asare_you_sure_wdiget_bp (Utilities|Text|MakeLiteralText "You progress isn't saved! Do you want to save it?") 10)
      (Utilities|FlowControl|Sequence
        (:then_0
          (EventDispatchers|BindEventtoOnYesAreYouSureWidget _asare_you_sure_wdiget_bp (EventDispatchers|CreateEvent :!event OnNewSaveAskProgressIsNotSavedYesDelegate)))
        (:then_1
          (EventDispatchers|BindEventtoOnNoAreYouSureWidget _asare_you_sure_wdiget_bp (EventDispatchers|CreateEvent :!event OnNewSaveAskProgressIsNotSavedNoDelegate)))
        (:then_2
          (EventDispatchers|BindEventtoOnCancelAreYouSureWidget _asare_you_sure_wdiget_bp (EventDispatchers|CreateEvent :!event OnNewSaveAskProgressIsNotSavedCancelDelegate)))))))

(fn OnNewSaveAskOverrideSaveNoDelegate
  (UIAreYouSureWidget|UnbindAllfromAreYouSureWidget)
  (CallFunction|CloseWidget "/Game/Blueprints/HUD/Customization/AreYouSureWdiget_BP.AreYouSureWdiget_BP_C"))

(fn OnNewSaveAskOverrideSaveCancelDelegate
  (UIAreYouSureWidget|UnbindAllfromAreYouSureWidget)
  (CallFunction|CloseWidget "/Game/Blueprints/HUD/Customization/AreYouSureWdiget_BP.AreYouSureWdiget_BP_C"))

(fn CreateNewSave
  (params (SaveName :type Name))
  (bind _returnvalue (SaveGame|CreateSaveGameObject "/Game/Blueprints/Customization/SamkaCharacterSaveClass_BP.SamkaCharacterSaveClass_BP_C"))
  (Default|SetSaveData _returnvalue SaveName (Utilities|String|StringToName (Class|HnomerBPLibraryPluginBPLibrary|GetProjectVersion)) (Class|KismetMathLibrary|Today) "None" "None" 0 (Utilities|Array|MakeArray) (Utilities|Struct|MakeBodyPartsColors_Struct "(R=1.000000,G=1.000000,B=1.000000,A=1.000000)" "(R=0.000000,G=0.000000,B=0.000000,A=1.000000)" "(R=1.000000,G=1.000000,B=1.000000,A=1.000000)") true true)
  (Save/LoadFunctions|LoadSave _returnvalue true false)
  (Customizing|SetProgressSaved false))

(fn UnbindAllfromAreYouSureWidget
  (bind _widgetobject (CallFunction|GetWidget "/Game/Blueprints/HUD/Customization/AreYouSureWdiget_BP.AreYouSureWdiget_BP_C"))
  (bind _asare_you_sure_wdiget_bp (Utilities|Casting|CastToAreYouSureWdiget_BP _widgetobject))
  (Utilities|FlowControl|Sequence
    (:then_0
      (EventDispatchers|UnbindallEventsfromOnYesAreYouSureWidget _asare_you_sure_wdiget_bp))
    (:then_1
      (EventDispatchers|UnbindallEventsfromOnNoAreYouSureWidget _asare_you_sure_wdiget_bp))
    (:then_2
      (EventDispatchers|UnbindallEventsfromOnCancelAreYouSureWidget _asare_you_sure_wdiget_bp))))

(fn OnNewSaveAskProgressIsNotSavedYesDelegate
  (UIAreYouSureWidget|UnbindAllfromAreYouSureWidget)
  (CallFunction|CloseWidget "/Game/Blueprints/HUD/Customization/AreYouSureWdiget_BP.AreYouSureWdiget_BP_C")
  (Save/LoadFunctions|SaveProgress)
  (Save/LoadFunctions|CreateNewSave (Variables|Default|GetPendingSaveFileName_BUFFER)))

(fn OnNewSaveAskProgressIsNotSavedNoDelegate
  (UIAreYouSureWidget|UnbindAllfromAreYouSureWidget)
  (CallFunction|CloseWidget "/Game/Blueprints/HUD/Customization/AreYouSureWdiget_BP.AreYouSureWdiget_BP_C")
  (Save/LoadFunctions|CreateNewSave (Variables|Default|GetPendingSaveFileName_BUFFER)))

(fn OnNewSaveAskProgressIsNotSavedCancelDelegate
  (UIAreYouSureWidget|UnbindAllfromAreYouSureWidget)
  (CallFunction|CloseWidget "/Game/Blueprints/HUD/Customization/AreYouSureWdiget_BP.AreYouSureWdiget_BP_C"))

(fn SaveProgress
  (bind _currentsavefile (Variables|Default|GetCurrentSaveFile))
  (Utilities|IsValid _currentsavefile
    (:Is%20Valid
      (bind _savename (Default|GetSaveData _currentsavefile))
      (if (!= (Variables|Customizing|GetThumbnail_BUFFER) 0)
        _
        (else
          (bind _returnvalue (Default|CMCaptureThumbnailPicture (Variables|Default|GetCustomizationManager)))
          (Variables|Customizing|SetThumbnail_BUFFER _returnvalue)))
      (Default|SetSaveData _currentsavefile _savename (Utilities|String|StringToName (Class|HnomerBPLibraryPluginBPLibrary|GetProjectVersion)) (Class|KismetMathLibrary|Today) "None" "None" (Variables|Customizing|GetThumbnail_BUFFER) (Variables|Default|GetMorphItemStructArray) (Variables|Default|GetBodyPartsColorsStruct) true true)
      (bind _issaved (CallFunction|Save "NewEnumerator0" _savename _currentsavefile))
      (Customizing|SetProgressSaved _issaved))))

(fn OnLoadSaveAskProgressIsNotSavedYes
  (UIAreYouSureWidget|UnbindAllfromAreYouSureWidget)
  (CallFunction|CloseWidget "/Game/Blueprints/HUD/Customization/AreYouSureWdiget_BP.AreYouSureWdiget_BP_C")
  (Save/LoadFunctions|SaveProgress)
  (bind _assamka_character_save_class_bp (Save/LoadFunctions|GetSavefromFile (Variables|Default|GetPendingSaveFileName_BUFFER)))
  (Save/LoadFunctions|LoadSave _assamka_character_save_class_bp true false))

(fn OnLoadSaveAskProgressIsNotSavedNo
  (UIAreYouSureWidget|UnbindAllfromAreYouSureWidget)
  (CallFunction|CloseWidget "/Game/Blueprints/HUD/Customization/AreYouSureWdiget_BP.AreYouSureWdiget_BP_C")
  (bind _assamka_character_save_class_bp (Save/LoadFunctions|GetSavefromFile (Variables|Default|GetPendingSaveFileName_BUFFER)))
  (Save/LoadFunctions|LoadSave _assamka_character_save_class_bp true false))

(fn OnLoadSaveAskProgressIsNotSavedCancel
  (UIAreYouSureWidget|UnbindAllfromAreYouSureWidget)
  (CallFunction|CloseWidget "/Game/Blueprints/HUD/Customization/AreYouSureWdiget_BP.AreYouSureWdiget_BP_C"))

(fn LoadSave
  (params (CurrentSaveFile :type Samka%20Character%20Save%20Class%20BP%20Object%20Reference) (IteruptAndNotifyAboutIncorrectValues :type Boolean) (IsSoftMix :type Boolean))
  (Utilities|IsValid (Variables|Default|GetCurrentSaveFile)
    (:Is%20Valid
      (if (!= CurrentSaveFile (Variables|Default|GetCurrentSaveFile))
        (bind _output_get (Variables|Default|SetCurrentSaveFile CurrentSaveFile :!label _label))
        (bind (_savename _saveversion _savedate _authorname _modifiedbyname _characterthumbnail _morphitemstruct_array _bodypartscolorsstruct) (Default|GetSaveData _output_get))
        (Variables|Default|SetBodyPartsColorsStruct _bodypartscolorsstruct)
        (bind (_isiterupted _mixedarray) (CallFunction|MixCustomMorphsArraywithMorphListArray _morphitemstruct_array (CallFunction|GetMorphList) IteruptAndNotifyAboutIncorrectValues IsSoftMix))
        (if _isiterupted
          (bind _widget_reference (CallFunction|OpenWidget "/Game/Blueprints/HUD/Customization/AreYouSureWdiget_BP.AreYouSureWdiget_BP_C" false 10))
          (bind _asare_you_sure_wdiget_bp (Utilities|Casting|CastToAreYouSureWdiget_BP _widget_reference))
          (Default|SetandShowAreYouSure _asare_you_sure_wdiget_bp (Utilities|Text|ToText(String) (Utilities|String|Append "You are about to load a save from earler version of the game! Difference between properties has been detected! 
Yes = force fix (may cause some data loss). 
No = soft fix (non-existing customization changes will not apply). 
Cancel = cancel loading. 
You can try manually making a backup file and try different options with it." "")) 10)
          (Utilities|FlowControl|Sequence
            (:then_0
              (EventDispatchers|BindEventtoOnYesAreYouSureWidget _asare_you_sure_wdiget_bp (EventDispatchers|CreateEvent :!event OnLoadSaveAskMixIteruptedYes)))
            (:then_1
              (EventDispatchers|BindEventtoOnNoAreYouSureWidget _asare_you_sure_wdiget_bp (EventDispatchers|CreateEvent :!event OnLoadSaveAskMixIteruptedNo)))
            (:then_2
              (EventDispatchers|BindEventtoOnCancelAreYouSureWidget _asare_you_sure_wdiget_bp (EventDispatchers|CreateEvent :!event OnLoadSaveAskMixIteruptedCancel))))
          (else
            (Variables|Default|SetMorphItemStructArray _mixedarray)
            (UICustomizationWidget|OnChangeCameraPositionCustomizationWidgetDelegate 5)
            (Customizing|EnterCustomizationEnvironment)
            (Customizing|SetProgressSaved true)))
        (else
          (UI|OnCloseCharacterSelectionMenuDelegate))))
    (:Is%20Not%20Valid
      (goto _label))))

(fn OnDeleteSaveAskDeleteSaveYes
  (UIAreYouSureWidget|UnbindAllfromAreYouSureWidget)
  (CallFunction|CloseWidget "/Game/Blueprints/HUD/Customization/AreYouSureWdiget_BP.AreYouSureWdiget_BP_C")
  (Save/LoadFunctions|DeleteSave (Variables|Default|GetPendingSaveFileName_BUFFER)))

(fn OnDeleteSaveAskDeleteSaveNo
  (UIAreYouSureWidget|UnbindAllfromAreYouSureWidget)
  (CallFunction|CloseWidget "/Game/Blueprints/HUD/Customization/AreYouSureWdiget_BP.AreYouSureWdiget_BP_C"))

(fn OnDeleteSaveAskDeleteSaveCancel
  (UIAreYouSureWidget|UnbindAllfromAreYouSureWidget)
  (CallFunction|CloseWidget "/Game/Blueprints/HUD/Customization/AreYouSureWdiget_BP.AreYouSureWdiget_BP_C"))

(fn DeleteSave
  (params (SaveName :type Name))
  (CallFunction|DeleteSave false SaveName)
  (UI|RefreshSavesList))

(fn RenameSave
  (params (SaveName :type Name) (NewSaveName :type Name))
  (if (Utilities|Name|NotEqual(Name) SaveName NewSaveName)
    (bind _isexists (CallFunction|IsSaveExists "NewEnumerator0" NewSaveName))
    (if (not _isexists)
      (bind (_issuccess _assamka_character_save_class_bp) (Save/LoadFunctions|GetSavefromFile SaveName))
      (if _issuccess
        (bind (_savename _saveversion _savedate _authorname _modifiedbyname _characterthumbnail _morphitemstruct_array _bodypartscolorsstruct _iscustomsave _iseditablesave) (Default|GetSaveData _assamka_character_save_class_bp))
        (Default|SetSaveData _assamka_character_save_class_bp NewSaveName _saveversion _savedate _authorname _modifiedbyname _characterthumbnail _morphitemstruct_array _bodypartscolorsstruct _iscustomsave _iseditablesave)
        (CallFunction|DeleteSave false SaveName)
        (CallFunction|Save "NewEnumerator0" NewSaveName _assamka_character_save_class_bp)
        (UI|RefreshSavesList)))))

(fn OnQuitAskProgressIsSavedYes
  (UIAreYouSureWidget|UnbindAllfromAreYouSureWidget)
  (CallFunction|CloseWidget "/Game/Blueprints/HUD/Customization/AreYouSureWdiget_BP.AreYouSureWdiget_BP_C")
  (Save/LoadFunctions|SaveProgress)
  (CallFunction|Quit true))

(fn OnQuitAskProgressIsSavedNo
  (UIAreYouSureWidget|UnbindAllfromAreYouSureWidget)
  (Customizing|SetProgressSaved true)
  (CallFunction|CloseWidget "/Game/Blueprints/HUD/Customization/AreYouSureWdiget_BP.AreYouSureWdiget_BP_C")
  (CallFunction|Quit true))

(fn OnQuitAskProgressIsSavedCancel
  (UIAreYouSureWidget|UnbindAllfromAreYouSureWidget)
  (CallFunction|CloseWidget "/Game/Blueprints/HUD/Customization/AreYouSureWdiget_BP.AreYouSureWdiget_BP_C"))

(fn Quit
  (params (ForceQuit :type Boolean))
  (if ForceQuit
    (CallFunction|SwitchULC "/Game/Levels/MainMenu_UpperLevelClass_BP.MainMenu_UpperLevelClass_BP_C" :!label _label)
    (elif (Variables|Customizing|GetIsProgressSaved)
      (goto _label)
      (else
        (bind _widget_reference (CallFunction|OpenWidget "/Game/Blueprints/HUD/Customization/AreYouSureWdiget_BP.AreYouSureWdiget_BP_C" false 10))
        (bind _asare_you_sure_wdiget_bp (Utilities|Casting|CastToAreYouSureWdiget_BP _widget_reference))
        (Default|SetandShowAreYouSure _asare_you_sure_wdiget_bp (Utilities|Text|MakeLiteralText "Your progress is not saved! Do you want to save it before quit?") 10)
        (Utilities|FlowControl|Sequence
          (:then_0
            (EventDispatchers|BindEventtoOnYesAreYouSureWidget _asare_you_sure_wdiget_bp (EventDispatchers|CreateEvent :!event OnQuitAskProgressIsSavedYes)))
          (:then_1
            (EventDispatchers|BindEventtoOnNoAreYouSureWidget _asare_you_sure_wdiget_bp (EventDispatchers|CreateEvent :!event OnQuitAskProgressIsSavedNo)))
          (:then_2
            (EventDispatchers|BindEventtoOnCancelAreYouSureWidget _asare_you_sure_wdiget_bp (EventDispatchers|CreateEvent :!event OnQuitAskProgressIsSavedCancel))))))))

(fn GetSavefromFile
  (params (SaveName :type Name))
  (bind (_issuccess _save_object) (CallFunction|GetSave "NewEnumerator0" false SaveName))
  (if _issuccess
    (bind _assamka_character_save_class_bp (Utilities|Casting|CastToSamkaCharacterSaveClass_BP _save_object)))
  (return _issuccess _assamka_character_save_class_bp))

(fn OnLoadSaveAskMixIteruptedYes
  (UIAreYouSureWidget|UnbindAllfromAreYouSureWidget)
  (CallFunction|CloseWidget "/Game/Blueprints/HUD/Customization/AreYouSureWdiget_BP.AreYouSureWdiget_BP_C")
  (bind _assamka_character_save_class_bp (Save/LoadFunctions|GetSavefromFile (Variables|Default|GetPendingSaveFileName_BUFFER)))
  (Save/LoadFunctions|LoadSave _assamka_character_save_class_bp false false))

(fn OnLoadSaveAskMixIteruptedNo
  (UIAreYouSureWidget|UnbindAllfromAreYouSureWidget)
  (CallFunction|CloseWidget "/Game/Blueprints/HUD/Customization/AreYouSureWdiget_BP.AreYouSureWdiget_BP_C")
  (bind _assamka_character_save_class_bp (Save/LoadFunctions|GetSavefromFile (Variables|Default|GetPendingSaveFileName_BUFFER)))
  (Save/LoadFunctions|LoadSave _assamka_character_save_class_bp false true))

(fn OnLoadSaveAskMixIteruptedCancel
  (UIAreYouSureWidget|UnbindAllfromAreYouSureWidget)
  (CallFunction|CloseWidget "/Game/Blueprints/HUD/Customization/AreYouSureWdiget_BP.AreYouSureWdiget_BP_C")
  (Variables|Default|SetCurrentSaveFile 0))

(fn EnterCustomizationEnvironment
  (if (and (Utilities|IsValid (Variables|Default|GetCurrentSaveFile)) (> (Utilities|Array|Length (Variables|Default|GetMorphItemStructArray)) 0))
    (Variables|Customizing|SetThumbnail_BUFFER 0)
    (UI|SetBackButton true)
    (Variables|Customizing|SetIsInCustomizationEnvironment true)
    (bind _widget_reference (CallFunction|OpenWidget "/Game/Blueprints/HUD/Customization/CustomizationWidget_BP.CustomizationWidget_BP_C" true 1))
    (CallFunction|CloseWidget "/Game/Blueprints/HUD/Customization/SaveLoadCustomizationWidget_BP.SaveLoadCustomizationWidget_BP_C")
    (bind _ascustomization_widget_bp (Utilities|Casting|CastToCustomizationWidget_BP _widget_reference))
    (Utilities|FlowControl|Sequence
      (:then_0
        (Utilities|FlowControl|Sequence
          (:then_0
            (EventDispatchers|BindEventtoOnClickedButtonChangeCameraPositionCustomizationWidgetDelegate _ascustomization_widget_bp (EventDispatchers|CreateEvent :!event OnChangeCameraPositionCustomizationWidgetDelegate)))
          (:then_1
            (EventDispatchers|BindEventtoOnClickedButtonLoadCustomizationWidgetDelegate _ascustomization_widget_bp (EventDispatchers|CreateEvent :!event OnLoadCustomizationWidgetDelegate)))
          (:then_2
            (EventDispatchers|BindEventtoOnClickedButtonQuitCustomizationWidgetDelegate _ascustomization_widget_bp (EventDispatchers|CreateEvent :!event OnQuitCustomizationWidgetDelegate)))
          (:then_3
            (EventDispatchers|BindEventtoOnClickedButtonSaveCustomizationWidgetDelegate _ascustomization_widget_bp (EventDispatchers|CreateEvent :!event OnSaveCustomizationWidgetDelegate)))
          (:then_4
            (EventDispatchers|BindEventtoOnClickedButtonSaveThumbnailCustomizationWidgetDelegate _ascustomization_widget_bp (EventDispatchers|CreateEvent :!event OnSaveThumbnailCustomizationWidgetDelegate)))
          (:then_5
            (EventDispatchers|BindEventtoOnMorphValueChangedCustomizationWidgetDelegate _ascustomization_widget_bp (EventDispatchers|CreateEvent :!event OnMorphValueChangedCustomizationWidgetDelegate)))
          (:then_6
            (EventDispatchers|BindEventtoOnRequestApplyColortoBodypartCustomizationWidgetDelegate _ascustomization_widget_bp (EventDispatchers|CreateEvent :!event OnRequestApplyColortoBodyPartCustomizationWidgetDelegate)))))
      (:then_1
        (UICustomizationWidget|OnChangeCameraPositionCustomizationWidgetDelegate 5)
        (Default|CMSetSamkaMorphs (Variables|Default|GetCustomizationManager) (Variables|Default|GetMorphItemStructArray))
        (bind (_savename _saveversion _savedate _authorname _modifiedbyname _characterthumbnail _morphitemstruct_array _bodypartscolorsstruct) (Default|GetSaveData (Variables|Default|GetCurrentSaveFile)))
        (Default|SetSaveName _ascustomization_widget_bp (Utilities|Text|ToText(Name) _savename))
        (Default|SetSectionName _ascustomization_widget_bp "Nothing Selected")
        (Default|RemoveMorphsEditorWidgets _ascustomization_widget_bp)
        (Default|CMApplyColortoBodyPart (Variables|Default|GetCustomizationManager) "NewEnumerator2")
        (Default|SetBodyPartsColors _ascustomization_widget_bp _bodypartscolorsstruct)
        (Save/LoadFunctions|ApplyLoadedBodyPartsColors)))))

(fn OnChangeCameraPositionCustomizationWidgetDelegate
  (params (New%20Camera%20Position :type Integer))
  (Default|CMChangeCamera (Variables|Default|GetCustomizationManager) New%20Camera%20Position))

(fn OnLoadCustomizationWidgetDelegate
  (UI|OpenCharacterSelectionMenu))

(fn OnQuitCustomizationWidgetDelegate
  (CallFunction|Quit false))

(fn OnSaveCustomizationWidgetDelegate
  (Save/LoadFunctions|SaveProgress)
  (Customizing|SetProgressSaved true))

(fn OnSaveThumbnailCustomizationWidgetDelegate
  (bind _returnvalue (Default|CMCaptureThumbnailPicture (Variables|Default|GetCustomizationManager)))
  (Variables|Customizing|SetThumbnail_BUFFER _returnvalue))

(fn OnMorphValueChangedCustomizationWidgetDelegate
  (params (Index :type Integer) (MorphStruct :type Morph%20Item%20Struct%20Structure))
  (Customizing|SetProgressSaved false)
  (Default|CMSetSamkaMorphs (Variables|Default|GetCustomizationManager) (Utilities|Array|MakeArray MorphStruct))
  (Utilities|Array|SetArrayElem (Variables|Default|GetMorphItemStructArray) Index MorphStruct))

(fn Init
  (bind (_isfound _customizationmanager) (CallFunction|GetCustomizationManager))
  (if _isfound
    (Variables|Default|SetCustomizationManager _customizationmanager)
    (CallFunction|InitSamkaCursorCollisionDelegates)
    (Input|EnableInput (Game|GetPlayerController 0))
    (CallFunction|SetInputMode true false false 0 "DoNotLock" false)
    (return true)
    (else
      (return false))))

(fn InitSamkaCursorCollisionDelegates
  (bind _customizationmanager (Variables|Default|GetCustomizationManager))
  (Utilities|FlowControl|Sequence
    (:then_0
      (EventDispatchers|BindEventtoOnSamkaCursorBeginOverlapBodyPartDelegate _customizationmanager (EventDispatchers|CreateEvent :!event OnSamkaCursorBeginOverlapBodyPartDelegate)))
    (:then_1
      (EventDispatchers|BindEventtoOnSamkaCursorEndOverlapBodyPartDelegate _customizationmanager (EventDispatchers|CreateEvent :!event OnSamkaCursorEndOverlapBodyPartDelegate)))
    (:then_2
      (EventDispatchers|BindEventtoOnSamkaClickedBodyPartDelegate _customizationmanager (EventDispatchers|CreateEvent :!event OnSamkaClickedBodyPartDelegate)))))

(fn OnSamkaCursorBeginOverlapBodyPartDelegate
  (params (BodyPart :type BodyParts_Enum%20Enum :default "NewEnumerator0"))
  (if (Variables|Customizing|GetIsInCustomizationEnvironment)
    (CallFunction|SetShowCursorTooltip true (Utilities|Text|ToText(String) (Utilities|String|EnumtoString BodyPart)) 1)))

(fn OnSamkaCursorEndOverlapBodyPartDelegate
  (CallFunction|SetShowCursorTooltip false "" 1))

(fn OnSamkaClickedBodyPartDelegate
  (params (BodyPart :type BodyParts_Enum%20Enum :default "NewEnumerator0"))
  (if (Variables|Customizing|GetIsInCustomizationEnvironment)
    (bind _widgetobject (CallFunction|GetWidget "/Game/Blueprints/HUD/Customization/CustomizationWidget_BP.CustomizationWidget_BP_C"))
    (bind _ascustomization_widget_bp (Utilities|Casting|CastToCustomizationWidget_BP _widgetobject))
    (Default|CreateMorphsEditorWidgetsforSection _ascustomization_widget_bp (Utilities|String|StringToName (Utilities|String|EnumtoString BodyPart)) (Variables|Default|GetMorphItemStructArray))))

(fn ExitCustomizationEnvironment
  (CallFunction|CloseWidget "/Game/Blueprints/HUD/Customization/CustomizationWidget_BP.CustomizationWidget_BP_C")
  (Variables|Customizing|SetIsInCustomizationEnvironment false))

(fn SetProgressSaved
  (params (IsSaved :type Boolean))
  (if (Math|Boolean|NotEqual(Boolean) IsSaved (Variables|Customizing|GetIsProgressSaved))
    (bind _output_get (Variables|Customizing|SetIsProgressSaved IsSaved))
    (bind _widgetobject (CallFunction|GetWidget "/Game/Blueprints/HUD/Customization/CustomizationWidget_BP.CustomizationWidget_BP_C"))
    (bind _ascustomization_widget_bp (Utilities|Casting|CastToCustomizationWidget_BP _widgetobject))
    (Default|SetSaveButtonEnabled _ascustomization_widget_bp (not _output_get))))

(fn RefreshSavesList
  (bind _widgetobject (CallFunction|GetWidget "/Game/Blueprints/HUD/Customization/SaveLoadCustomizationWidget_BP.SaveLoadCustomizationWidget_BP_C"))
  (bind _assave_load_customization_widget_bp (Utilities|Casting|CastToSaveLoadCustomizationWidget_BP _widgetobject))
  (Default|Refresh _assave_load_customization_widget_bp))

(fn SetBackButton
  (params (On/Off :type Boolean))
  (bind _widgetobject (CallFunction|GetWidget "/Game/Blueprints/HUD/Customization/SaveLoadCustomizationWidget_BP.SaveLoadCustomizationWidget_BP_C"))
  (bind _assave_load_customization_widget_bp (Utilities|Casting|CastToSaveLoadCustomizationWidget_BP _widgetobject))
  (Default|SetBackButton _assave_load_customization_widget_bp On/Off))

(fn OnRequestApplyColortoBodyPartCustomizationWidgetDelegate
  (params (Body%20Part :type ColorBodyParts_ENum%20Enum :default "NewEnumerator2") (Color :type Linear%20Color%20Structure))
  (Default|CMApplyColortoBodyPart (Variables|Default|GetCustomizationManager) Body%20Part Color)
  (Customizing|SetProgressSaved false)
  (switch Utilities|FlowControl|Switch|SwitchonColorBodyParts_ENum Body%20Part
    (:NewEnumerator0
      (Variables|Default|SetBodyPartsColorsStruct (Utilities|Struct|MakeBodyPartsColors_Struct Color (.Hair (Utilities|Struct|BreakBodyPartsColors_Struct (Variables|Default|GetBodyPartsColorsStruct))) (.Eyes (Utilities|Struct|BreakBodyPartsColors_Struct (Variables|Default|GetBodyPartsColorsStruct))))))
    (:NewEnumerator1
      (Variables|Default|SetBodyPartsColorsStruct (Utilities|Struct|MakeBodyPartsColors_Struct (.Skin (Utilities|Struct|BreakBodyPartsColors_Struct (Variables|Default|GetBodyPartsColorsStruct))) Color (.Eyes (Utilities|Struct|BreakBodyPartsColors_Struct (Variables|Default|GetBodyPartsColorsStruct))))))
    (:NewEnumerator3
      (Variables|Default|SetBodyPartsColorsStruct (Utilities|Struct|MakeBodyPartsColors_Struct (.Skin (Utilities|Struct|BreakBodyPartsColors_Struct (Variables|Default|GetBodyPartsColorsStruct))) (.Hair (Utilities|Struct|BreakBodyPartsColors_Struct (Variables|Default|GetBodyPartsColorsStruct))) Color)))))

(fn ApplyLoadedBodyPartsColors
  (bind _customizationmanager (Variables|Default|GetCustomizationManager))
  (bind _bodypartscolorsstruct (Variables|Default|GetBodyPartsColorsStruct))
  (bind (_skin _hair _eyes) (Utilities|Struct|BreakBodyPartsColors_Struct _bodypartscolorsstruct))
  (Default|CMApplyColortoBodyPart _customizationmanager "NewEnumerator0" _skin)
  (Default|CMApplyColortoBodyPart _customizationmanager "NewEnumerator1" _hair)
  (Default|CMApplyColortoBodyPart _customizationmanager "NewEnumerator3" _eyes))