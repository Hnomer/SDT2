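; BlinkManager is a component that drives random eye blinking for a Samka character through its SS_Anim_Instance.
; It finds the anim instance on a Samka_BP owner's root mesh, or on an assigned skeletal component for other owners.
; Blink-rate presets or a custom rate become a per-tick percent chance scaled by tick interval, rolled each tick to set DoBlink.
; CloseEyes and OpenEyes hold the eyes shut or release them, pausing and resuming blinking.
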(event EventBeginPlay
  (CallFunction|Init)
  (CallFunction|SetBlinksPerMinute "NewEnumerator1"))

(event EventTick
  (params (DeltaSeconds :type Float%20%28single-precision%29))
  (CallFunction|TryBlink DeltaSeconds))

(fn CloseEyes
  (Variables|Default|SetCanBlink false)
  (Variables|/Script/Sex_Simulator.SS_Anim_Instance|SetDoCloseEyes (Variables|Default|GetSamkaAnimationClass) true))

(fn OpenEyes
  (Variables|/Script/Sex_Simulator.SS_Anim_Instance|SetDoCloseEyes (Variables|Default|GetSamkaAnimationClass) false)
  (Variables|Default|SetCanBlink true))

(fn TryBlink
  (params (DeltaTime :type Float%20%28single-precision%29))
  (if (Variables|Default|GetCanBlink)
    (if (<= (Math|Random|RandomIntegerinRange 0 100) (Variables|Default|GetBlinkChance))
      (Variables|/Script/Sex_Simulator.SS_Anim_Instance|SetDoBlink (Variables|Default|GetSamkaAnimationClass) true))))

(fn SetBlinksPerMinute
  (params (BlinkSpeedMode :type BlinkSpeedModesENum%20Enum :default "NewEnumerator0") (CustomBlinksPerMinute :type Integer))
  (switch Utilities|FlowControl|Switch|SwitchonBlinkSpeedModesENum BlinkSpeedMode
    (:NewEnumerator0
      (LocalVariables|SetNew_BlinksPerMinute 17.0))
    (:NewEnumerator1
      (LocalVariables|SetNew_BlinksPerMinute 27.0))
    (:NewEnumerator2
      (LocalVariables|SetNew_BlinksPerMinute 37.0))
    (:NewEnumerator3
      (LocalVariables|SetNew_BlinksPerMinute 47.0))
    (:NewEnumerator4
      (LocalVariables|SetNew_BlinksPerMinute (Math|Conversions|ToFloat(Integer) CustomBlinksPerMinute))))
  (Variables|Default|SetBlinkChance (Math|Float|Floor (* 100 (/ (LocalVariables|GetNew_BlinksPerMinute) (/ 6e+01 (Class|ActorComponent|GetComponentTickInterval)))))))

(fn Init
  (bind _samkaskeletalcomponent (Variables|Default|GetSamkaSkeletalComponent))
  (bind _assamka_bp (Utilities|Casting|CastToSamka_BP (Components|GetOwner))
    (:then
      (Variables|Default|SetSamkaActor _assamka_bp)
      (bind _asskeletal_mesh_component (Utilities|Casting|CastToSkeletalMeshComponent (Variables|/Script/Engine.Actor|GetRootComponent _assamka_bp)))
      (bind _asss_anim_instance (Utilities|Casting|CastToSS_Anim_Instance (Components|SkeletalMesh|GetAnimInstance _asskeletal_mesh_component)))
      (Variables|Default|SetSamkaAnimationClass _asss_anim_instance))
    (:CastFailed
      (Utilities|IsValid _samkaskeletalcomponent
        (:Is%20Valid
          (bind _asss_anim_instance_2 (Utilities|Casting|CastToSS_Anim_Instance (Components|SkeletalMesh|GetAnimInstance _samkaskeletalcomponent)))
          (Variables|Default|SetSamkaAnimationClass _asss_anim_instance_2))))))