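; Global Blueprint function library giving the game one-call access to its managers, plus string, math, cursor, fade and sound helpers.
; Most wrappers forward to GameInstance-held managers for widgets, lower/upper level classes and saves; object and customization managers are found by actor tag.
; Settings helpers load or save a settings object, choosing new defaults by platform and GPU brand.
; Morph helpers parse, merge and rewrite a sectioned morph-list text file in CustomAssets.
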(fn GetObjectManager
  (bind _outactors (Actor|GetAllActorswithTag 0 "ObjectsManager"))
  (if (> (Utilities|Array|Length _outactors) 0)
    (bind _asobjects_manager (Utilities|Casting|CastToObjectsManager (Utilities|Array|Get(acopy) _outactors))
      (:then
        (return true _asobjects_manager))
      (:CastFailed
        _)))
  (return false 0))

(fn CutStringtoLength
  (params (InString :type String) (MaxLength :type Integer))
  (bind _returnvalue (Utilities|String|Len InString))
  (if (> _returnvalue MaxLength)
    (return (Utilities|String|LeftChop InString (Math|Integer|Absolute(Integer) (- MaxLength _returnvalue))))
    (else
      (return InString))))

(fn ConvertNormalizedFloattoRange
  (params (Value :type Float%20%28single-precision%29) (MinValue :type Float%20%28single-precision%29) (MaxValue :type Float%20%28single-precision%29))
  (return (+ (* Value (- MaxValue MinValue)) MinValue)))

(fn IsStringContainsCharacters
  (params (String :type String) (Substrings :type Array%20of%20Strings))
  (bind _array_element (Utilities|Array|ForEachLoopwithBreak Substrings :!label _label)
    (:LoopBody
      (if (Utilities|String|Contains String _array_element false true)
        (goto _label Break)))
    (:Completed
      (return (Utilities|String|Contains String _array_element false true)))))

(fn IsStringContainsBannedCharacters
  (params (String :type String))
  (return (MyFNCLib|IsStringContainsCharacters String (Utilities|Array|MakeArray "/" "\\" "*" "<" ">" ":" "?" "\"" "|"))))

(fn GetWidgetManager
  (return true (Variables|/Game/Blueprints/GameInstance_BP.GameInstance_BP_C|GetWidgetManager (MyFNCLib|GetCustomGameInstance))))

(fn OpenWidget
  (params (WidgetClass :type User%20Widget%20Class%20Reference) (AddOnScreen :type Boolean) (Z%20Order :type Integer))
  (bind (_isfound _widgetmanager) (MyFNCLib|GetWidgetManager))
  (if (!= WidgetClass 0)
    (if _isfound
      (bind _widget_object (Default|WMOpenWidget _widgetmanager WidgetClass))
      (if AddOnScreen
        (if (UserInterface|Viewport|IsinViewport _widget_object)
          _
          (else
            (UserInterface|Viewport|AddtoViewport _widget_object Z%20Order))))
      (return _widget_object))))

(fn CloseWidget
  (params (WidgetClass :type User%20Widget%20Class%20Reference))
  (bind (_isfound _widgetmanager) (MyFNCLib|GetWidgetManager))
  (if _isfound
    (Default|WMCloseWidget _widgetmanager WidgetClass)))

(fn SetLoadingScreenEnabled
  (params (On/Off :type Boolean) (HideCursor :type Boolean) (ZOrder :type Integer))
  (bind (_isfound _widgetmanager) (MyFNCLib|GetWidgetManager))
  (if _isfound
    (if On/Off
      (bind _widget_object (Default|WMOpenWidget _widgetmanager "/Game/Blueprints/HUD/LoadingScreen/LoadingScreen.LoadingScreen_C"))
      (if (UserInterface|Viewport|IsinViewport _widget_object)
        (bind _asloading_screen (Utilities|Casting|CastToLoadingScreen _widget_object))
        (Default|Reload _asloading_screen)
        (else
          (UserInterface|Viewport|AddtoViewport _widget_object ZOrder)))
      (if HideCursor
        (MyFNCLib|SetCursorVisibility false))
      (else
        (bind _asloading_screen_2 (Utilities|Casting|CastToLoadingScreen (Default|WMGetWidget _widgetmanager "/Game/Blueprints/HUD/LoadingScreen/LoadingScreen.LoadingScreen_C")))
        (if (Variables|/Game/Blueprints/HUD/LoadingScreen/LoadingScreen.LoadingScreen_C|GetIsLoading _asloading_screen_2)
          (Default|LoadingScreenEventFinishLoading _asloading_screen_2))))))

(fn LoadLLC
  (params (LevelName :type String) (ShouldBeVisibleAfterLoading :type Boolean) (LoadingScreen :type Boolean) (ZOrder :type Integer) (Don'tDisableLoadingScreen :type Boolean))
  (bind (_isfound _levelmanager) (MyFNCLib|GetLLCManager))
  (if _isfound
    (bind (_success _levelobject) (Default|LLCMLoadLevel _levelmanager LevelName ShouldBeVisibleAfterLoading LoadingScreen ZOrder Don'tDisableLoadingScreen))
    (return _success _levelobject)))

(fn UnloadLLC
  (params (LevelName :type String))
  (bind (_isfound _levelmanager) (MyFNCLib|GetLLCManager))
  (if _isfound
    (bind _issuccess (Default|LLCMUnloadLevel _levelmanager LevelName))
    (return _issuccess)
    (else
      (return false))))

(fn GetLoadedLLC
  (params (LevelName :type String))
  (bind (_isfound _levelmanager) (MyFNCLib|GetLLCManager))
  (bind (_isfound_2 _level) (Default|LLCMGetLoadedLevel _levelmanager LevelName))
  (if _isfound
    (if _isfound_2
      (return true _level)
      (else
        (return false 0)))))

(fn GetLLCManager
  (return true (Variables|/Game/Blueprints/GameInstance_BP.GameInstance_BP_C|GetLLCManager (MyFNCLib|GetCustomGameInstance))))

(fn HideLLC
  (params (LevelName :type String))
  (bind (_isfound _levelmanager) (MyFNCLib|GetLLCManager))
  (if _isfound
    (Default|LLCMHideLevel _levelmanager LevelName)))

(fn GetCustomGameInstance
  (bind _asgame_instance_bp (Utilities|Casting|CastToGameInstance_BP (Game|GetGameInstance)))
  (return _asgame_instance_bp))

(fn CreateULCInstance
  (params (Level%20Class :type Base%20Upper%20Level%20Class%20BP%20Class%20Reference))
  (bind _returnvalue (Class|VictoryBPFunctionLibrary|SpawnActorIntoLevel Level%20Class "Persistant_Level" "0, 0, 0" "0, 0, 0" true))
  (bind _asbase_upper_level_class_bp (Utilities|Casting|CastToBaseUpperLevelClass_BP _returnvalue))
  (bind (_level _streaminglevel _widget_reference) (Default|ULCLoad _asbase_upper_level_class_bp))
  (return _asbase_upper_level_class_bp _streaminglevel _widget_reference))

(fn DeleteULCInstance
  (params (LevelInstanse :type Base%20Upper%20Level%20Class%20BP%20Object%20Reference))
  (Default|ULCUnload LevelInstanse))

(fn HideULCInstance
  (params (LevelInstance :type Base%20Upper%20Level%20Class%20BP%20Object%20Reference))
  (Default|ULCHide LevelInstance))

(fn SwitchULC
  (params (LevelClass :type Base%20Upper%20Level%20Class%20BP%20Class%20Reference))
  (bind (_isfound _upperlevelclassmanager) (MyFNCLib|GetULCManager))
  (if _isfound
    (Default|ULCMSwitchLevelClass _upperlevelclassmanager LevelClass)))

(fn GetULCManager
  (return true (Variables|/Game/Blueprints/GameInstance_BP.GameInstance_BP_C|GetULCManager (MyFNCLib|GetCustomGameInstance))))

(fn SetCursorVisibility
  (params (IsVisible :type Boolean))
  (Variables|/Script/Engine.PlayerController|SetbShowMouseCursor (Game|GetPlayerController 0) IsVisible))

(fn SetInputMode
  (params (GameAndUI :type Boolean) (GameOnly :type Boolean) (UI%20Only :type Boolean) (InWidgetToFocus :type Widget%20Object%20Reference) (InMouseLockMode :type EMouseLockMode%20Enum :default "DoNotLock") (bHideCursorDuringCapture :type Boolean))
  (bind _returnvalue (Game|GetPlayerController 0))
  (if GameAndUI
    (Input|SetInputModeGameandUI _returnvalue InWidgetToFocus InMouseLockMode bHideCursorDuringCapture)
    (elif GameOnly
      (Input|SetInputModeGameOnly _returnvalue)
      (elif UI%20Only
        (Input|SetInputModeUIOnly _returnvalue InWidgetToFocus InMouseLockMode)))))

(fn GetWidget
  (params (WidgetClass :type User%20Widget%20Class%20Reference))
  (bind (_isfound _widgetmanager) (MyFNCLib|GetWidgetManager))
  (if _isfound
    (return (Default|WMGetWidget _widgetmanager WidgetClass))
    (else
      (return 0))))

(fn GetSavesManager
  (bind _custom_game_instance (MyFNCLib|GetCustomGameInstance))
  (bind _savesmanager (Variables|/Game/Blueprints/GameInstance_BP.GameInstance_BP_C|GetSavesManager _custom_game_instance))
  (return (Utilities|IsValid _savesmanager) _savesmanager))

(fn GetAllSaves
  (params (Save%20Type :type SaveFileType_ENum%20Enum :default "NewEnumerator0") (IncludeBuitInSaves :type Boolean) (SortByDate :type Boolean))
  (bind (_isfound _saves_manager) (MyFNCLib|GetSavesManager))
  (if _isfound
    (bind _save_objects_array (Default|SMGetAllSaveFiles _saves_manager IncludeBuitInSaves false SortByDate Save%20Type))
    (return _save_objects_array)))

(fn GetSave
  (params (Save%20Type :type SaveFileType_ENum%20Enum :default "NewEnumerator0") (IsExtetnalSaveName :type Boolean) (SaveName :type Name))
  (bind (_isfound _saves_manager) (MyFNCLib|GetSavesManager))
  (if _isfound
    (bind (_issuccess _returnvalue) (Default|SMGetSave _saves_manager Save%20Type IsExtetnalSaveName SaveName))
    (return _issuccess _returnvalue)))

(fn Save
  (params (SaveType :type SaveFileType_ENum%20Enum :default "NewEnumerator0") (SlotName :type Name) (Save%20Object :type Save%20Game%20Object%20Reference))
  (bind (_isfound _saves_manager) (MyFNCLib|GetSavesManager))
  (if _isfound
    (bind _issaved (Default|SMSave _saves_manager SaveType SlotName Save%20Object))
    (return _issaved)))

(fn DeleteSave
  (params (DeleteByExternalName :type Boolean) (Save%20name :type Name))
  (bind (_isfound _saves_manager) (MyFNCLib|GetSavesManager))
  (if _isfound
    (bind _issuccess (Default|SMDeleteSave _saves_manager DeleteByExternalName Save%20name))
    (return _issuccess)))

(fn SetSamkaMorphs!GamingLevelOnly!
  (params (MorphsArray :type Array%20of%20Morph%20Item%20Struct%20Structures))
  (bind (_isfound _objectmanager) (MyFNCLib|GetObjectManager))
  (if _isfound
    (Default|OMSetSamkaMorphs _objectmanager MorphsArray)
    (return true)
    (else
      (return false))))

(fn GetSettingsSaveObject
  (bind (_issuccess _save_object) (MyFNCLib|GetSave "NewEnumerator1" false "settings"))
  (if _issuccess
    (bind _assettings_save_class_bp (Utilities|Casting|CastToSettingsSaveClass_BP _save_object)
      (:then
        (return true _assettings_save_class_bp))
      (:CastFailed
        _)))
  (return false 0))

(fn GetDatafromSettingsSaveObject
  (bind (_issuccess _assettings_save_class_bp) (MyFNCLib|GetSettingsSaveObject))
  (if _issuccess
    (return true (Variables|/Game/Blueprints/SettingsSaveClass_BP.SettingsSaveClass_BP_C|GetSettingsStruct _assettings_save_class_bp))
    (else
      (bind _settingsobject (MyFNCLib|CreateNewSettingsSaveObject))
      (MyFNCLib|Save "NewEnumerator1" "settings" _settingsobject)
      (return true (Variables|/Game/Blueprints/SettingsSaveClass_BP.SettingsSaveClass_BP_C|GetSettingsStruct _settingsobject)))))

(fn SaveDatatoSettingsSaveObject
  (params (SettingsStruct :type Settings%20Save%20Struct%20Structure))
  (bind (_issuccess _assettings_save_class_bp) (MyFNCLib|GetSettingsSaveObject))
  (if _issuccess
    (Variables|/Game/Blueprints/SettingsSaveClass_BP.SettingsSaveClass_BP_C|SetSettingsStruct _assettings_save_class_bp SettingsStruct)
    (bind _issaved (MyFNCLib|Save "NewEnumerator1" "settings" _assettings_save_class_bp))
    (return _issaved)))

(fn IsSaveExists
  (params (Save%20Type :type SaveFileType_ENum%20Enum :default "NewEnumerator0") (SaveName :type Name))
  (bind (_isfound _saves_manager) (MyFNCLib|GetSavesManager))
  (if _isfound
    (bind _isexists (Default|SMIsSaveExists _saves_manager Save%20Type SaveName))
    (return _isexists)))

(fn IsStringEmptyorSpacesOnly
  (params (String :type String))
  (if (Class|VictoryBPFunctionLibrary|StringIsEmpty String)
    _
    (else
      (bind _output_get (LocalVariables|SetArrayFromString (Utilities|String|GetCharacterArrayfromString String)))
      (Utilities|Array|RemoveItem _output_get " ")
      (if (> (Utilities|Array|Length _output_get) 0)
        (return false)
        (else
          _))))
  (return true))

(fn GetMorphListasArrayOfMorphStructs
  (bind _returnvalue (Class|HnomerBPLibraryPluginBPLibrary|GetGameContentDirPath))
  (bind _returnvalue_2 (Utilities|String|Append _returnvalue "CustomAssets/morphslist.txt"))
  (bind (_stringarray _arraysize _returnvalue_3) (Class|VictoryBPFunctionLibrary|LoadStringArrayfromFile _returnvalue_2 true))
  (if _returnvalue_3
    (for _array_element _stringarray
      (if (>= (Utilities|String|FindSubstring _array_element "*") 0)
        (LocalVariables|SetCurrentSectionName (Utilities|String|StringToName (Utilities|Array|Get(acopy) (Class|VictoryBPFunctionLibrary|StringExplodeString _array_element "*" 0 false) 1)))
        (else
          (bind _output_get (LocalVariables|SetMorphItemStruct (Utilities|Struct|MakeMorphItemStruct (Utilities|String|StringToName (Utilities|Array|Get(acopy) (Class|VictoryBPFunctionLibrary|StringExplodeString _array_element "#" 0 false))) (LocalVariables|GetCurrentSectionName) (Utilities|String|StringToName (Utilities|Array|Get(acopy) (Class|VictoryBPFunctionLibrary|StringExplodeString _array_element "#" 0 false) 1)) (Math|Conversions|ToFloat(Integer) (Utilities|Array|Get(acopy) (Class|VictoryBPFunctionLibrary|StringExplodeString _array_element "#" 0 false) 2)) (Math|Conversions|ToFloat(Integer) (Utilities|Array|Get(acopy) (Class|VictoryBPFunctionLibrary|StringExplodeString _array_element "#" 0 false) 3)) (Math|Conversions|ToFloat(Integer) (Utilities|Array|Get(acopy) (Class|VictoryBPFunctionLibrary|StringExplodeString _array_element "#" 0 false) 4)))))
          (Utilities|Array|Add (LocalVariables|GetMorphItemStructsArray) _output_get))))
    (return true (LocalVariables|GetMorphItemStructsArray))
    (else
      (return false 0))))

(fn MixCustomMorphsArraywithMorphListArray
  (params (Custom%20Morphs :type Array%20of%20Morph%20Item%20Struct%20Structures) (MorphList%20Array :type Array%20of%20Morph%20Item%20Struct%20Structures) (IteruptAndNotifyAboutIncorrectValues :type Boolean) (IsSoftMix :type Boolean))
  (LocalVariables|SetCustomArray Custom%20Morphs)
  (for _array_element MorphList%20Array
    (LocalVariables|SetHasMorphBeenFound false)
    (LocalVariables|SetMorphItem _array_element)
    (bind (_array_element_2 _array_index) (Utilities|Array|ForEachLoopwithBreak (LocalVariables|GetCustomArray) :!label _label)
      (:LoopBody
        (if (Utilities|Name|Equal(Name) (Utilities|Struct|BreakMorphItemStruct _array_element_2) (Utilities|Struct|BreakMorphItemStruct _array_element))
          (LocalVariables|SetHasMorphBeenFound true)
          (if (Math|Float|InRange(Float) (.CurrentValue (Utilities|Struct|BreakMorphItemStruct _array_element_2)) (.MinimumValue (Utilities|Struct|BreakMorphItemStruct _array_element)) (.MaximumValue (Utilities|Struct|BreakMorphItemStruct _array_element)))
            (Utilities|Struct|SetmembersinMorphItemStruct (LocalVariables|GetMorphItem) (.CurrentValue (Utilities|Struct|BreakMorphItemStruct _array_element_2)))
            (goto _label Break)
            (else
              ;[1 1 1 1 11] Is Iterupt
              (if IteruptAndNotifyAboutIncorrectValues
                (return true 0)
                (else
                  ;[1 1 1 1 11] Is Soft Mix
                  (if IsSoftMix
                    (Utilities|Struct|SetmembersinMorphItemStruct (LocalVariables|GetMorphItem) (.MinimumValue (Utilities|Struct|BreakMorphItemStruct _array_element_2)) (.MaximumValue (Utilities|Struct|BreakMorphItemStruct _array_element_2)) (.CurrentValue (Utilities|Struct|BreakMorphItemStruct _array_element_2)) (.DefaultValue (Utilities|Struct|BreakMorphItemStruct _array_element_2)))
                    (goto _label Break)
                    (else
                      (Utilities|Struct|SetmembersinMorphItemStruct (LocalVariables|GetMorphItem) (Math|Float|Clamp(Float) (.CurrentValue (Utilities|Struct|BreakMorphItemStruct _array_element_2)) (.MinimumValue (Utilities|Struct|BreakMorphItemStruct _array_element)) (.MaximumValue (Utilities|Struct|BreakMorphItemStruct _array_element))))
                      (goto _label Break)))))))))
      (:Completed
        (if (LocalVariables|GetHasMorphBeenFound)
          (Utilities|Array|RemoveIndex (LocalVariables|GetCustomArray) _array_index))
        (Utilities|Array|Add (LocalVariables|GetFinalArray) (LocalVariables|GetMorphItem)))))
  (if (> (Utilities|Array|Length (LocalVariables|GetCustomArray)) 0)
    (if IteruptAndNotifyAboutIncorrectValues
      (return true 0)
      (else
        _)))
  (return false (LocalVariables|GetFinalArray)))

(fn WriteMorphItemtoMorphList
  (params (MorphArrayStruct :type Morph%20Item%20Struct%20Structure))
  (bind (_readablename _sectionname _morphname _minimumvalue _maximumvalue _currentvalue _defaultvalue) (Utilities|Struct|BreakMorphItemStruct MorphArrayStruct))
  (bind (_sectionname_2 _morphname_2) (Utilities|Struct|BreakMorphItemStruct MorphArrayStruct))
  (bind _returnvalue (Utilities|String|ToString(Float) _minimumvalue))
  (bind _returnvalue_2 (Utilities|String|ToString(Float) _maximumvalue))
  (bind _returnvalue_3 (Utilities|String|ToString(Name) _readablename))
  (bind _returnvalue_4 (Utilities|String|ToString(Name) _morphname))
  (bind _returnvalue_5 (Utilities|String|ToString(Float) _defaultvalue))
  (bind _returnvalue_6 (Utilities|String|ToString(Name) _sectionname_2))
  (bind _returnvalue_7 (Utilities|String|Append _returnvalue_3 "#" _returnvalue_4 "#" _returnvalue "#" _returnvalue_2 "#" _returnvalue_5))
  (bind _returnvalue_8 (Utilities|String|Append "*" _returnvalue_6 "*"))
  (bind _output_get (LocalVariables|SetArray (.StringArray (Class|VictoryBPFunctionLibrary|LoadStringArrayfromFile (Utilities|String|Append (Class|HnomerBPLibraryPluginBPLibrary|GetGameContentDirPath) "CustomAssets/morphslist.txt") true))))
  (bind (_array_element _array_index) (Utilities|Array|ForEachLoopwithBreak _output_get :!label _label)
    (:LoopBody
      (if (Utilities|String|Contains _array_element (Utilities|String|ToString(Name) _morphname_2))
        (bind _index (Utilities|FlowControl|ForLoopwithBreak _array_index 0)
          (:LoopBody
            (if (>= (Utilities|String|FindSubstring (Utilities|Array|Get(acopy) (LocalVariables|GetArray) _index) "*") 0)
              (if (Utilities|Name|Equal(Name) (Utilities|String|StringToName (Utilities|Array|Get(acopy) (Class|VictoryBPFunctionLibrary|StringExplodeString (Utilities|Array|Get(acopy) (LocalVariables|GetArray) _index) "*" 0 false) 1)) _sectionname)
                (Utilities|Array|SetArrayElem (LocalVariables|GetArray) _array_index _returnvalue_7 true)
                (bind _returnvalue_9 (Class|VictoryBPFunctionLibrary|FileIOSaveStringArraytoFile (Utilities|String|Append (Class|HnomerBPLibraryPluginBPLibrary|GetGameContentDirPath) "CustomAssets/") "morphslist.txt" (LocalVariables|GetArray) true :!label _label_2))
                (return _returnvalue_9)
                (else
                  (Utilities|Array|RemoveIndex (LocalVariables|GetArray) _index)
                  (goto _label Break))))))))
    (:Completed
      (if (!= (Utilities|Array|FindItem (LocalVariables|GetArray) _returnvalue_8) -1)
        (Utilities|Array|Insert (LocalVariables|GetArray) _returnvalue_7 (+ (Utilities|Array|FindItem (LocalVariables|GetArray) _returnvalue_8) 1))
        (goto _label_2)
        (else
          (Utilities|Array|Add (LocalVariables|GetArray) _returnvalue_8)
          (Utilities|Array|Add (LocalVariables|GetArray) _returnvalue_7)
          (goto _label_2))))))

(fn GetMorphList
  (return (Variables|/Game/Blueprints/GameInstance_BP.GameInstance_BP_C|GetMorphListMorphItemsStructArray (MyFNCLib|GetCustomGameInstance))))

(fn GetCustomizationManager
  (bind _outactors (Actor|GetAllActorswithTag 0 "CustomizationManager"))
  (if (> (Utilities|Array|Length _outactors) 0)
    (bind _ascustomization_manager_bp (Utilities|Casting|CastToCustomizationManager_BP (Utilities|Array|Get(acopy) _outactors))
      (:then
        (return true _ascustomization_manager_bp))
      (:CastFailed
        _)))
  (return false 0))

(fn SetShowCursorTooltip
  (params (On/Off :type Boolean) (InText :type Text) (Z%20Order :type Integer))
  (bind _widget_reference (MyFNCLib|OpenWidget "/Game/Blueprints/HUD/Customization/TooltipWidget_BP.TooltipWidget_BP_C" true Z%20Order))
  (bind _astooltip_widget_bp (Utilities|Casting|CastToTooltipWidget_BP _widget_reference))
  (Default|SetShowTooltipTextonCursor _astooltip_widget_bp On/Off InText))

(fn SetSamkaBodyPartsColors!GamingLevelOnly!
  (params (BodyPartsColorsStruct :type Body%20Parts%20Colors%20Struct%20Structure))
  (bind (_isfound _objectmanager) (MyFNCLib|GetObjectManager))
  (if _isfound
    (Default|OMSetSamkaBodyPartsColors _objectmanager BodyPartsColorsStruct)
    (return true)
    (else
      (return false))))

(fn GetSoundManager
  (bind _custom_game_instance (MyFNCLib|GetCustomGameInstance))
  (bind _soundmanager (Variables|/Game/Blueprints/GameInstance_BP.GameInstance_BP_C|GetSoundManager _custom_game_instance))
  (return (Utilities|IsValid _soundmanager) _soundmanager))

(fn SetPhysicsEnabled
  (params (IsEnabled :type Boolean))
  (bind (_isfound _objectmanager) (MyFNCLib|GetObjectManager))
  (if _isfound
    (Default|OMSetPhysicsEnabled _objectmanager IsEnabled)
    (else
      (bind (_isfound_2 _customizationmanager) (MyFNCLib|GetCustomizationManager))
      (if _isfound_2
        (Default|CMSetPhysicsEnabled _customizationmanager IsEnabled)))))

(fn CreateNewSettingsSaveObject
  (bind (_windows_ _mac) (Class|VictoryBPFunctionLibrary|OperatingSystemGetCurrentPlatform))
  (bind _returnvalue (SaveGame|CreateSaveGameObject "/Game/Blueprints/SettingsSaveClass_BP.SettingsSaveClass_BP_C"))
  (Utilities|FlowControl|Sequence
    (:then_0
      (if _windows_
        (if (.IsNvidia (Class|VictoryBPFunctionLibrary|GetUserDisplayAdapterBrand))
          (LocalVariables|SetSettingsStruct (Utilities|Struct|MakeSettingsSave_Struct true false))
          (else
            (LocalVariables|SetSettingsStruct (Utilities|Struct|MakeSettingsSave_Struct true false false))))
        (elif _mac
          (LocalVariables|SetSettingsStruct (Utilities|Struct|MakeSettingsSave_Struct true true false))
          (else
            (LocalVariables|SetSettingsStruct (Utilities|Struct|MakeSettingsSave_Struct true true false))))))
    (:then_1
      (Variables|/Game/Blueprints/SettingsSaveClass_BP.SettingsSaveClass_BP_C|SetSettingsStruct _returnvalue (LocalVariables|GetSettingsStruct))
      (return _returnvalue))))

(fn GetCurrentULC
  (bind (_isfound _upperlevelclassmanager) (MyFNCLib|GetULCManager))
  (if _isfound
    (return (Variables|/Game/Blueprints/Managers/UpperLevelClassManager_BP.UpperLevelClassManager_BP_C|GetCurrentLevelClass _upperlevelclassmanager))))

(fn ModifyLocationbyVectorLength
  (params (Location :type Vector) (Vector :type Vector) (Length :type Float%20%28single-precision%29))
  (return (+ Location (* Vector Length))))

(fn GetNormalizedFloatfromVectorRange
  (params (Vector1 :type Vector) (Vector2 :type Vector) (VectorInBetween :type Vector))
  (return (Math|Float|NormalizetoRange (Math|Vector|VectorLength (- Vector1 VectorInBetween)) 0.0 (Math|Vector|VectorLength (- Vector1 Vector2)))))

(fn PlayUISound
  (params (Sound :type Sound%20Base%20Object%20Reference) (PitchMultiplier :type Float%20%28single-precision%29) (StartTime :type Float%20%28single-precision%29) (ConcurrencySettings :type Sound%20Concurrency%20Object%20Reference))
  (bind _asgame_instance_bp (Utilities|Casting|CastToGameInstance_BP (Game|GetGameInstance)))
  (Audio|PlaySound2D _asgame_instance_bp Sound (Variables|/Game/Blueprints/GameInstance_BP.GameInstance_BP_C|GetUIVolume _asgame_instance_bp) PitchMultiplier StartTime ConcurrencySettings 0))

(fn Fadein
  (bind _widget_reference (MyFNCLib|OpenWidget "/Game/Blueprints/HUD/CustomUIComponents/Fade_Widget.Fade_Widget_C" true 999))
  (bind _asfade_widget (Utilities|Casting|CastToFade_Widget _widget_reference))
  (Default|Fade _asfade_widget true))

(fn FadeOut
  (bind _widget_reference (MyFNCLib|OpenWidget "/Game/Blueprints/HUD/CustomUIComponents/Fade_Widget.Fade_Widget_C" true 999))
  (bind _asfade_widget (Utilities|Casting|CastToFade_Widget _widget_reference))
  (Default|Fade _asfade_widget false))

(fn PlayStunnedBlurEffect
  (bind _widgetobject (MyFNCLib|GetWidget "/Game/Blueprints/HUD/InGameHUD/InGameHUD.InGameHUD_C"))
  (bind _asin_game_hud (Utilities|Casting|CastToInGameHUD _widgetobject))
  (Default|PlayBlurStunEffect _asin_game_hud))

(fn GetDistance
  (params (Point%20A :type Vector) (Point%20B :type Vector))
  (return (Math|Vector|VectorLength (- Point%20A Point%20B))))