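; Customization manager actor that drives the Samka character's customization scene: camera switching, morph targets, skin, hair and eye colors, and physics toggling.
; On BeginPlay it retries until the Samka actor is valid, then binds delegates and applies the saved PhysX setting.
; It relays body-part hover and click events through its own dispatchers.
; Thumbnails are built as textures from render-target pixels.
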(event EventBeginPlay
  (bind _samkacustomizationactor (Variables|Default|GetSamkaCustomizationActor))
  (Utilities|IsValid _samkacustomizationactor :!label _label
    (:Is%20Valid
      (Variables|Default|SetSamkaSkeletal (Variables|/Game/Blueprints/Customization/Customization_Samka_BP.Customization_Samka_BP_C|GetSamka _samkacustomizationactor))
      (CallFunction|InitSamkaDelegates)
      (bind (_settings_loaded _settingsstruct) (CallFunction|GetDatafromSettingsSaveObject))
      (if _settings_loaded
        (CallFunction|CMSetPhysicsEnabled (.IsEnablePhysX (Utilities|Struct|BreakSettingsSave_Struct _settingsstruct)))))
    (:Is%20Not%20Valid
      (Utilities|FlowControl|Delay 0.2)
      (goto _label))))

(event Collision|EventActorBeginOverlap
  (params (OtherActor :type Actor%20Object%20Reference)))

(event EventTick
  (params (DeltaSeconds :type Float%20%28single-precision%29)))

(fn ConstructionScript
  (Rendering|SetVisibility (Variables|Default|GetDefaultSceneRoot) false true))

(fn CMChangeCamera
  (params (CameraIndex :type Integer))
  (switch int CameraIndex
    (:1
      (LocalVariables|SetNewCamera (Variables|Default|GetCameraHead)))
    (:2
      (LocalVariables|SetNewCamera (Variables|Default|GetCameraChest)))
    (:3
      (LocalVariables|SetNewCamera (Variables|Default|GetCameraHips)))
    (:4
      (LocalVariables|SetNewCamera (Variables|Default|GetCameraLegs)))
    (:5
      (LocalVariables|SetNewCamera (Variables|Default|GetCameraOverview))))
  (Default|SwitchtoThisCamera (LocalVariables|GetNewCamera)))

(fn CMSetSamkaMorphs
  (params (MorphsStructArray :type Array%20of%20Morph%20Item%20Struct%20Structures))
  (for _array_element MorphsStructArray
    (Components|SkeletalMesh|SetMorphTarget (Variables|Default|GetSamkaSkeletal) (.MorphName (Utilities|Struct|BreakMorphItemStruct _array_element)) (.CurrentValue (Utilities|Struct|BreakMorphItemStruct _array_element)) true)))

(fn InitSamkaDelegates
  (bind _samkacustomizationactor (Variables|Default|GetSamkaCustomizationActor))
  (Utilities|FlowControl|Sequence
    (:then_0
      (EventDispatchers|BindEventtoOnBeginCursorOverlapSamkaBodyPartDelegate _samkacustomizationactor (EventDispatchers|CreateEvent :!event OnSamkaCursorBeginOverlapBodyPartDelegate)))
    (:then_1
      (EventDispatchers|BindEventtoOnEndCursorOverlapSamkaBodyPartDelegate _samkacustomizationactor (EventDispatchers|CreateEvent :!event OnSamkaCursorEndOverlapBodyPartDelegate)))
    (:then_2
      (EventDispatchers|BindEventtoOnClickedSamkaBodyPartDelegate _samkacustomizationactor (EventDispatchers|CreateEvent :!event OnSamkaClickedBodyPartDelegate)))))

(fn OnSamkaCursorBeginOverlapBodyPartDelegate
  (params (BodyPart :type BodyParts_Enum%20Enum :default "NewEnumerator0"))
  (Default|CallOnSamkaCursorBeginOverlapBodyPartDelegate BodyPart))

(fn OnSamkaCursorEndOverlapBodyPartDelegate
  (Default|CallOnSamkaCursorEndOverlapBodyPartDelegate))

(fn OnSamkaClickedBodyPartDelegate
  (params (BodyPart :type BodyParts_Enum%20Enum :default "NewEnumerator0"))
  (Default|CallOnSamkaClickedBodyPartDelegate BodyPart))

(fn CMCaptureThumbnailPicture
  (bind _returnvalue (Class|HnomerBPLibraryPluginBPLibrary|GetPixelsArrayfromRenderTarget "/Game/Blueprints/HUD/Customization/ThumbnailRenderTexture_Demo.ThumbnailRenderTexture_Demo"))
  (bind _returnvalue_2 (Class|HnomerBPLibraryPluginBPLibrary|GetTexture2DfromPixelsArray _returnvalue 512 512))
  (return _returnvalue_2))

(fn CMApplyColortoBodyPart
  (params (Body%20Part :type ColorBodyParts_ENum%20Enum :default "NewEnumerator2") (Color :type Linear%20Color%20Structure))
  (bind _returnvalue (Math|Conversions|ToVector(LinearColor) Color))
  (bind _samkacustomizationactor (Variables|Default|GetSamkaCustomizationActor))
  (bind _samka (Variables|/Game/Blueprints/Customization/Customization_Samka_BP.Customization_Samka_BP_C|GetSamka _samkacustomizationactor))
  (switch Utilities|FlowControl|Switch|SwitchonColorBodyParts_ENum Body%20Part
    (:NewEnumerator0
      (Rendering|Material|SetVectorParameterValueonMaterials _samka "SkinColorAlt" _returnvalue))
    (:NewEnumerator1
      (Rendering|Material|SetVectorParameterValueonMaterials (Variables|/Game/Blueprints/Customization/Customization_Samka_BP.Customization_Samka_BP_C|GetHair1 _samkacustomizationactor) "HairColorAlt" _returnvalue))
    (:NewEnumerator3
      (Rendering|Material|SetVectorParameterValueonMaterials _samka "EyesColorAlt" _returnvalue))))

(fn CMSetPhysicsEnabled
  (params (IsEnabled :type Boolean))
  (Physics|SetSimulatePhysics (Variables|/Game/Blueprints/Customization/Customization_Samka_BP.Customization_Samka_BP_C|GetSamka (Variables|Default|GetSamkaCustomizationActor)) IsEnabled))