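; Manager actor that switches between upper level class instances, tracking them in an array along with the current one.
; On a switch, it deletes the outgoing instance when the saved settings enable low memory mode, and otherwise hides it for reuse.
; It then looks up the requested class among cached instances, calling ULCLoad on a valid match or creating a new instance, and makes the result current.
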(event EventBeginPlay)

(event Collision|EventActorBeginOverlap
  (params (OtherActor :type Actor%20Object%20Reference)))

(event EventTick
  (params (DeltaSeconds :type Float%20%28single-precision%29)))

(fn ConstructionScript
  (Rendering|SetVisibility (Variables|Default|GetDefaultSceneRoot) false true))

(fn ULCMSwitchLevelClass
  (params (LevelClass :type Base%20Upper%20Level%20Class%20BP%20Class%20Reference))
  (bind (_isfound _levelclassreference) (CallFunction|ULCMGetLevelClassReferencebyClass LevelClass))
  (bind _levelclassesarray (Variables|Default|GetLevelClassesArray))
  (if (!= (Variables|Default|GetCurrentLevelClass) 0)
    (bind _settingsstruct (CallFunction|GetDatafromSettingsSaveObject))
    (if (.IsLowMemoryMode (Utilities|Struct|BreakSettingsSave_Struct _settingsstruct))
      (Utilities|Array|RemoveItem (Variables|Default|GetLevelClassesArray) (Variables|Default|GetCurrentLevelClass))
      (CallFunction|DeleteULCInstance (Variables|Default|GetCurrentLevelClass))
      (else
        (CallFunction|HideULCInstance (Variables|Default|GetCurrentLevelClass)))))
  (if _isfound
    (bind _level (Default|ULCLoad _levelclassreference))
    (Utilities|Array|Add _levelclassesarray _level)
    (Variables|Default|SetCurrentLevelClass _level)
    (else
      (bind _level_2 (CallFunction|CreateULCInstance LevelClass))
      (Utilities|Array|Add _levelclassesarray _level_2)
      (Variables|Default|SetCurrentLevelClass _level_2))))

(fn ULCMGetLevelClassReferencebyClass
  (params (LevelClass :type Base%20Upper%20Level%20Class%20BP%20Class%20Reference))
  (bind (_array_element _array_index) (Utilities|Array|ForEachLoopwithBreak (Variables|Default|GetLevelClassesArray))
    (:LoopBody
      (if (== (Utilities|GetClass _array_element) LevelClass)
        (Utilities|IsValid _array_element
          (:Is%20Valid
            (return true _array_element))
          (:Is%20Not%20Valid
            (Utilities|Array|RemoveIndex (Variables|Default|GetLevelClassesArray) _array_index)
            (return false 0)))))
    (:Completed
      (return false 0))))