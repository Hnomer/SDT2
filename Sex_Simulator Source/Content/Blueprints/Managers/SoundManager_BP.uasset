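; Sound manager actor that holds the game's master, character, ambient, music and UI volume levels.
; On BeginPlay it loads each level from the settings save object and applies it through its setters.
; Each setter broadcasts a change delegate, with category volumes scaled by master, and a master change rebroadcasts every category.
; Only UI volume has a getter here, returning the master-scaled value.
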(event EventBeginPlay
  (bind _settingsstruct (CallFunction|GetDatafromSettingsSaveObject))
  (CallFunction|SetMasterVolume (.MasterVolume (Utilities|Struct|BreakSettingsSave_Struct _settingsstruct)))
  (CallFunction|SetCharactersVolume (.CharactersVolume (Utilities|Struct|BreakSettingsSave_Struct _settingsstruct)))
  (CallFunction|SetAmbientVolume (.AmbientVolume (Utilities|Struct|BreakSettingsSave_Struct _settingsstruct)))
  (CallFunction|SetMusicVolume (.MusicVolume (Utilities|Struct|BreakSettingsSave_Struct _settingsstruct)))
  (CallFunction|SetUIVolume (.UIVolume (Utilities|Struct|BreakSettingsSave_Struct _settingsstruct))))

(event Collision|EventActorBeginOverlap
  (params (OtherActor :type Actor%20Object%20Reference)))

(event EventTick
  (params (DeltaSeconds :type Float%20%28single-precision%29)))

(fn ConstructionScript
  (Rendering|SetVisibility (Variables|Default|GetDefaultSceneRoot) false true))

(fn SetMasterVolume
  (params (MasterVolume :type Float%20%28single-precision%29))
  (bind _output_get (Variables|Default|SetMasterVolume MasterVolume))
  (CallFunction|SetCharactersVolume (Variables|Default|GetCharactersVolume))
  (CallFunction|SetAmbientVolume (Variables|Default|GetAmbientVolume))
  (CallFunction|SetMusicVolume (Variables|Default|GetMusicVolume))
  (CallFunction|SetUIVolume (Variables|Default|GetUIVolume))
  (Default|CallSoundManageronMasterVolumeChangedDelegate _output_get))

(fn SetCharactersVolume
  (params (Volume :type Float%20%28single-precision%29))
  (bind _output_get (Variables|Default|SetCharactersVolume Volume))
  (Default|CallSoundManageronCharactersVolumeChangedDelegate (* _output_get (Variables|Default|GetMasterVolume))))

(fn SetAmbientVolume
  (params (Volume :type Float%20%28single-precision%29))
  (bind _output_get (Variables|Default|SetAmbientVolume Volume))
  (Default|CallSoundManageronAmbientVolumeChangedDelegate (* _output_get (Variables|Default|GetMasterVolume))))

(fn SetMusicVolume
  (params (Volume :type Float%20%28single-precision%29))
  (bind _output_get (Variables|Default|SetMusicVolume Volume))
  (Default|CallSoundManageronMusicVolumeChangedDelegate (* _output_get (Variables|Default|GetMasterVolume))))

(fn SetUIVolume
  (params (UIVolume :type Float%20%28single-precision%29))
  (bind _output_get (Variables|Default|SetUIVolume UIVolume))
  (Default|CallSoundManageronUIVolumeChangedDelegate (* _output_get (Variables|Default|GetMasterVolume))))

(fn GetUIVolume
  (return (* (Variables|Default|GetUIVolume) (Variables|Default|GetMasterVolume))))