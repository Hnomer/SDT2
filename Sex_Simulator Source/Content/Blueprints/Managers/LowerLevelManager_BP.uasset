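; Lower-level manager actor that loads, shows, hides and unloads streaming level instances by name, with an optional loading screen.
; LLCM_LoadLevel reveals an already loaded level or creates an instance at the origin, tracks it in a StreamingLevels array, then fires a loaded-and-visible delegate.
; On a switch, ManagePreviousLevel unloads the previous level in low-memory mode from saved settings, otherwise just hides it for reuse.
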(event EventBeginPlay)

(event Collision|EventActorBeginOverlap
  (params (OtherActor :type Actor%20Object%20Reference)))

(event EventTick
  (params (DeltaSeconds :type Float%20%28single-precision%29)))

(fn ConstructionScript
  (Rendering|SetVisibility (Variables|Default|GetDefaultSceneRoot) false true))

(fn LLCMLoadLevel
  (params (Level%20Name :type String) (ShouldBeVisibleAfterLoading :type Boolean) (LoadingScreen :type Boolean) (ZOrder :type Integer) (Don'tDisableLoadingScreen :type Boolean))
  (bind (_isfound _level) (LevelController|LLCMGetLoadedLevel Level%20Name))
  (Variables|Default|SetIsDisableLoadingScreenAfterLevelIsLoaded (not Don'tDisableLoadingScreen))
  (if _isfound
    (if (Utilities|Enum|Equal(Enum) (Variables|LevelController|GetCurrentLevelName) Level%20Name)
      _
      (else
        (LevelController|ManagePreviousLevel)
        (Variables|LevelController|SetCurrentLevelName Level%20Name)
        (CallFunction|SetLoadingScreenEnabled true false)))
    (Variables|/Script/Engine.LevelStreaming|SetbShouldBeVisible _level true)
    (Default|CallLLCMonLevelLoadedandVisibleDelegate)
    (LevelController|OnLevelLoaded)
    (return true _level)
    (else
      (LevelController|ManagePreviousLevel)
      (bind (_boutsuccess _levelobject) (LevelController|LoadLevelIntoMemory Level%20Name ShouldBeVisibleAfterLoading))
      (if _boutsuccess
        (LevelController|AddtoStreamingLevelsArray _levelobject)
        (if LoadingScreen
          (CallFunction|SetLoadingScreenEnabled true false ZOrder)
          (EventDispatchers|BindEventtoOnLevelLoaded _levelobject (EventDispatchers|CreateEvent :!event OnLevelLoaded))
          (Variables|LevelController|SetCurrentLevelName Level%20Name)
          (return _boutsuccess _levelobject))
        (else
          (return _boutsuccess _levelobject))))))

(fn OnLevelLoaded
  (if (Variables|Default|GetIsDisableLoadingScreenAfterLevelIsLoaded)
    (CallFunction|SetLoadingScreenEnabled false false))
  (Default|CallLLCMonLevelLoadedandVisibleDelegate))

(fn LoadLevelIntoMemory
  (params (LevelName :type String) (ShouldBeVisibleAfterLoading :type Boolean))
  (bind (_boutsuccess _returnvalue) (Class|LevelStreamingKismet|LoadLevelInstance LevelName (Math|Vector|MakeVector 0.0 0.0 0.0) (Math|Rotator|MakeRotator 0.0 0.0 0.0)))
  (Variables|/Script/Engine.LevelStreaming|SetbShouldBeVisible _returnvalue ShouldBeVisibleAfterLoading)
  (return _boutsuccess _returnvalue))

(fn LLCMUnloadLevel
  (params (LevelName :type String))
  (bind (_isfound _level) (LevelController|LLCMGetLoadedLevel LevelName))
  (if _isfound
    (Class|VictoryBPFunctionLibrary|UnloadStreamingLevel _level)
    (LevelController|RemovefromStreamingLevelsArray _level))
  (return true))

(fn LLCMGetLoadedLevel
  (params (LevelName :type String))
  (bind _array_element (Utilities|Array|ForEachLoopwithBreak (Variables|LevelController|GetStreamingLevels))
    (:LoopBody
      (if (Utilities|String|Contains (Utilities|String|ToString(Name) (Class|LevelStreaming|GetWorldAssetPackageFName _array_element)) LevelName false true)
        (return true _array_element)))
    (:Completed
      (return false 0))))

(fn AddtoStreamingLevelsArray
  (params (Level :type Level%20Streaming%20Kismet%20Object%20Reference%20%28by%20ref%29))
  (Utilities|Array|Add (Variables|LevelController|GetStreamingLevels) Level))

(fn RemovefromStreamingLevelsArray
  (params (Level :type Level%20Streaming%20Kismet%20Object%20Reference%20%28by%20ref%29))
  (bind _returnvalue (Utilities|Array|RemoveItem (Variables|LevelController|GetStreamingLevels) Level))
  (return _returnvalue))

(fn LLCMHideLevel
  (params (LevelName :type String))
  (bind (_isfound _level) (LevelController|LLCMGetLoadedLevel LevelName))
  (if _isfound
    (Variables|/Script/Engine.LevelStreaming|SetbShouldBeVisible _level false)))

(fn ManagePreviousLevel
  (bind _currentlevelname (Variables|LevelController|GetCurrentLevelName))
  (if (Utilities|Enum|NotEqual(Enum) (Variables|LevelController|GetCurrentLevelName) "")
    (bind _settingsstruct (CallFunction|GetDatafromSettingsSaveObject))
    (if (.IsLowMemoryMode (Utilities|Struct|BreakSettingsSave_Struct _settingsstruct))
      (LevelController|LLCMUnloadLevel _currentlevelname)
      (else
        (LevelController|LLCMHideLevel _currentlevelname)))))