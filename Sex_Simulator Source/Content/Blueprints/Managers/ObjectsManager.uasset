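; Manager actor for an adult game that fronts the male (Samec) and female (Samka) character actors for morphs, colors, anatomy sizing, voice pitch and physics.
; Each tick compares head-socket distance to genital length to detect oral contact and fire events.
; When contact ends, it can spawn a saliva cable from the nearest bone.
; It also switches and shakes the player camera, and swaps in translucent materials for POV views.
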(event EventBeginPlay
  (bind (_settings_loaded _settingsstruct) (CallFunction|GetDatafromSettingsSaveObject))
  (if _settings_loaded
    (CallFunction|OMSetPhysicsEnabled (.IsEnablePhysX (Utilities|Struct|BreakSettingsSave_Struct _settingsstruct)))))

(event Collision|EventActorBeginOverlap
  (params (OtherActor :type Actor%20Object%20Reference)))

(event EventTick
  (params (DeltaSeconds :type Float%20%28single-precision%29))
  (CallFunction|CalculateSucking)
  (CallFunction|ShakePlayerCamera))

(fn ConstructionScript
  (Rendering|SetVisibility (Variables|Default|GetDefaultSceneRoot) false true))

(fn OMGetPActorSocketTransform
  (params (Porn%20Actor :type PornActors_Enum%20Enum :default "NewEnumerator0") (SocketName :type Name) (TransformSpace :type ERelativeTransformSpace%20Enum :default "RTS_World"))
  (bind _samecactor (Variables|Default|GetSamecActor))
  (switch Utilities|FlowControl|Switch|SwitchonPornActors_Enum Porn%20Actor
    (:NewEnumerator0
      (return (Transformation|GetSocketTransform (Variables|/Game/Blueprints/Actors/Samka_BP.Samka_BP_C|GetSamkaSkeletalMesh (Variables|Default|GetSamkaActor)) SocketName TransformSpace)))
    (:NewEnumerator1
      (return (Transformation|GetSocketTransform (Variables|/Script/Engine.Actor|GetRootComponent _samecactor) SocketName TransformSpace)))
    (:NewEnumerator2
      (return (Transformation|GetSocketTransform (Variables|/Game/Blueprints/Actors/Samec_BP.Samec_BP_C|GetShadowSamec _samecactor) SocketName TransformSpace)))))

(fn OMSetDickScale
  (params (IsBetween%200-1 :type Boolean) (AddToCurrent :type Boolean) (Scale :type Float%20%28single-precision%29))
  (bind _samecactor (Variables|Default|GetSamecActor))
  (if IsBetween%200-1
    (Default|SetDickScale _samecactor AddToCurrent (CallFunction|ConvertNormalizedFloattoRange Scale (Variables|/Game/Blueprints/Actors/Samec_BP.Samec_BP_C|GetMinDickScale _samecactor) (Variables|/Game/Blueprints/Actors/Samec_BP.Samec_BP_C|GetMaxDickScale _samecactor)))
    (else
      (Default|SetDickScale _samecactor AddToCurrent Scale)))
  (Default|CallEDonDickScaleChanged (CallFunction|OMGetDickScale) (CallFunction|OMGetDickNormalizedScale)))

(fn OMSetDickLength
  (params (IsBetween%200-1 :type Boolean) (IsAddToCurrent :type Boolean) (Length :type Float%20%28single-precision%29))
  (bind _samecactor (Variables|Default|GetSamecActor))
  (bind _maxdicklength (Variables|/Game/Blueprints/Actors/Samec_BP.Samec_BP_C|GetMaxDickLength _samecactor))
  (bind _mindicklength (Variables|/Game/Blueprints/Actors/Samec_BP.Samec_BP_C|GetMinDickLength _samecactor))
  (bind _rangedvalue (CallFunction|ConvertNormalizedFloattoRange Length _mindicklength _maxdicklength))
  (if IsBetween%200-1
    (Default|SetDickLength _samecactor IsAddToCurrent _rangedvalue)
    (Default|CallEDonDickLengthChanged _rangedvalue)
    (else
      (Default|SetDickLength _samecactor IsAddToCurrent Length)
      (Default|CallEDonDickLengthChanged Length))))

(fn OMGetDickScale
  (return (Variables|/Game/Blueprints/Actors/Samec_BP.Samec_BP_C|GetDickScale (Variables|Default|GetSamecActor))))

(fn OMGetDickMaximumandMinimumScale
  (bind _samecactor (Variables|Default|GetSamecActor))
  (return (Variables|/Game/Blueprints/Actors/Samec_BP.Samec_BP_C|GetMinDickScale _samecactor) (Variables|/Game/Blueprints/Actors/Samec_BP.Samec_BP_C|GetMaxDickScale _samecactor)))

(fn OMIsDickAttachedTomouth
  (return (Variables|/Game/Blueprints/Actors/Samec_BP.Samec_BP_C|GetIsDickAttachedToMouth (Variables|Default|GetSamecActor))))

(fn OMResetActors
  (Class|HnomerBPLibraryPluginBPLibrary|ResetActor (Variables|Default|GetSamecActor))
  (Class|HnomerBPLibraryPluginBPLibrary|ResetActor (Variables|Default|GetSamkaActor)))

(fn OMSetSamkaMorphs
  (params (MorphsArray :type Array%20of%20Morph%20Item%20Struct%20Structures))
  (bind _samkaactor (Variables|Default|GetSamkaActor))
  (bind _samkaskeletalmesh (Variables|/Game/Blueprints/Actors/Samka_BP.Samka_BP_C|GetSamkaSkeletalMesh _samkaactor))
  (Utilities|IsValid _samkaactor
    (:Is%20Valid
      (for _array_element (Variables|/Script/Engine.SkeletalMesh|GetMorphTargets (Variables|/Script/Engine.SkinnedMeshComponent|GetSkeletalMesh _samkaskeletalmesh))
        (Components|SkeletalMesh|SetMorphTarget _samkaskeletalmesh (Utilities|String|StringToName (Utilities|GetObjectName _array_element)) 0.0 true)
        (Default|CallEDonSamkaCharacterChanged))
      (for _array_element_2 MorphsArray
        (Components|SkeletalMesh|SetMorphTarget _samkaskeletalmesh (.MorphName (Utilities|Struct|BreakMorphItemStruct _array_element_2)) (.CurrentValue (Utilities|Struct|BreakMorphItemStruct _array_element_2)) true)))))

(fn OMSetSamkaBodyPartsColors
  (params (BodyPartsColorsStruct :type Body%20Parts%20Colors%20Struct%20Structure))
  (bind (_skin _hair _eyes) (Utilities|Struct|BreakBodyPartsColors_Struct BodyPartsColorsStruct))
  (bind _samkaactor (Variables|Default|GetSamkaActor))
  (bind _returnvalue (Math|Conversions|ToVector(LinearColor) _hair))
  (bind _samka (Variables|/Game/Blueprints/Actors/Samka_BP.Samka_BP_C|GetSamka _samkaactor))
  (Utilities|FlowControl|Sequence
    (:then_0
      (Rendering|Material|SetVectorParameterValueonMaterials _samka "SkinColorAlt" (Math|Conversions|ToVector(LinearColor) _skin))
      (Rendering|Material|SetVectorParameterValueonMaterials _samka "EyesColorAlt" (Math|Conversions|ToVector(LinearColor) _eyes)))
    (:then_1
      (Rendering|Material|SetVectorParameterValueonMaterials (Variables|/Game/Blueprints/Actors/Samka_BP.Samka_BP_C|GetHairShadowMask _samkaactor) "HairColorAlt" _returnvalue)
      (Rendering|Material|SetVectorParameterValueonMaterials (Variables|/Game/Blueprints/Actors/Samka_BP.Samka_BP_C|GetHairTrans _samkaactor) "HairColorAlt" _returnvalue))))

(fn OMSetSamecSkinColor
  (params (Color :type Linear%20Color%20Structure))
  (Rendering|Material|SetVectorParameterValueonMaterials (Variables|/Game/Blueprints/Actors/Samec_BP.Samec_BP_C|GetSamec_D_v1 (Variables|Default|GetSamecActor)) "SkinColorAlt" (Math|Conversions|ToVector(LinearColor) Color)))

(fn OMSetPhysicsEnabled
  (params (IsEnabled :type Boolean))
  (Physics|SetSimulatePhysics (Variables|/Game/Blueprints/Actors/Samka_BP.Samka_BP_C|GetSamka (Variables|Default|GetSamkaActor)) IsEnabled))

(fn OMSetSamkaVoicePitchMultiplier
  (params (NewPitchMultiplier :type Float%20%28single-precision%29))
  (Default|SetVoicePitchMultiplier (Variables|Default|GetSamkaActor) NewPitchMultiplier))

(fn OMGetDickTotalLength
  (bind _dicklength (Default|GetDickLength (Variables|Default|GetSamecActor)))
  (return _dicklength))

(fn OMGetDickVector
  (bind _transform (CallFunction|OMGetPActorSocketTransform "NewEnumerator1" "Gen1" "RTS_World"))
  (bind _location (Math|Transform|BreakTransform _transform))
  (return _location (Math|Vector|Normalize (- (.Location (Math|Transform|BreakTransform (CallFunction|OMGetPActorSocketTransform "NewEnumerator1" "Gen6" "RTS_World"))) _location))))

(fn OMGetDickNormalizedScale
  (bind _samecactor (Variables|Default|GetSamecActor))
  (return (Math|Float|NormalizetoRange (Variables|/Game/Blueprints/Actors/Samec_BP.Samec_BP_C|GetDickScale _samecactor) (Variables|/Game/Blueprints/Actors/Samec_BP.Samec_BP_C|GetMinDickScale _samecactor) (Variables|/Game/Blueprints/Actors/Samec_BP.Samec_BP_C|GetMaxDickScale _samecactor))))

(fn OMStartErection
  (Default|SamecStartErection (Variables|Default|GetSamecActor)))

(fn OMSetErectionSpeed
  (params (ErectionSpeedPerSecond :type Float%20%28single-precision%29))
  (Variables|/Game/Blueprints/Actors/Samec_BP.Samec_BP_C|SetErectionSpeedPerSecond (Variables|Default|GetSamecActor) ErectionSpeedPerSecond))

(fn OMSetErectionProperties
  (params (ErectedDickLength :type Float%20%28single-precision%29) (ErectedDickSize :type Float%20%28single-precision%29) (ErectionSpeedPerSecond :type Float%20%28single-precision%29))
  (bind _samecactor (Variables|Default|GetSamecActor))
  (Variables|/Game/Blueprints/Actors/Samec_BP.Samec_BP_C|SetErectedDickLength _samecactor ErectedDickLength)
  (Variables|/Game/Blueprints/Actors/Samec_BP.Samec_BP_C|SetErectedDickSize _samecactor ErectedDickSize)
  (Variables|/Game/Blueprints/Actors/Samec_BP.Samec_BP_C|SetErectionSpeedPerSecond _samecactor ErectionSpeedPerSecond))

(fn OMSetMalePOV
  (params (On%20/Off :type Boolean))
  (bind _samkaactor (Variables|Default|GetSamkaActor))
  (bind _samecactor (Variables|Default|GetSamecActor))
  (bind _samec_d_v1 (Variables|/Game/Blueprints/Actors/Samec_BP.Samec_BP_C|GetSamec_D_v1 _samecactor))
  (if On%20/Off
    (bind _asmaterial_instance (Utilities|Casting|CastToMaterialInstance (Rendering|Material|GetMaterial _samec_d_v1 9)))
    (Variables|Default|SetSamecTorsoMaterial _asmaterial_instance)
    (Rendering|Material|SetMaterial _samec_d_v1 9 (Variables|Default|GetTranslucentMaterialInstance))
    (Variables|/Game/Blueprints/Actors/Samka_BP.Samka_BP_C|SetIsLockHeadMovement _samkaactor true)
    (Variables|/Game/Blueprints/Actors/Samka_BP.Samka_BP_C|SetTargetHeadAngle _samkaactor 2e+01)
    (else
      (Rendering|Material|SetMaterial _samec_d_v1 9 (Variables|Default|GetSamecTorsoMaterial))
      (Variables|/Game/Blueprints/Actors/Samka_BP.Samka_BP_C|SetIsLockHeadMovement _samkaactor false)
      (Variables|/Game/Blueprints/Actors/Samka_BP.Samka_BP_C|SetTargetHeadAngle _samkaactor (Variables|/Game/Blueprints/Actors/Samka_BP.Samka_BP_C|GetConstMaxHeadAngle _samkaactor)))))

(fn OMSetFemalePOV
  (params (On%20/%20Off :type Boolean))
  (bind _samkaactor (Variables|Default|GetSamkaActor))
  (bind _translucentmaterialinstance (Variables|Default|GetTranslucentMaterialInstance))
  (bind _samka (Variables|/Game/Blueprints/Actors/Samka_BP.Samka_BP_C|GetSamka _samkaactor))
  (if On%20/%20Off
    (bind _asmaterial_instance (Utilities|Casting|CastToMaterialInstance (Rendering|Material|GetMaterial _samka 5)))
    (Variables|Default|SetSamkaFaceMaterial _asmaterial_instance)
    (Rendering|Material|SetMaterial _samka 5 _translucentmaterialinstance)
    (Rendering|Material|SetMaterial _samka 0 _translucentmaterialinstance)
    (else
      (Rendering|Material|SetMaterial _samka 5 (Variables|Default|GetSamkaFaceMaterial))
      (Rendering|Material|SetMaterial _samka 0 "/Game/Models/Samka_D_v1/Materials/Samka_D_Eyelashes.Samka_D_Eyelashes"))))

(fn CalculateSucking
  (LocalVariables|SetGen1Location (.DickGen1Location (CallFunction|OMGetDickVector)))
  (LocalVariables|SetDickLength (CallFunction|OMGetDickTotalLength))
  (Variables|Default|SetGen1ToHeadDistance (Math|Vector|VectorLength (- (LocalVariables|GetGen1Location) (.Location (Math|Transform|BreakTransform (CallFunction|OMGetPActorSocketTransform "NewEnumerator0" "headSocket" "RTS_World"))))))
  (Variables|Default|SetGen6ToHeadDistance (- (Variables|Default|GetGen1ToHeadDistance) (LocalVariables|GetDickLength)))
  (if (< (Variables|Default|GetGen6ToHeadDistance) 0.0)
    (if (Variables|Default|GetIsSucking)
      (Default|CallEDonISSuckingTick)
      (if (> (Variables|Default|GetFurthestSuckedDickPoint) (Variables|Default|GetGen1ToHeadDistance))
        (Variables|Default|SetFurthestSuckedDickPoint (Variables|Default|GetGen1ToHeadDistance)))
      (else
        (Variables|Default|SetIsSucking true)
        (Default|CallEDonIsSuckingChanged true)))
    (elif (Variables|Default|GetIsSucking)
      (Variables|Default|SetIsSucking false)
      (Default|CallEDonIsSuckingChanged false)
      (CallFunction|OMCreateSalivaCableEffect 0 "None")
      (else
        (Default|CallEDonNOTIsSuckingTick)))))

(fn OMSetCameraShakeValue
  (params (CameraShakeValue :type Float%20%28single-precision%29))
  (Variables|Default|SetCameraShakeValue CameraShakeValue))

(fn ShakePlayerCamera
  (bind _newplayercamera (Variables|Default|GetNewPlayerCamera))
  (if (!= (Variables|Default|GetCurrentPlayerCamera) _newplayercamera)
    (Utilities|IsValid (Variables|Default|GetCurrentPlayerCamera)
      (:Is%20Valid
        (Transformation|SetWorldRotation (Variables|Default|GetCurrentPlayerCamera) (Math|Conversions|RotationFromXVector (Variables|Default|GetCameraDefaultForwardVector)) false false))
      (:Is%20Not%20Valid
        _))
    (Utilities|IsValid (Variables|Default|GetNewPlayerCamera)
      (:Is%20Valid
        (Variables|Default|SetCameraDefaultForwardVector (Math|Vector|GetForwardVector _newplayercamera))
        (Variables|Default|SetCurrentPlayerCamera (Variables|Default|GetNewPlayerCamera)))))
  (if (not (Math|Float|NearlyEqual(Float) (Variables|Default|GetCameraShakeValue) 0.0 0.01))
    (Utilities|IsValid (Variables|Default|GetCurrentPlayerCamera)
      (:Is%20Valid
        (Transformation|SetWorldRotation (Variables|Default|GetCurrentPlayerCamera) (Math|Conversions|RotationFromXVector (Math|Random|RandomUnitVectorinConeinDegrees (Variables|Default|GetCameraDefaultForwardVector) (/ (Variables|Default|GetCameraShakeValue) 1e+01))) false false)))))

(fn OMSetPlayerCamera
  (params (Actor%20With%20Camera :type Actor%20Object%20Reference))
  (bind _returnvalue (Actor|GetComponentbyClass Actor%20With%20Camera "/Script/Engine.CameraComponent"))
  (Utilities|IsValid _returnvalue
    (:Is%20Valid
      (Game|Player|SetViewTargetwithBlend (Game|GetPlayerController 0) Actor%20With%20Camera 0.0 "VTBlend_Linear" 0.0 false)
      (Variables|Default|SetNewPlayerCamera _returnvalue))))

(fn OMCreateSalivaCableEffect
  (params (Quantity :type Integer) (FurthestDickBone :type Name))
  (bind _furthestsuckeddickpoint (Variables|Default|GetFurthestSuckedDickPoint))
  (bind _location (CallFunction|OMDickMetricsPointtoLocation _furthestsuckeddickpoint))
  (bind (_x _y _z) (Math|Vector|BreakVector _location))
  (if (Variables|Default|GetIsSalivaEnabled)
    (bind _bone (CallFunction|GetClothestDickBonetoLocation _location))
    (bind _returnvalue (Game|SpawnActorfromClass "/Game/Blueprints/Actors/SalivaCable_BP.SalivaCable_BP_C" (Math|Transform|MakeTransform (Math|Vector|MakeVector _x _y (- _z 1.8))) "AlwaysSpawn" 0 0))
    (Transformation|AttachActorToActor _returnvalue (Variables|Default|GetSamecActor) _bone "KeepWorld" "KeepWorld" "KeepWorld" true)
    (Class|CableComponent|SetAttachEndto (Variables|/Game/Blueprints/Actors/SalivaCable_BP.SalivaCable_BP_C|GetCable _returnvalue) (Variables|Default|GetSamkaActor) "Samka" (Utilities|String|StringToName (Utilities|String|Append "SalivaSocket" (Utilities|String|ToString(Integer) (Math|Random|RandomIntegerinRange 1 4)))))
    (Variables|/Script/CableComponent.CableComponent|SetCableGravityScale (Variables|/Game/Blueprints/Actors/SalivaCable_BP.SalivaCable_BP_C|GetCable _returnvalue) 13.0)
    (Utilities|Array|Add (Variables|Default|GetSalivaObjectsArray) _returnvalue)))

(fn GetLocationBetweenTwoDickBonesbyNormalizedValue
  (params (Normalized%20Value :type Float%20%28single-precision%29))
  (bind _transform (CallFunction|OMGetPActorSocketTransform "NewEnumerator2" "None" "RTS_World"))
  (return (Math|Transform|InverseTransformLocation _transform (Math|Vector|Lerp(Vector) (.Location (Math|Transform|BreakTransform _transform)) (.Location (Math|Transform|BreakTransform (CallFunction|OMGetPActorSocketTransform "NewEnumerator2" "None" "RTS_World"))) Normalized%20Value))))

(fn OMDickMetricsPointtoLocation
  (params (Point :type Float%20%28single-precision%29))
  (bind (_dickgen1location _dickvector) (CallFunction|OMGetDickVector))
  (return (+ _dickgen1location (* _dickvector Point))))

(fn GetClothestDickBonetoLocation
  (params (Location :type Vector))
  (bind _array (LocalVariables|GetArray))
  (LocalVariables|SetOur%20Location Location)
  (Utilities|Array|Add _array (CallFunction|GetDistance (.Location (Math|Transform|BreakTransform (CallFunction|OMGetPActorSocketTransform "NewEnumerator1" "Gen1" "RTS_World"))) (LocalVariables|GetOur%20Location)))
  (Utilities|Array|Add _array (CallFunction|GetDistance (.Location (Math|Transform|BreakTransform (CallFunction|OMGetPActorSocketTransform "NewEnumerator1" "Gen2" "RTS_World"))) (LocalVariables|GetOur%20Location)))
  (Utilities|Array|Add _array (CallFunction|GetDistance (.Location (Math|Transform|BreakTransform (CallFunction|OMGetPActorSocketTransform "NewEnumerator1" "Gen3" "RTS_World"))) (LocalVariables|GetOur%20Location)))
  (Utilities|Array|Add _array (CallFunction|GetDistance (.Location (Math|Transform|BreakTransform (CallFunction|OMGetPActorSocketTransform "NewEnumerator1" "Gen4" "RTS_World"))) (LocalVariables|GetOur%20Location)))
  (Utilities|Array|Add _array (CallFunction|GetDistance (.Location (Math|Transform|BreakTransform (CallFunction|OMGetPActorSocketTransform "NewEnumerator1" "Gen5" "RTS_World"))) (LocalVariables|GetOur%20Location)))
  (Utilities|Array|Add _array (CallFunction|GetDistance (.Location (Math|Transform|BreakTransform (CallFunction|OMGetPActorSocketTransform "NewEnumerator1" "Gen6" "RTS_World"))) (LocalVariables|GetOur%20Location)))
  (switch int (.IndexOfMinValue (Math|Float|MinOfFloatArray (LocalVariables|GetArray)))
    (:0
      (return "Gen1"))
    (:1
      (return "Gen2"))
    (:2
      (return "Gen3"))
    (:3
      (return "Gen4"))
    (:4
      (return "Gen5"))
    (:5
      (return "Gen6"))))

(fn OMGetDickLengthMultiplier
  (bind _samecactor (Variables|Default|GetSamecActor))
  (bind _dicklengthmultiplier (Variables|/Game/Blueprints/Actors/Samec_BP.Samec_BP_C|GetDickLengthMultiplier _samecactor))
  (return _dicklengthmultiplier (Math|Float|NormalizetoRange _dicklengthmultiplier (Variables|/Game/Blueprints/Actors/Samec_BP.Samec_BP_C|GetMinDickLength _samecactor) (Variables|/Game/Blueprints/Actors/Samec_BP.Samec_BP_C|GetMaxDickLength _samecactor))))

(fn OMSetSalivaEnabled
  (params (isEnabled :type Boolean))
  (bind _output_get (Variables|Default|SetIsSalivaEnabled isEnabled))
  (if (not _output_get)
    (for _array_element (Variables|Default|GetSalivaObjectsArray)
      (Actor|DestroyActor _array_element))
    (Utilities|Array|Clear (Variables|Default|GetSalivaObjectsArray))))