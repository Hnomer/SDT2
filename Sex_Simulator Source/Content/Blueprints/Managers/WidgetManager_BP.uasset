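; Widget manager actor that creates, caches and closes UI widgets by class.
; WMOpenWidget returns the cached instance found by WMGetWidget, or creates and stores one without adding it to screen.
; WMCloseWidget removes the widget from its parent but keeps it cached for reuse.
; Shortly after BeginPlay, it calls OpenWidget to show the FPS counter on a high ZOrder if saved settings enable it.
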(event EventBeginPlay
  (Utilities|FlowControl|Delay 2.0)
  (bind _settingsstruct (CallFunction|GetDatafromSettingsSaveObject))
  (if (.IsShowFPS (Utilities|Struct|BreakSettingsSave_Struct _settingsstruct))
    (CallFunction|OpenWidget "/Game/Blueprints/HUD/InGameHUD/FPSWidget_BP.FPSWidget_BP_C" true 999)))

(event Collision|EventActorBeginOverlap
  (params (OtherActor :type Actor%20Object%20Reference)))

(event EventTick
  (params (DeltaSeconds :type Float%20%28single-precision%29)))

(fn ConstructionScript
  (Rendering|SetVisibility (Variables|Default|GetDefaultSceneRoot) false true))

(fn WMOpenWidget
  (params (Widget%20Class :type User%20Widget%20Class%20Reference))
  (bind _widget (CallFunction|WMGetWidget Widget%20Class))
  (if (!= _widget 0)
    (return _widget)
    (else
      (bind _returnvalue (UserInterface|CreateWidget Widget%20Class))
      (Utilities|Array|Add (Variables|Default|GetWidgetObjectsArray) _returnvalue)
      (return _returnvalue))))

(fn WMCloseWidget
  (params (WidgetClass :type User%20Widget%20Class%20Reference))
  (bind _widget (CallFunction|WMGetWidget WidgetClass))
  (if (!= _widget 0)
    (Widget|RemovefromParent _widget)))

(fn WMGetWidget
  (params (WidgetClass :type User%20Widget%20Class%20Reference))
  (bind _array_element (Utilities|Array|ForEachLoopwithBreak (Variables|Default|GetWidgetObjectsArray))
    (:LoopBody
      (if (== (Utilities|GetClass _array_element) WidgetClass)
        (return _array_element)))
    (:Completed
      (return 0))))