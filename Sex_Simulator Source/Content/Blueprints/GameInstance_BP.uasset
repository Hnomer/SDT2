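; Game instance that bootstraps the game's managers and opens the main menu.
; Init caches the morph list as an array of structs.
; When the persistent level is created, it spawns saves, sound, widget, lower-level and upper-level class manager actors, sets UI-only mouse input and switches to the main menu upper-level class.
; It reads UI volume from SoundManager and binds to its change delegate; a Mac fullscreen fix exists but never runs.
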(event Custom|On_PersistantLevelCreated
  (bind _returnvalue (Game|GetPlayerController 0))
  (CallFunction|CreateManagers)
  (Variables|/Script/Engine.PlayerController|SetbShowMouseCursor _returnvalue true)
  (Input|SetInputModeUIOnly _returnvalue 0 "DoNotLock")
  (CallFunction|SwitchULC "/Game/Levels/MainMenu_UpperLevelClass_BP.MainMenu_UpperLevelClass_BP_C"))

(event EventInit
  (CallFunction|PopulateMorphListMorphItemsStructArray))

(fn CheckScreenModeforMac
  (if (.Mac (Class|VictoryBPFunctionLibrary|OperatingSystemGetCurrentPlatform))
    (bind _returnvalue (Settings|GetGameUserSettings))
    (switch Utilities|FlowControl|Switch|SwitchonEWindowMode (Class|GameUserSettings|GetFullscreenMode _returnvalue)
      (:WindowedFullscreen
        (Class|GameUserSettings|SetFullscreenMode _returnvalue "Fullscreen")
        (Class|GameUserSettings|SetScreenResolution _returnvalue (Class|GameUserSettings|GetScreenResolution _returnvalue))
        (Class|GameUserSettings|ApplyResolutionSettings _returnvalue false)))))

(fn PopulateMorphListMorphItemsStructArray
  (bind (_issuccess _arrayofmorphstructs) (CallFunction|GetMorphListasArrayOfMorphStructs))
  (if _issuccess
    (Variables|Default|SetMorphListMorphItemsStructArray _arrayofmorphstructs)))

(fn ChangeUIVolume
  (params (NewVolume :type Float%20%28single-precision%29))
  (Variables|Default|SetUIVolume NewVolume))

(fn CreateManagers
  (bind _returnvalue (Math|Transform|MakeTransform "0, 0, 0"))
  (bind _returnvalue_2 (Game|SpawnActorfromClass "/Game/Blueprints/Customization/SavesManager_BP.SavesManager_BP_C" _returnvalue "AlwaysSpawn" 0 0))
  (Variables|Default|SetSavesManager _returnvalue_2)
  (bind _returnvalue_3 (Game|SpawnActorfromClass "/Game/Blueprints/Managers/SoundManager_BP.SoundManager_BP_C" _returnvalue "AlwaysSpawn" 0 0))
  (Variables|Default|SetSoundManager _returnvalue_3)
  (bind _returnvalue_4 (Game|SpawnActorfromClass "/Game/Blueprints/Managers/WidgetManager_BP.WidgetManager_BP_C" _returnvalue "AlwaysSpawn" 0 0))
  (Variables|Default|SetWidgetManager _returnvalue_4)
  (bind _returnvalue_5 (Game|SpawnActorfromClass "/Game/Blueprints/Managers/LowerLevelManager_BP.LowerLevelManager_BP_C" _returnvalue "AlwaysSpawn" 0 0))
  (Variables|Default|SetLLCManager _returnvalue_5)
  (bind _returnvalue_6 (Game|SpawnActorfromClass "/Game/Blueprints/Managers/UpperLevelClassManager_BP.UpperLevelClassManager_BP_C" _returnvalue "AlwaysSpawn" 0 0))
  (Variables|Default|SetULCManager _returnvalue_6)
  (Variables|Default|SetUIVolume (Default|GetUIVolume (Variables|Default|GetSoundManager)))
  (EventDispatchers|BindEventtoSoundManageronUIVolumeChangedDelegate (Variables|Default|GetSoundManager) (EventDispatchers|CreateEvent :!event ChangeUIVolume)))