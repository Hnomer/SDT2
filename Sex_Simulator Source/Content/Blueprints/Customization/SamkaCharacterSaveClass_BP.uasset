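; Save data class for Samka character customization, holding morph items, body part colors, name, version, date, author metadata and custom/editable flags.
; SetSaveData copies all inputs into member variables and converts the thumbnail texture into a pixel array for storage.
; GetSaveData returns every field, rebuilding a 512x512 texture from stored pixels, or using the CharacterThumbnail texture when no pixels exist.
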(fn SetSaveData
  (params (SaveName :type Name) (SaveVersion :type Name) (SaveDate :type Date%20Time%20Structure) (AuthorName :type Name) (ModifiedByName :type Name) (Thumbnail :type Texture%202D%20Object%20Reference) (MorphItemStruct_Array :type Array%20of%20Morph%20Item%20Struct%20Structures) (BodyPartsColorsStruct :type Body%20Parts%20Colors%20Struct%20Structure) (IsCustomSave :type Boolean) (IsEditableSave :type Boolean))
  (Utilities|FlowControl|Sequence
    (:then_0
      (Variables|Default|SetSaveName SaveName))
    (:then_1
      (Variables|Default|SetSaveVersion SaveVersion))
    (:then_2
      (Variables|Default|SetAuthorName AuthorName))
    (:then_3
      (Variables|Default|SetModifiedByName ModifiedByName))
    (:then_4
      (Variables|Default|SetMorphItemStruct_Array MorphItemStruct_Array))
    (:then_5
      (Variables|Default|SetIsCustomSave IsCustomSave))
    (:then_6
      (Variables|Default|SetIsEditableSave IsEditableSave))
    (:then_7
      (Variables|Default|SetSaveDate SaveDate))
    (:then_8
      (bind _returnvalue (Class|HnomerBPLibraryPluginBPLibrary|GetPixelsArrayfromTexture2D Thumbnail))
      (Variables|Default|SetCharacterThumbnailPixels _returnvalue))
    (:then_9
      (Variables|Default|SetBodyPartsColorsStruct BodyPartsColorsStruct))))

(fn GetSaveData
  (bind _characterthumbnailpixels (Variables|Default|GetCharacterThumbnailPixels))
  (if (> (Utilities|Array|Length _characterthumbnailpixels) 0)
    (bind _returnvalue (Class|HnomerBPLibraryPluginBPLibrary|GetTexture2DfromPixelsArray _characterthumbnailpixels 512 512))
    (LocalVariables|SetThumbnailTexture _returnvalue)
    (elif (!= (Variables|Default|GetCharacterThumbnail) 0)
      (LocalVariables|SetThumbnailTexture (Variables|Default|GetCharacterThumbnail))))
  (return (Variables|Default|GetSaveName) (Variables|Default|GetSaveVersion) (Variables|Default|GetSaveDate) (Variables|Default|GetAuthorName) (Variables|Default|GetModifiedByName) (LocalVariables|GetThumbnailTexture) (Variables|Default|GetMorphItemStruct_Array) (Variables|Default|GetBodyPartsColorsStruct) (Variables|Default|GetIsCustomSave) (Variables|Default|GetIsEditableSave)))