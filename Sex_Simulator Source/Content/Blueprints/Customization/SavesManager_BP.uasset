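; SavesManager_BP is an actor that saves, loads, lists and deletes character customization and settings save games.
; Female and male saves get slot prefixes, while settings use one fixed slot, created if loading fails.
; Lookups match slot file names or internal SaveName by scanning files, and female loads fall back to built-in saves instantiated from game instance classes.
; Listings can include built-ins and sort newest first by repeated maximum selection.
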(event EventBeginPlay)

(event Collision|EventActorBeginOverlap
  (params (OtherActor :type Actor%20Object%20Reference)))

(event EventTick
  (params (DeltaSeconds :type Float%20%28single-precision%29)))

(fn ConstructionScript
  (Rendering|SetVisibility (Variables|Default|GetDefaultSceneRoot) false true))

(fn SMGetAllSaveFiles
  (params (IncludeBuitInSaves :type Boolean) (BuilInSavesOnly :type Boolean) (SortByDate :type Boolean) (Save%20Type :type SaveFileType_ENum%20Enum :default "NewEnumerator0"))
  (bind _savesarray (LocalVariables|GetSavesArray))
  (if BuilInSavesOnly
    (for _array_element (Variables|/Game/Blueprints/GameInstance_BP.GameInstance_BP_C|GetBuiltInSaves_Array (CallFunction|GetCustomGameInstance)) :!label _label
      (bind _returnvalue (SaveGame|CreateSaveGameObject _array_element))
      (bind _assave_base_class_bp (Utilities|Casting|CastToSaveBaseClass_BP _returnvalue))
      (Utilities|Array|Add (LocalVariables|GetSavesArray) _assave_base_class_bp))
    (else
      (for _array_element_2 (Class|VictoryBPFunctionLibrary|SaveGameObjectGetAllSaveSlotFileNames)
        (bind (_issuccess _returnvalue_2) (CallFunction|SMGetSave Save%20Type true (Utilities|String|StringToName _array_element_2)))
        (if _issuccess
          (Utilities|Array|Add (LocalVariables|GetSavesArray) _returnvalue_2)))
      (if IncludeBuitInSaves
        (goto _label)
        (else
          _))))
  (if SortByDate
    (bind _sortedsaveobjectsarray (CallFunction|SMSortSavesbyCreationDate _savesarray))
    (return _sortedsaveobjectsarray)
    (else
      (return _savesarray))))

(fn SMSave
  (params (SaveType :type SaveFileType_ENum%20Enum :default "NewEnumerator0") (SlotName :type Name) (Save%20Object :type Save%20Game%20Object%20Reference))
  (switch Utilities|FlowControl|Switch|SwitchonSaveFileType_ENum SaveType
    (:NewEnumerator0
      (LocalVariables|SetPreffix "chFem_"))
    (:NewEnumerator2
      (LocalVariables|SetPreffix "chMal_"))
    (:NewEnumerator1
      (bind _returnvalue (SaveGame|SaveGametoSlot Save%20Object "settings"))
      (return _returnvalue)))
  (bind _returnvalue_2 (SaveGame|SaveGametoSlot Save%20Object (Utilities|String|Append (LocalVariables|GetPreffix) (Utilities|String|ToString(Name) SlotName))))
  (return _returnvalue_2))

(fn SMGetSave
  (params (Save%20Type :type SaveFileType_ENum%20Enum :default "NewEnumerator0") (IsExtetnalSaveName :type Boolean) (SaveName :type Name))
  (switch Utilities|FlowControl|Switch|SwitchonSaveFileType_ENum Save%20Type
    (:NewEnumerator0
      (if IsExtetnalSaveName
        (bind _returnvalue (SaveGame|LoadGamefromSlot (.LeftS (Utilities|String|Split (Utilities|String|ToString(Name) SaveName) "." "IgnoreCase" "FromEnd"))))
        (bind _assave_base_class_bp (Utilities|Casting|CastToSaveBaseClass_BP _returnvalue)
          (:then
            (return true _assave_base_class_bp))
          (:CastFailed
            _))
        (else
          (bind (_isfound _externalname _saveobject) (CallFunction|SMGetSavewithInternalName SaveName))
          (if _isfound
            (return _isfound _saveobject)
            (else
              _))))
      (bind _save_objects_array (CallFunction|SMGetAllSaveFiles false true false "NewEnumerator0"))
      (for _array_element _save_objects_array
        (if (Utilities|Name|Equal(Name) (Variables|/Game/Blueprints/Customization/SaveBaseClass_BP.SaveBaseClass_BP_C|GetSaveName _array_element) SaveName)
          (return true _array_element)))
      (return false 0))
    (:NewEnumerator1
      (bind _returnvalue_2 (SaveGame|LoadGamefromSlot "settings"))
      (bind _assettings_save_class_bp (Utilities|Casting|CastToSettingsSaveClass_BP _returnvalue_2)
        (:then
          (return true _assettings_save_class_bp))
        (:CastFailed
          (bind _returnvalue_3 (SaveGame|CreateSaveGameObject "/Game/Blueprints/SettingsSaveClass_BP.SettingsSaveClass_BP_C"))
          (bind _issaved (CallFunction|SMSave "NewEnumerator1" "settings" _returnvalue_3))
          (return _issaved _assettings_save_class_bp))))))

(fn SMDeleteSave
  (params (DeleteByExternalName :type Boolean) (slot%20name :type Name))
  (if DeleteByExternalName
    (bind _returnvalue (SaveGame|DeleteGameinSlot (Utilities|String|ToString(Name) slot%20name)))
    (return _returnvalue)
    (else
      (bind (_isfound _externalname) (CallFunction|SMGetSavewithInternalName slot%20name))
      (if _isfound
        (bind _returnvalue_2 (SaveGame|DeleteGameinSlot (Utilities|String|ToString(Name) _externalname)))
        (return _returnvalue_2)
        (else
          (return false))))))

(fn SMSortSavesbyCreationDate
  (params (Save%20Objects%20Array :type Array%20of%20Save%20Base%20Class%20BP%20Object%20References))
  (bind _output_get (LocalVariables|SetSavesArray Save%20Objects%20Array))
  (bind _output_get_2 (LocalVariables|SetArrayLength (Utilities|Array|Length _output_get)))
  (for _index (range 1 _output_get_2)
    (for _array_element (LocalVariables|GetSavesArray)
      (if (> (Variables|/Game/Blueprints/Customization/SaveBaseClass_BP.SaveBaseClass_BP_C|GetSaveDate _array_element) (LocalVariables|GetMostRecentDate))
        (LocalVariables|SetMostRecentDate (Variables|/Game/Blueprints/Customization/SaveBaseClass_BP.SaveBaseClass_BP_C|GetSaveDate _array_element))
        (LocalVariables|SetMostRecentSave _array_element)))
    (Utilities|Array|Add (LocalVariables|GetSavesArraySortedByDate) (LocalVariables|GetMostRecentSave))
    (Utilities|Array|RemoveItem (LocalVariables|GetSavesArray) (LocalVariables|GetMostRecentSave))
    (LocalVariables|SetMostRecentDate (Math|DateTime|MakeDateTime 0 0 0))
    (LocalVariables|SetMostRecentSave 0))
  (return (LocalVariables|GetSavesArraySortedByDate)))

(fn SMIsSaveExists
  (params (Save%20Type :type SaveFileType_ENum%20Enum :default "NewEnumerator0") (SaveName :type Name))
  (bind _save_objects_array (CallFunction|SMGetAllSaveFiles false false false Save%20Type))
  (bind _array_element (Utilities|Array|ForEachLoopwithBreak _save_objects_array)
    (:LoopBody
      (if (Utilities|Name|Equal(Name) (Variables|/Game/Blueprints/Customization/SaveBaseClass_BP.SaveBaseClass_BP_C|GetSaveName _array_element) SaveName)
        (return true)))
    (:Completed
      (return false))))

(fn SMGetSavewithInternalName
  (params (InternalSaveName :type Name))
  (for _array_element (Class|VictoryBPFunctionLibrary|SaveGameObjectGetAllSaveSlotFileNames)
    (bind _returnvalue (SaveGame|LoadGamefromSlot (.LeftS (Utilities|String|Split _array_element "." "IgnoreCase" "FromEnd"))))
    (bind _assave_base_class_bp (Utilities|Casting|CastToSaveBaseClass_BP _returnvalue))
    (if (Utilities|Name|Equal(Name) (Variables|/Game/Blueprints/Customization/SaveBaseClass_BP.SaveBaseClass_BP_C|GetSaveName _assave_base_class_bp) InternalSaveName)
      (return true (Utilities|String|StringToName (.LeftS (Utilities|String|Split _array_element "." "IgnoreCase" "FromEnd"))) _assave_base_class_bp)))
  (return false "None" 0))