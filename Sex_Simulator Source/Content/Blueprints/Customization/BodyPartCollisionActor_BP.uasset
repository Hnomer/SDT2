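; Cursor-pickable collision actor that represents one named body part in the customization system.
; The construction script enables query-only collision and visibility on the Box, Sphere or Capsule component selected by CollisionShape.
; Cursor begin-over, end-over and click events from all three shapes are routed into shared delegate calls that pass BodyPartName to listeners.
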(event OnClicked(Capsule)
  (params (TouchedComponent :type Primitive%20Component%20Object%20Reference) (ButtonPressed :type Key%20Structure))
  (Default|CallOnCollisionClickedDelegate (Variables|Default|GetBodyPartName)))

(event OnClicked(Box)
  (params (TouchedComponent :type Primitive%20Component%20Object%20Reference) (ButtonPressed :type Key%20Structure))
  (Default|CallOnCollisionClickedDelegate (Variables|Default|GetBodyPartName)))

(event OnBeginCursorOver(Box)
  (params (TouchedComponent :type Primitive%20Component%20Object%20Reference))
  (Default|CallOnCollisionBeginOverlapDelegate (Variables|Default|GetBodyPartName)))

(event OnEndCursorOver(Box)
  (params (TouchedComponent :type Primitive%20Component%20Object%20Reference))
  (Default|CallOnCollisionEndOverlapDelegate (Variables|Default|GetBodyPartName)))

(event OnBeginCursorOver(Sphere)
  (params (TouchedComponent :type Primitive%20Component%20Object%20Reference))
  (Default|CallOnCollisionBeginOverlapDelegate (Variables|Default|GetBodyPartName)))

(event OnEndCursorOver(Sphere)
  (params (TouchedComponent :type Primitive%20Component%20Object%20Reference))
  (Default|CallOnCollisionEndOverlapDelegate (Variables|Default|GetBodyPartName)))

(event OnClicked(Sphere)
  (params (TouchedComponent :type Primitive%20Component%20Object%20Reference) (ButtonPressed :type Key%20Structure))
  (Default|CallOnCollisionClickedDelegate (Variables|Default|GetBodyPartName)))

(event OnBeginCursorOver(Capsule)
  (params (TouchedComponent :type Primitive%20Component%20Object%20Reference))
  (Default|CallOnCollisionBeginOverlapDelegate (Variables|Default|GetBodyPartName)))

(event OnEndCursorOver(Capsule)
  (params (TouchedComponent :type Primitive%20Component%20Object%20Reference))
  (Default|CallOnCollisionEndOverlapDelegate (Variables|Default|GetBodyPartName)))

(fn ConstructionScript
  (bind _box (Variables|Default|GetBox))
  (bind _sphere (Variables|Default|GetSphere))
  (bind _capsule (Variables|Default|GetCapsule))
  (switch Utilities|FlowControl|Switch|SwitchonCollisionShape_ENum (Variables|Default|GetCollisionShape)
    (:NewEnumerator0
      (Collision|SetCollisionEnabled _box "QueryOnly")
      (Rendering|SetVisibility _box true false))
    (:NewEnumerator1
      (Collision|SetCollisionEnabled _sphere "QueryOnly")
      (Rendering|SetVisibility _sphere true false))
    (:NewEnumerator2
      (Collision|SetCollisionEnabled _capsule "QueryOnly")
      (Rendering|SetVisibility _capsule true false))))