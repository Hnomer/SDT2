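; Preview actor for the Samka character on the customization screen, driving its in-game AnimBP in customization mode.
; On BeginPlay it binds child body-part collision actors' hover and click delegates for relay through its own calls, and initializes BlinkManager with the skeletal mesh.
; Timeline-driven events rotate the actor's yaw and interpolate a clamped head up/down value on the AnimInstance, with easing back.
; Debug hit printing and disconnected UV-trace experiments remain.
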(event OnComponentHit(Samka)
  (params (HitComponent :type Primitive%20Component%20Object%20Reference) (OtherActor :type Actor%20Object%20Reference) (OtherComp :type Primitive%20Component%20Object%20Reference) (NormalImpulse :type Vector :default "0, 0, 0") (Hit :type Hit%20Result%20Structure%20%28by%20ref%29))
  (Development|PrintString "Hello"))

(event Custom|HeadUpDown
  (params (Force :type Float%20%28single-precision%29) (Back :type Boolean))
  (bind _returnvalue (Utilities|Time|GetWorldDeltaSeconds))
  (bind _animinstance (Variables|Default|GetAnimInstance))
  (Timeline|HeadUpDownTimeline PlayFromStart
    (:Update
      (if Back
        (Variables|/Game/Models/Samka_D_v1/Mesh/Test/Animations/AnimBP_SamkaInGame.AnimBP_SamkaInGame_C|SetHeadUpDownValue _animinstance (Math|Interpolation|FInterpTo (Variables|/Game/Models/Samka_D_v1/Mesh/Test/Animations/AnimBP_SamkaInGame.AnimBP_SamkaInGame_C|GetHeadUpDownValue _animinstance) 0.0 _returnvalue 3.0))
        (else
          (Variables|/Game/Models/Samka_D_v1/Mesh/Test/Animations/AnimBP_SamkaInGame.AnimBP_SamkaInGame_C|SetHeadUpDownValue _animinstance (Math|Interpolation|FInterpTo (Variables|/Game/Models/Samka_D_v1/Mesh/Test/Animations/AnimBP_SamkaInGame.AnimBP_SamkaInGame_C|GetHeadUpDownValue _animinstance) (Math|Float|Clamp(Float) (+ Force (Variables|/Game/Models/Samka_D_v1/Mesh/Test/Animations/AnimBP_SamkaInGame.AnimBP_SamkaInGame_C|GetHeadUpDownValue _animinstance)) -2e+01 2e+01) _returnvalue 1e+03)))))))

(event Custom|RotateSamka
  (params (Force :type Float%20%28single-precision%29))
  (bind _returnvalue (Transformation|GetActorRotation))
  (bind (_roll _pitch _yaw) (Math|Rotator|BreakRotator _returnvalue))
  (Timeline|RotateSamkaTimeline PlayFromStart
    (:Update
      (Transformation|SetActorRotation (Math|Rotator|MakeRotator _roll _pitch (Math|Interpolation|FInterpTo _yaw (+ (* Force 2.0) _yaw) (Utilities|Time|GetWorldDeltaSeconds) 1e+03))))))

(event EventBeginPlay
  (bind _blinkmanager (Variables|Default|GetBlinkManager))
  (Utilities|FlowControl|Sequence
    (:then_0
      (CallFunction|InitBodyParts)
      (bind _asanim_bp_samka_in_game (Utilities|Casting|CastToAnimBP_SamkaInGame (Components|SkeletalMesh|GetAnimInstance (Variables|Default|GetSamka))))
      (bind _output_get (Variables|Default|SetAnimInstance _asanim_bp_samka_in_game))
      (Variables|/Game/Models/Samka_D_v1/Mesh/Test/Animations/AnimBP_SamkaInGame.AnimBP_SamkaInGame_C|SetIsCustomization _output_get true))
    (:then_1
      (Variables|/Game/Blueprints/BlinkManager.BlinkManager_C|SetSamkaSkeletalComponent _blinkmanager (Variables|Default|GetSamka))
      (Default|Init _blinkmanager))))

(event EventTick
  (params (DeltaSeconds :type Float%20%28single-precision%29)))

(fn ConstructionScript
  (Variables|Default|SetSamkaSkeletalMesh (Variables|Default|GetSamka)))

(fn OnCursorBeginOverlapBodyPartDelegate
  (params (BodyPart :type BodyParts_Enum%20Enum :default "NewEnumerator0"))
  (Default|CallOnBeginCursorOverlapSamkaBodyPartDelegate BodyPart))

(fn OnCursorEndOverlapBodyPartDelegate
  (params (BodyPart :type BodyParts_Enum%20Enum :default "NewEnumerator0"))
  (Default|CallOnEndCursorOverlapSamkaBodyPartDelegate))

(fn OnClickedBodyPartDelegate
  (params (BodyPart :type BodyParts_Enum%20Enum :default "NewEnumerator0"))
  (Default|CallOnClickedSamkaBodyPartDelegate BodyPart))

(fn InitBodyParts
  (for _array_element (Actor|GetAllChildActors true)
    (bind _asbody_part_collision_actor_bp (Utilities|Casting|CastToBodyPartCollisionActor_BP _array_element))
    (Utilities|Array|Add (Variables|Default|GetCollisionActorsArray) _asbody_part_collision_actor_bp)
    (Utilities|FlowControl|Sequence
      (:then_0
        (EventDispatchers|BindEventtoOnCollisionBeginOverlapDelegate _asbody_part_collision_actor_bp (EventDispatchers|CreateEvent :!event OnCursorBeginOverlapBodyPartDelegate)))
      (:then_1
        (EventDispatchers|BindEventtoOnCollisionEndOverlapDelegate _asbody_part_collision_actor_bp (EventDispatchers|CreateEvent :!event OnCursorEndOverlapBodyPartDelegate)))
      (:then_2
        (EventDispatchers|BindEventtoOnCollisionClickedDelegate _asbody_part_collision_actor_bp (EventDispatchers|CreateEvent :!event OnClickedBodyPartDelegate))))))