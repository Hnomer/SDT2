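; Male character actor for an adult game, driving genital and left-hand poses through its animation instance.
; ObjectManager sucking-state events blend genital aim between default and partner's mouth, while throat-tagged overlaps hide bone segments by zero-scaling.
; An erection timeline raises length and scale, mirrored to a shadow mesh for measurement.
; Spring-smoothed input moves the hand until it grips the partner's head, then also forwards input to that actor.
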(event EventBeginPlay
  (bind _defaultlefthandposition (Variables|Default|GetDefaultLeftHandPosition))
  (bind _returnvalue (Transformation|GetWorldLocation _defaultlefthandposition))
  (CallFunction|Init)
  (Variables|Default|SetLeftHandPosition _returnvalue)
  (Variables|Default|SetConstDefaultLeftHandPosition _returnvalue)
  (Input|EnableInput (Game|GetPlayerController 0)))

(event Collision|EventActorBeginOverlap
  (params (OtherActor :type Actor%20Object%20Reference)))

(event EventTick
  (params (DeltaSeconds :type Float%20%28single-precision%29))
  (CallFunction|EGHandsPoseEventTick DeltaSeconds))

(event EventOnReset
  (bind _objectmanager (Variables|Default|GetObjectManager))
  (Default|OMSetDickLength _objectmanager false false 0.0)
  (Default|OMSetDickScale _objectmanager false false 1.0))

(event OnComponentBeginOverlap(DickPart_2)
  (params (OverlappedComponent :type Primitive%20Component%20Object%20Reference) (OtherActor :type Actor%20Object%20Reference) (OtherComp :type Primitive%20Component%20Object%20Reference) (OtherBodyIndex :type Integer) (bFromSweep :type Boolean) (SweepResult :type Hit%20Result%20Structure%20%28by%20ref%29))
  (Collision|OnDickPartBeginOverlap OverlappedComponent OtherComp))

(event OnComponentEndOverlap(DickPart_6)
  (params (OverlappedComponent :type Primitive%20Component%20Object%20Reference) (OtherActor :type Actor%20Object%20Reference) (OtherComp :type Primitive%20Component%20Object%20Reference) (OtherBodyIndex :type Integer))
  (Collision|OnDickPartEndOverlap OverlappedComponent OtherComp))

(event OnComponentEndOverlap(DickPart_5)
  (params (OverlappedComponent :type Primitive%20Component%20Object%20Reference) (OtherActor :type Actor%20Object%20Reference) (OtherComp :type Primitive%20Component%20Object%20Reference) (OtherBodyIndex :type Integer))
  (Collision|OnDickPartEndOverlap OverlappedComponent OtherComp))

(event OnComponentEndOverlap(DickPart_4)
  (params (OverlappedComponent :type Primitive%20Component%20Object%20Reference) (OtherActor :type Actor%20Object%20Reference) (OtherComp :type Primitive%20Component%20Object%20Reference) (OtherBodyIndex :type Integer))
  (Collision|OnDickPartEndOverlap OverlappedComponent OtherComp))

(event OnComponentEndOverlap(DickPart_3)
  (params (OverlappedComponent :type Primitive%20Component%20Object%20Reference) (OtherActor :type Actor%20Object%20Reference) (OtherComp :type Primitive%20Component%20Object%20Reference) (OtherBodyIndex :type Integer))
  (Collision|OnDickPartEndOverlap OverlappedComponent OtherComp))

(event OnComponentEndOverlap(DickPart_2)
  (params (OverlappedComponent :type Primitive%20Component%20Object%20Reference) (OtherActor :type Actor%20Object%20Reference) (OtherComp :type Primitive%20Component%20Object%20Reference) (OtherBodyIndex :type Integer))
  (Collision|OnDickPartEndOverlap OverlappedComponent OtherComp))

(event OnComponentEndOverlap(DickTree)
  (params (OverlappedComponent :type Primitive%20Component%20Object%20Reference) (OtherActor :type Actor%20Object%20Reference) (OtherComp :type Primitive%20Component%20Object%20Reference) (OtherBodyIndex :type Integer)))

(event OnComponentBeginOverlap(DickTree)
  (params (OverlappedComponent :type Primitive%20Component%20Object%20Reference) (OtherActor :type Actor%20Object%20Reference) (OtherComp :type Primitive%20Component%20Object%20Reference) (OtherBodyIndex :type Integer) (bFromSweep :type Boolean) (SweepResult :type Hit%20Result%20Structure%20%28by%20ref%29)))

(event OnComponentBeginOverlap(DickHead)
  (params (OverlappedComponent :type Primitive%20Component%20Object%20Reference) (OtherActor :type Actor%20Object%20Reference) (OtherComp :type Primitive%20Component%20Object%20Reference) (OtherBodyIndex :type Integer) (bFromSweep :type Boolean) (SweepResult :type Hit%20Result%20Structure%20%28by%20ref%29)))

(event OnComponentEndOverlap(DickHead)
  (params (OverlappedComponent :type Primitive%20Component%20Object%20Reference) (OtherActor :type Actor%20Object%20Reference) (OtherComp :type Primitive%20Component%20Object%20Reference) (OtherBodyIndex :type Integer)))

(event OnComponentBeginOverlap(DickPart_6)
  (params (OverlappedComponent :type Primitive%20Component%20Object%20Reference) (OtherActor :type Actor%20Object%20Reference) (OtherComp :type Primitive%20Component%20Object%20Reference) (OtherBodyIndex :type Integer) (bFromSweep :type Boolean) (SweepResult :type Hit%20Result%20Structure%20%28by%20ref%29))
  (Collision|OnDickPartBeginOverlap OverlappedComponent OtherComp))

(event OnComponentBeginOverlap(DickPart_5)
  (params (OverlappedComponent :type Primitive%20Component%20Object%20Reference) (OtherActor :type Actor%20Object%20Reference) (OtherComp :type Primitive%20Component%20Object%20Reference) (OtherBodyIndex :type Integer) (bFromSweep :type Boolean) (SweepResult :type Hit%20Result%20Structure%20%28by%20ref%29))
  (Collision|OnDickPartBeginOverlap OverlappedComponent OtherComp))

(event OnComponentBeginOverlap(DickPart_4)
  (params (OverlappedComponent :type Primitive%20Component%20Object%20Reference) (OtherActor :type Actor%20Object%20Reference) (OtherComp :type Primitive%20Component%20Object%20Reference) (OtherBodyIndex :type Integer) (bFromSweep :type Boolean) (SweepResult :type Hit%20Result%20Structure%20%28by%20ref%29))
  (Collision|OnDickPartBeginOverlap OverlappedComponent OtherComp))

(event OnComponentBeginOverlap(DickPart_3)
  (params (OverlappedComponent :type Primitive%20Component%20Object%20Reference) (OtherActor :type Actor%20Object%20Reference) (OtherComp :type Primitive%20Component%20Object%20Reference) (OtherBodyIndex :type Integer) (bFromSweep :type Boolean) (SweepResult :type Hit%20Result%20Structure%20%28by%20ref%29))
  (Collision|OnDickPartBeginOverlap OverlappedComponent OtherComp))

(event Custom|Samec_DetachDickFromMouth
  (Utilities|FlowControl|Sequence
    (:then_0
      (Timeline|SetDickToMouthLocation_Timeline Stop
        (:Update
          (DickPose|SetDickVeiwDirection (DickPose|GetDickViewDirectionatMouth)))))
    (:then_1
      (bind _newtrack_0 (Timeline|SetDickToNormalPosition PlayFromStart)
        (:Update
          (DickPose|SetDickVeiwDirection (Math|Vector|Lerp(Vector) (DickPose|GetDickViewDirection) (DickPose|GetDickDefaultViewDirection) _newtrack_0)))))))

(event Custom|Samec_AttachDickToMouth
  (Utilities|FlowControl|Sequence
    (:then_0
      (bind _newtrack_0 (Timeline|SetDickToNormalPosition Stop)
        (:Update
          (DickPose|SetDickVeiwDirection (Math|Vector|Lerp(Vector) (DickPose|GetDickViewDirection) (DickPose|GetDickDefaultViewDirection) _newtrack_0)))))
    (:then_1
      (Timeline|SetDickToMouthLocation_Timeline PlayFromStart
        (:Update
          (DickPose|SetDickVeiwDirection (DickPose|GetDickViewDirectionatMouth)))))))

(event Custom|Samec_EEE
  (params (Value :type Float%20%28single-precision%29))
  (Utilities|FlowControl|Sequence
    (:then_0
      (bind _newtrack_0 (Timeline|SetDickToNormalPosition Stop)
        (:Update
          (DickPose|SetDickVeiwDirection (Math|Vector|Lerp(Vector) (DickPose|GetDickViewDirection) (DickPose|GetDickDefaultViewDirection) _newtrack_0)))))
    (:then_1
      (DickPose|SetDickVeiwDirection (Math|Vector|Lerp(Vector) (DickPose|GetDickViewDirectionatMouth) (DickPose|GetDickDefaultViewDirection) Value)))))

(event Custom|Samec_StartErection
  (Timeline|Erection Play
    (:Update
      (bind _isfullyerected (Erection|CalculateandSetErection))
      (if _isfullyerected
        (Timeline|Erection Stop)))))

(event Custom|EG_HandsPose_EventTick
  (params (DeltaSeconds :type Float%20%28single-precision%29))
  (if (Variables|Default|GetIsHoldingHead)
    (LeftHandPose|SetLeftHandPositiontoSamkaHead)
    (else
      (CallFunction|SetLeftHandPosition 0.0 0.0 false)
      (LeftHandPose|ApplyPositiontoLeftHand (Variables|Default|GetLeftHandPosition)))))

(event Custom|EG_InputX
  (params (Input :type Float%20%28single-precision%29))
  (CallFunction|ReceiveLeftHandInput Input 0.0 false false)
  (if (Variables|Default|GetIsHoldingHead)
    (Default|EGControlsReceiveMouseInputX (Variables|/Game/Blueprints/Managers/ObjectsManager.ObjectsManager_C|GetSamkaActor (Variables|Default|GetObjectManager)) Input)))

(event Custom|EG_InputY
  (params (Input :type Float%20%28single-precision%29))
  (CallFunction|ReceiveLeftHandInput 0.0 Input false false)
  (if (Variables|Default|GetIsHoldingHead)
    (Default|EGControlsReceiveMouseInputY (Variables|/Game/Blueprints/Managers/ObjectsManager.ObjectsManager_C|GetSamkaActor (Variables|Default|GetObjectManager)) Input)))

(event Input|KeyboardEvents|K
  (params (Key :type Key%20Structure))
  (:Pressed
    (Variables|Default|SetIsHoldingHead false)
    (CallFunction|ReceiveLeftHandInput 0.0 0.0 true false)))

(fn ConstructionScript)

(fn ManageCensorVersion
  (bind _asgame_instance_bp (Utilities|Casting|CastToGameInstance_BP (Game|GetGameInstance)))
  (CallFunction|SetCensor (Variables|/Game/Blueprints/GameInstance_BP.GameInstance_BP_C|GetIsCensoredVersion _asgame_instance_bp)))

(fn SetCensor
  (params (IsCensor :type Boolean))
  (Rendering|SetVisibility (Variables|Default|GetCensorCube1) IsCensor false))

(fn SetDickLength
  (params (AddToCurrent :type Boolean) (LengthMultiplier :type Float%20%28single-precision%29))
  (bind _animinstance (Variables|Default|GetAnimInstance))
  (bind _mindicklength (Variables|DickSize|GetMinDickLength))
  (bind _maxdicklength (Variables|DickSize|GetMaxDickLength))
  (if AddToCurrent
    (Variables|DickSize|SetDickLengthMultiplier (Math|Float|Clamp(Float) (+ (Variables|DickSize|GetDickLengthMultiplier) LengthMultiplier) _mindicklength _maxdicklength))
    (else
      (Variables|DickSize|SetDickLengthMultiplier (Math|Float|Clamp(Float) LengthMultiplier _mindicklength _maxdicklength))))
  (Variables|/Game/Models/Samec_D_v1/Samec_Animation_BP.Samec_Animation_BP_C|SetGen2_Legth _animinstance (Math|Vector|Lerp(Vector) "0, 0, 0" "0,-0.150000,1.000000" (Variables|DickSize|GetDickLengthMultiplier)))
  (Variables|/Game/Models/Samec_D_v1/Samec_Animation_BP.Samec_Animation_BP_C|SetGen3_Legth _animinstance (Math|Vector|Lerp(Vector) "0, 0, 0" "0,-0.350000,1.000000" (Variables|DickSize|GetDickLengthMultiplier)))
  (Variables|/Game/Models/Samec_D_v1/Samec_Animation_BP.Samec_Animation_BP_C|SetGen4_Legth _animinstance (Math|Vector|Lerp(Vector) "0, 0, 0" "0,-0.550000,1.000000" (Variables|DickSize|GetDickLengthMultiplier)))
  (Variables|/Game/Models/Samec_D_v1/Samec_Animation_BP.Samec_Animation_BP_C|SetGen5_Legth _animinstance (Math|Vector|Lerp(Vector) "0, 0, 0" "0,-0.700000,1.000000" (Variables|DickSize|GetDickLengthMultiplier)))
  (ShadowCopy|SetShadowCopyDickLength (Math|Vector|Lerp(Vector) "0, 0, 0" "0,-0.150000,1.000000" (Variables|DickSize|GetDickLengthMultiplier)) (Math|Vector|Lerp(Vector) "0, 0, 0" "0,-0.350000,1.000000" (Variables|DickSize|GetDickLengthMultiplier)) (Math|Vector|Lerp(Vector) "0, 0, 0" "0,-0.550000,1.000000" (Variables|DickSize|GetDickLengthMultiplier)) (Math|Vector|Lerp(Vector) "0, 0, 0" "0,-0.700000,1.000000" (Variables|DickSize|GetDickLengthMultiplier))))

(fn Init
  (Utilities|FlowControl|Sequence
    (:then_0
      (bind _assamec_animation_bp (Utilities|Casting|CastToSamec_Animation_BP (Components|SkeletalMesh|GetAnimInstance (Variables|Default|GetSamec_D_v1))))
      (Variables|Default|SetAnimInstance _assamec_animation_bp)
      ;[1 1 1] INIT SHADOW COPY OF GUY USED FOR DICK CALCULATIONS
      (ShadowCopy|InitShadowCopy))
    (:then_1
      (DickPose|SetDickVeiwDirection (DickPose|GetDickDefaultViewDirection)))
    (:then_2
      (bind (_isfound _objectmanager) (CallFunction|GetObjectManager))
      (if _isfound
        (Variables|Default|SetObjectManager _objectmanager)
        (else
          (Development|PrintString "ERROR: OBJECT MANAGER NOT FOUND IN GUY_CHAR" true true "(R=1.000000,G=0.101476,B=0.000000,A=1.000000)" 15.0))))
    (:then_3
      (CallFunction|ManageCensorVersion))
    (:then_4
      (EventDispatchers|BindEventtoEDonISSuckingTick (Variables|Default|GetObjectManager) (EventDispatchers|CreateEvent :!event OnISSuckingTick))
      (EventDispatchers|BindEventtoEDonNOTIsSuckingTick (Variables|Default|GetObjectManager) (EventDispatchers|CreateEvent :!event OnNOTSuckingTick))
      (EventDispatchers|BindEventtoEDonIsSuckingChanged (Variables|Default|GetObjectManager) (EventDispatchers|CreateEvent :!event OnIsSuckingChanged)))))

(fn GetDickDefaultViewDirection
  (return (+ (* (Math|Vector|GetForwardVector (Transformation|GetActorRotation)) 40) (Transformation|GetSocketLocation (Variables|Default|GetSamec_D_v1) "Gen1"))))

(fn SetDickVeiwDirection
  (params (Location%20To%20Look%20At :type Vector))
  (Variables|/Game/Models/Samec_D_v1/Samec_Animation_BP.Samec_Animation_BP_C|SetTestDickLocation (Variables|Default|GetAnimInstance) Location%20To%20Look%20At)
  (Variables|/Game/Models/Samec_D_v1/Samec_Animation_BP.Samec_Animation_BP_C|SetTestDickRotation (Variables|Default|GetAnimInstance) (Math|Rotator|MakeRotator (+ (* (.Pitch (Math|Rotator|BreakRotator (Math|Rotator|FindLookatRotation (Transformation|GetSocketLocation (Variables|Default|GetSamec_D_v1) "Gen1") Location%20To%20Look%20At))) -1.0) 98.0) 0.0 -9e+01)))

(fn GetDickViewDirectionatMouth
  (bind _samec_d_v1 (Variables|Default|GetSamec_D_v1))
  (bind _objectmanager (Variables|Default|GetObjectManager))
  (bind _returnvalue (Transformation|GetSocketLocation _samec_d_v1 "Gen1"))
  (bind _transform (Default|OMGetPActorSocketTransform _objectmanager "NewEnumerator0" "headSocket" "RTS_World"))
  (bind _location (Math|Transform|BreakTransform _transform))
  (return (+ (* (Math|Vector|GetForwardVector (Math|Rotator|FindLookatRotation (+ _returnvalue (* (Math|Vector|GetForwardVector (Math|Rotator|FindLookatRotation _returnvalue (Transformation|GetSocketLocation _samec_d_v1 "Gen6"))) -20)) _location)) 50) _location)))

(fn GetDickViewDirection
  (return (Variables|/Game/Models/Samec_D_v1/Samec_Animation_BP.Samec_Animation_BP_C|GetTestDickLocation (Variables|Default|GetAnimInstance))))

(fn OnDickPartBeginOverlap
  (params (OverlappedComponent :type Primitive%20Component%20Object%20Reference) (OtherComponent :type Primitive%20Component%20Object%20Reference))
  (if (Utilities|Array|ContainsItem (Variables|/Script/Engine.ActorComponent|GetComponentTags OtherComponent) "Throat")
    (DickPose|HideDickPart (Transformation|GetAttachSocketName OverlappedComponent))))

(fn HideDickPart
  (params (DickBoneName :type Name))
  (bind _animinstance (Variables|Default|GetAnimInstance))
  (switch name DickBoneName
    (:Gen2
      (Variables|/Game/Models/Samec_D_v1/Samec_Animation_BP.Samec_Animation_BP_C|SetGen2Scale _animinstance "0, 0, 0"))
    (:Gen3
      (Variables|/Game/Models/Samec_D_v1/Samec_Animation_BP.Samec_Animation_BP_C|SetGen3Scale _animinstance "0, 0, 0"))
    (:Gen4
      (Variables|/Game/Models/Samec_D_v1/Samec_Animation_BP.Samec_Animation_BP_C|SetGen4Scale _animinstance "0, 0, 0"))
    (:Gen5
      (Variables|/Game/Models/Samec_D_v1/Samec_Animation_BP.Samec_Animation_BP_C|SetGen5Scale _animinstance "0, 0, 0"))
    (:Gen6
      (Variables|/Game/Models/Samec_D_v1/Samec_Animation_BP.Samec_Animation_BP_C|SetGen6Scale _animinstance "0, 0, 0"))))

(fn RevealDickPart
  (params (DickBoneName :type Name))
  (bind _animinstance (Variables|Default|GetAnimInstance))
  (bind _dickscale (Variables|DickSize|GetDickScale))
  (bind _returnvalue (Math|Conversions|ToVector(Float) _dickscale))
  (switch name DickBoneName
    (:Gen2
      (Variables|/Game/Models/Samec_D_v1/Samec_Animation_BP.Samec_Animation_BP_C|SetGen2Scale _animinstance _returnvalue))
    (:Gen3
      (Variables|/Game/Models/Samec_D_v1/Samec_Animation_BP.Samec_Animation_BP_C|SetGen3Scale _animinstance _returnvalue))
    (:Gen4
      (Variables|/Game/Models/Samec_D_v1/Samec_Animation_BP.Samec_Animation_BP_C|SetGen4Scale _animinstance _returnvalue))
    (:Gen5
      (Variables|/Game/Models/Samec_D_v1/Samec_Animation_BP.Samec_Animation_BP_C|SetGen5Scale _animinstance _returnvalue))
    (:Gen6
      (Variables|/Game/Models/Samec_D_v1/Samec_Animation_BP.Samec_Animation_BP_C|SetGen6Scale _animinstance _returnvalue))))

(fn OnDickPartEndOverlap
  (params (OvelappedComponent :type Primitive%20Component%20Object%20Reference) (OtherComponent :type Primitive%20Component%20Object%20Reference))
  (if (Utilities|Array|ContainsItem (Variables|/Script/Engine.ActorComponent|GetComponentTags OtherComponent) "Throat")
    (DickPose|RevealDickPart (Transformation|GetAttachSocketName OvelappedComponent))))

(fn OnDickHeadBeginOverlap
  (params (OverlapedComponent :type Primitive%20Component%20Object%20Reference) (OtherComponent :type Primitive%20Component%20Object%20Reference))
  (if (Utilities|Array|ContainsItem (Variables|/Script/Engine.ActorComponent|GetComponentTags OtherComponent) "Mouth")
    (Variables|Default|SetIsDickAttachedToMouth true)
    (CallFunction|SamecAttachDicktoMouth)))

(fn OnDickHeadEndOverlap
  (params (OverlapedComponent :type Primitive%20Component%20Object%20Reference) (OtherComponent :type Primitive%20Component%20Object%20Reference))
  (if (Utilities|Array|ContainsItem (Variables|/Script/Engine.ActorComponent|GetComponentTags OtherComponent) "Mouth")
    (if (not (Class|PrimitiveComponent|IsOverlappingComponent OtherComponent (Variables|Default|GetDickTree)))
      (Variables|Default|SetIsDickAttachedToMouth false)
      (CallFunction|SamecDetachDickfromMouth))))

(fn OnDickTreeBeginOverlap
  (params (OverlappedComponent :type Primitive%20Component%20Object%20Reference) (OtherComponent :type Primitive%20Component%20Object%20Reference))
  (if (Utilities|Array|ContainsItem (Variables|/Script/Engine.ActorComponent|GetComponentTags OtherComponent) "Mouth")
    (Variables|Default|SetIsDickAttachedToMouth true)
    (CallFunction|SamecAttachDicktoMouth)))

(fn OnDickTreeEndOverlap
  (params (OverlappedComponent :type Primitive%20Component%20Object%20Reference) (OtherComponent :type Primitive%20Component%20Object%20Reference)))

(fn ApplyPositiontoLeftHand
  (params (Location :type Vector))
  (Variables|/Game/Models/Samec_D_v1/Samec_Animation_BP.Samec_Animation_BP_C|SetLeftHandPosition (Variables|Default|GetAnimInstance) Location))

(fn GetSamkaHandSocketLocation
  (return (.Location (Math|Transform|BreakTransform (Default|OMGetPActorSocketTransform (Variables|Default|GetObjectManager) "NewEnumerator0" "headHandleSocket" "RTS_World")))))

(fn SetLeftHandPositiontoSamkaHead
  (LeftHandPose|ApplyPositiontoLeftHand (LeftHandPose|GetSamkaHandSocketLocation)))

(fn SetDickScale
  (params (AddToCurrent :type Boolean) (NewScale :type Float%20%28single-precision%29))
  (bind _animinstance (Variables|Default|GetAnimInstance))
  (if AddToCurrent
    (Variables|DickSize|SetDickScale (Math|Float|Clamp(Float) (+ NewScale (Variables|DickSize|GetDickScale)) (Variables|DickSize|GetMinDickScale) (Variables|DickSize|GetMaxDickScale)))
    (else
      (Variables|DickSize|SetDickScale (Math|Float|Clamp(Float) NewScale (Variables|DickSize|GetMinDickScale) (Variables|DickSize|GetMaxDickScale)))))
  (if (DickPose|IsDickPartHidden "Gen1")
    _
    (else
      (Variables|/Game/Models/Samec_D_v1/Samec_Animation_BP.Samec_Animation_BP_C|SetGen1Scale _animinstance (Math|Vector|MakeVector (Variables|DickSize|GetDickScale) (Variables|DickSize|GetDickScale) (Variables|DickSize|GetDickScale)))
      (if (DickPose|IsDickPartHidden "Gen2")
        _
        (else
          (Variables|/Game/Models/Samec_D_v1/Samec_Animation_BP.Samec_Animation_BP_C|SetGen2Scale _animinstance (Math|Vector|MakeVector (Variables|DickSize|GetDickScale) (Variables|DickSize|GetDickScale) (Variables|DickSize|GetDickScale)))
          (if (DickPose|IsDickPartHidden "Gen3")
            _
            (else
              (Variables|/Game/Models/Samec_D_v1/Samec_Animation_BP.Samec_Animation_BP_C|SetGen3Scale _animinstance (Math|Vector|MakeVector (Variables|DickSize|GetDickScale) (Variables|DickSize|GetDickScale) (Variables|DickSize|GetDickScale)))
              (if (DickPose|IsDickPartHidden "Gen4")
                _
                (else
                  (Variables|/Game/Models/Samec_D_v1/Samec_Animation_BP.Samec_Animation_BP_C|SetGen4Scale _animinstance (Math|Vector|MakeVector (Variables|DickSize|GetDickScale) (Variables|DickSize|GetDickScale) (Variables|DickSize|GetDickScale)))
                  (if (DickPose|IsDickPartHidden "Gen5")
                    _
                    (else
                      (Variables|/Game/Models/Samec_D_v1/Samec_Animation_BP.Samec_Animation_BP_C|SetGen5Scale _animinstance (Math|Vector|MakeVector (Variables|DickSize|GetDickScale) (Variables|DickSize|GetDickScale) (Variables|DickSize|GetDickScale)))
                      (if (DickPose|IsDickPartHidden "Gen6")
                        _
                        (else
                          (Variables|/Game/Models/Samec_D_v1/Samec_Animation_BP.Samec_Animation_BP_C|SetGen6Scale _animinstance (Math|Vector|MakeVector (Variables|DickSize|GetDickScale) (Variables|DickSize|GetDickScale) (Variables|DickSize|GetDickScale)))))))))))))))
  (ShadowCopy|SetShadowCopyDickScale (Math|Vector|MakeVector (Variables|DickSize|GetDickScale) (Variables|DickSize|GetDickScale) (Variables|DickSize|GetDickScale)) (Math|Vector|MakeVector (Variables|DickSize|GetDickScale) (Variables|DickSize|GetDickScale) (Variables|DickSize|GetDickScale)) (Math|Vector|MakeVector (Variables|DickSize|GetDickScale) (Variables|DickSize|GetDickScale) (Variables|DickSize|GetDickScale)) (Math|Vector|MakeVector (Variables|DickSize|GetDickScale) (Variables|DickSize|GetDickScale) (Variables|DickSize|GetDickScale)) (Math|Vector|MakeVector (Variables|DickSize|GetDickScale) (Variables|DickSize|GetDickScale) (Variables|DickSize|GetDickScale)) (Math|Vector|MakeVector (Variables|DickSize|GetDickScale) (Variables|DickSize|GetDickScale) (Variables|DickSize|GetDickScale))))

(fn SetShadowCopyDickViewDirection
  (Variables|/Game/Models/Samec_D_v1/Samec_Animation_BP.Samec_Animation_BP_C|SetTestDickLocation (Variables|ShadowCopy|GetShadowCopyAnimInstance) (+ (* (Math|Vector|GetForwardVector (Transformation|GetActorRotation)) 40) (Transformation|GetSocketLocation (Variables|Default|GetShadowSamec) "Gen1"))))

(fn InitShadowCopy
  (bind _assamec_animation_bp (Utilities|Casting|CastToSamec_Animation_BP (Components|SkeletalMesh|GetAnimInstance (Variables|Default|GetShadowSamec))))
  (bind _output_get (Variables|ShadowCopy|SetShadowCopyAnimInstance _assamec_animation_bp))
  (ShadowCopy|SetShadowCopyDickViewDirection)
  (Variables|/Game/Models/Samec_D_v1/Samec_Animation_BP.Samec_Animation_BP_C|SetIsShadowCopy _output_get true))

(fn SetShadowCopyDickLength
  (params (Gen2 :type Vector) (Gen3 :type Vector) (Gen4 :type Vector) (Gen5 :type Vector))
  (bind _shadowcopyaniminstance (Variables|ShadowCopy|GetShadowCopyAnimInstance))
  (Variables|/Game/Models/Samec_D_v1/Samec_Animation_BP.Samec_Animation_BP_C|SetGen2_Legth _shadowcopyaniminstance Gen2)
  (Variables|/Game/Models/Samec_D_v1/Samec_Animation_BP.Samec_Animation_BP_C|SetGen3_Legth _shadowcopyaniminstance Gen3)
  (Variables|/Game/Models/Samec_D_v1/Samec_Animation_BP.Samec_Animation_BP_C|SetGen4_Legth _shadowcopyaniminstance Gen4)
  (Variables|/Game/Models/Samec_D_v1/Samec_Animation_BP.Samec_Animation_BP_C|SetGen5_Legth _shadowcopyaniminstance Gen5))

(fn SetShadowCopyDickScale
  (params (Gen1 :type Vector) (Gen2 :type Vector) (Gen3 :type Vector) (Gen4 :type Vector) (Gen5 :type Vector) (Gen6 :type Vector))
  (bind _shadowcopyaniminstance (Variables|ShadowCopy|GetShadowCopyAnimInstance))
  (Variables|/Game/Models/Samec_D_v1/Samec_Animation_BP.Samec_Animation_BP_C|SetGen1Scale _shadowcopyaniminstance Gen1)
  (Variables|/Game/Models/Samec_D_v1/Samec_Animation_BP.Samec_Animation_BP_C|SetGen2Scale _shadowcopyaniminstance Gen2)
  (Variables|/Game/Models/Samec_D_v1/Samec_Animation_BP.Samec_Animation_BP_C|SetGen3Scale _shadowcopyaniminstance Gen3)
  (Variables|/Game/Models/Samec_D_v1/Samec_Animation_BP.Samec_Animation_BP_C|SetGen4Scale _shadowcopyaniminstance Gen4)
  (Variables|/Game/Models/Samec_D_v1/Samec_Animation_BP.Samec_Animation_BP_C|SetGen5Scale _shadowcopyaniminstance Gen5)
  (Variables|/Game/Models/Samec_D_v1/Samec_Animation_BP.Samec_Animation_BP_C|SetGen6Scale _shadowcopyaniminstance Gen6))

(fn GetDickLength
  (bind _shadowsamec (Variables|Default|GetShadowSamec))
  (return (Math|Vector|VectorLength (- (Transformation|GetSocketLocation _shadowsamec "Gen1") (Transformation|GetSocketLocation _shadowsamec "Gen6")))))

(fn CalculateandSetErection
  (bind _objectmanager (Variables|Default|GetObjectManager))
  (Variables|Erection|SetErectionLevel (+ (Variables|Erection|GetErectionLevel) (/ (Variables|Erection|GetErectionSpeedPerSecond) (/ 1.0 (Utilities|Time|GetWorldDeltaSeconds)))))
  (Default|OMSetDickLength _objectmanager false false (Math|Float|Lerp (Variables|Erection|GetUnerectedDickLength) (Variables|Erection|GetErectedDickLength) (Variables|Erection|GetErectionLevel)))
  (Default|OMSetDickScale _objectmanager false false (Math|Float|Lerp (Variables|Erection|GetUnerectedDickSize) (Variables|Erection|GetErectedDickSize) (Variables|Erection|GetErectionLevel)))
  (if (>= (Variables|Erection|GetErectionLevel) 1.0)
    (Variables|Erection|SetErectionLevel 1.0)
    (Default|OMSetDickLength _objectmanager false false (Math|Float|Lerp (Variables|Erection|GetUnerectedDickLength) (Variables|Erection|GetErectedDickLength) (Variables|Erection|GetErectionLevel)))
    (Default|OMSetDickScale _objectmanager false false (Math|Float|Lerp (Variables|Erection|GetUnerectedDickSize) (Variables|Erection|GetErectedDickSize) (Variables|Erection|GetErectionLevel)))
    (return true)
    (else
      (return false))))

(fn IsDickPartHidden
  (params (Dick%20Part :type Name))
  (bind _animinstance (Variables|Default|GetAnimInstance))
  (switch name Dick%20Part
    (:Gen1
      (LocalVariables|SetScale (Variables|/Game/Models/Samec_D_v1/Samec_Animation_BP.Samec_Animation_BP_C|GetGen1Scale _animinstance)))
    (:Gen2
      (LocalVariables|SetScale (Variables|/Game/Models/Samec_D_v1/Samec_Animation_BP.Samec_Animation_BP_C|GetGen2Scale _animinstance)))
    (:Gen3
      (LocalVariables|SetScale (Variables|/Game/Models/Samec_D_v1/Samec_Animation_BP.Samec_Animation_BP_C|GetGen3Scale _animinstance)))
    (:Gen4
      (LocalVariables|SetScale (Variables|/Game/Models/Samec_D_v1/Samec_Animation_BP.Samec_Animation_BP_C|GetGen4Scale _animinstance)))
    (:Gen5
      (LocalVariables|SetScale (Variables|/Game/Models/Samec_D_v1/Samec_Animation_BP.Samec_Animation_BP_C|GetGen5Scale _animinstance)))
    (:Gen6
      (LocalVariables|SetScale (Variables|/Game/Models/Samec_D_v1/Samec_Animation_BP.Samec_Animation_BP_C|GetGen6Scale _animinstance))))
  (return (Math|Vector|Equal(Vector) (LocalVariables|GetScale) "0, 0, 0" 0.0001)))

(fn SetProlongedHand
  (params (IsProlonged :type Boolean))
  (Variables|/Game/Models/Samec_D_v1/Samec_Animation_BP.Samec_Animation_BP_C|SetIsProlongHand (Variables|Default|GetAnimInstance) IsProlonged))

(fn OnISSuckingTick)

(fn OnNOTSuckingTick
  (bind _objectmanager (Variables|Default|GetObjectManager))
  (bind _gen6toheaddistance (Variables|/Game/Blueprints/Managers/ObjectsManager.ObjectsManager_C|GetGen6ToHeadDistance _objectmanager))
  (if (<= _gen6toheaddistance 3.0)
    (CallFunction|SamecEEE (Math|Float|NormalizetoRange _gen6toheaddistance 0.15 3.0))))

(fn OnIsSuckingChanged
  (params (IsSucking :type Boolean))
  (if IsSucking
    (CallFunction|SamecAttachDicktoMouth)
    (else
      (CallFunction|SamecDetachDickfromMouth))))

(fn SetLeftHandPosition
  (params (InputX :type Float%20%28single-precision%29) (InputY :type Float%20%28single-precision%29) (IsSetManually :type Boolean))
  (bind _animinstance (Variables|Default|GetAnimInstance))
  (bind _returnvalue (Class|KismetMathLibrary|FloatSpringInterp (Variables|Default|GetLeftHandX) (Variables|Default|GetTargetLeftHandX) (Variables|Default|GetSpring1) 0.1 1.0 (Utilities|Time|GetWorldDeltaSeconds) 0.01))
  (Variables|Default|SetLeftHandX _returnvalue)
  (bind _returnvalue_2 (Class|KismetMathLibrary|FloatSpringInterp (Variables|Default|GetLeftHandY) (Variables|Default|GetTargetLeftHandY) (Variables|Default|GetSpring2) 0.1 1.0 (Utilities|Time|GetWorldDeltaSeconds) 0.01))
  (Variables|Default|SetLeftHandY _returnvalue_2)
  (bind _lefthandposition (CallFunction|CalculateLeftHandPositionbyXYVariables))
  (Variables|Default|SetLeftHandPosition _lefthandposition)
  (if (<= (CallFunction|GetDistance (.Location (Math|Transform|BreakTransform (Default|OMGetPActorSocketTransform (Variables|Default|GetObjectManager) "NewEnumerator0" "headHandleSocket" "RTS_World"))) (Variables|Default|GetLeftHandPosition)) 6.0)
    (Variables|Default|SetIsHoldingHead true)
    (Variables|/Game/Models/Samec_D_v1/Samec_Animation_BP.Samec_Animation_BP_C|SetIsLeftHandRelaxed _animinstance false)
    (else
      (Variables|/Game/Models/Samec_D_v1/Samec_Animation_BP.Samec_Animation_BP_C|SetIsLeftHandRelaxed _animinstance true))))

(fn CalculateLeftHandPositionbyXYVariables
  (bind _constdefaultlefthandposition (Variables|Default|GetConstDefaultLeftHandPosition))
  (bind (_x _y _z) (Math|Vector|BreakVector _constdefaultlefthandposition))
  (return (Math|Vector|MakeVector (+ _x (Variables|Default|GetLeftHandX)) _y (+ _z (Variables|Default|GetLeftHandY)))))

(fn ReceiveLeftHandInput
  (params (X :type Float%20%28single-precision%29) (Y :type Float%20%28single-precision%29) (IsManual :type Boolean) (IsSkipInterpolation :type Boolean))
  (if IsManual
    (Variables|Default|SetTargetLeftHandX (Math|Float|Clamp(Float) X (Variables|Default|GetMinLeftHandX) (Variables|Default|GetMaxLeftHandX)))
    (Variables|Default|SetTargetLeftHandY (Math|Float|Clamp(Float) Y (Variables|Default|GetMinLeftHandY) (Variables|Default|GetMaxLeftHandY)))
    (if IsSkipInterpolation
      _)
    (elif (!= X 0.0)
      (Variables|Default|SetTargetLeftHandX (Math|Float|Clamp(Float) (+ (Variables|Default|GetTargetLeftHandX) X) (Variables|Default|GetMinLeftHandX) (Variables|Default|GetMaxLeftHandX)))
      (else
        (Variables|Default|SetTargetLeftHandY (Math|Float|Clamp(Float) (+ Y (Variables|Default|GetTargetLeftHandY)) (Variables|Default|GetMinLeftHandY) (Variables|Default|GetMaxLeftHandY)))))))