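; AudioActor is a sound-emitting actor that plays single sounds, random picks from named sound arrays, or a simple looping sound.
; Non-forced requests play only if their importance matches or beats the current sound, which fades out first.
; On BeginPlay it binds to SoundManager's Characters, Ambient and Music volume delegates, initially setting volume to master times channel volume.
; A stereo flag drives spatialization; RandomizeAudio is an unfinished stub.
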(event OnAudioFinished(Audio)
  (Variables|Default|SetIsSoundPlayingNow false)
  (if (Variables|Default|GetIsSimpleSoundLoop)
    (Audio|Components|Audio|Play (Variables|Default|GetAudio) 0.0)))

(event Custom|AA_PlaySound
  (params (Sound :type Sound%20Struct%20Structure) (Play%20NOW :type Boolean))
  (bind _fadeoutdefaultduration (Variables|Default|GetFadeOutDefaultDuration))
  (if Play%20NOW
    (CallFunction|PlaySoundNow Sound :!label _label)
    (else
      (bind _ismoreimportant (CallFunction|PlaySoundbyImportance Sound))
      (if _ismoreimportant
        (if (Variables|Default|GetIsSoundPlayingNow)
          (Audio|Components|Audio|FadeOut (Variables|Default|GetAudio) _fadeoutdefaultduration 0.0 :!class /Script/Engine.AudioComponent)
          (Utilities|FlowControl|Delay _fadeoutdefaultduration)
          (goto _label)
          (else
            (goto _label)))))))

(event EventBeginPlay
  (CallFunction|Init))

(event Collision|EventActorBeginOverlap
  (params (OtherActor :type Actor%20Object%20Reference)))

(event EventTick
  (params (DeltaSeconds :type Float%20%28single-precision%29)))

(fn ConstructionScript
  (Variables|/Script/Engine.AudioComponent|SetbAllowSpatialization (Variables|Default|GetAudio) (Variables|Default|GetIsStereo)))

(fn AAPlayRandomSoundfromAudioStruct
  (params (StructName :type Name))
  (bind (_isfound _soundarray) (CallFunction|FindAudioStructArraybyName StructName))
  (if _isfound
    (CallFunction|AAPlaySound (Utilities|Array|Get(acopy) _soundarray (Math|Random|RandomIntegerinRange 0 (- (Utilities|Array|Length _soundarray) 1))) false)))

(fn PlaySoundbyImportance
  (params (SoundStruct :type Sound%20Struct%20Structure))
  (if (Variables|Default|GetIsSoundPlayingNow)
    (return (>= (.Importance (Utilities|Struct|BreakSoundStruct SoundStruct)) (.Importance (Utilities|Struct|BreakSoundStruct (Variables|Default|GetSoundPlayingNowStruct)))))
    (else
      (return true))))

(fn PlaySoundNow
  (params (Sound :type Sound%20Struct%20Structure))
  (bind _audio (Variables|Default|GetAudio))
  (Audio|Components|Audio|SetSound _audio (.SoundBase (Utilities|Struct|BreakSoundStruct Sound)))
  (Audio|Components|Audio|Play _audio 0.0)
  (Variables|Default|SetIsSoundPlayingNow true)
  (Variables|Default|SetSoundPlayingNowStruct Sound))

(fn RandomizeAudio
  (params (StructName :type Name) (SoundStructArray :type Array%20of%20Sound%20Struct%20Structures))
  (bind _output_get (LocalVariables|SetSoundStructArray_Local (.SoundArray (CallFunction|FindAudioStructArraybyName StructName))))
  (if (Variables|Default|GetIsHumanizeRandom)
    _))

(fn FindAudioStructArraybyName
  (params (Name :type Name))
  (bind _array_element (Utilities|Array|ForEachLoopwithBreak (Variables|Default|GetAudioStructsArray) :!label _label)
    (:LoopBody
      (if (Utilities|Name|Equal(Name) Name (.SoundArrayName (Utilities|Struct|BreakAudioArrayStruct _array_element)))
        (goto _label Break)))
    (:Completed
      (return (Utilities|Name|Equal(Name) Name (.SoundArrayName (Utilities|Struct|BreakAudioArrayStruct _array_element))) (.SoundsArray (Utilities|Struct|BreakAudioArrayStruct _array_element))))))

(fn OnMasterVolumeChanged
  (params (NewMasterVolume :type Float%20%28single-precision%29))
  (Audio|Components|Audio|SetVolumeMultiplier (Variables|Default|GetAudio) NewMasterVolume :!class /Script/Engine.AudioComponent))

(fn OnCharactersVolumeChanged
  (params (NewVolume :type Float%20%28single-precision%29))
  (if (Utilities|Enum|Equal(Enum) (Variables|Default|GetSoundChannel) "NewEnumerator0")
    (Audio|Components|Audio|SetVolumeMultiplier (Variables|Default|GetAudio) NewVolume :!class /Script/Engine.AudioComponent)))

(fn OnAmbientVolumeChanged
  (params (NewVolume :type Float%20%28single-precision%29))
  (if (Utilities|Enum|Equal(Enum) (Variables|Default|GetSoundChannel) "NewEnumerator1")
    (Audio|Components|Audio|SetVolumeMultiplier (Variables|Default|GetAudio) NewVolume :!class /Script/Engine.AudioComponent)))

(fn OnMusicVolumeChanged
  (params (NewVolume :type Float%20%28single-precision%29))
  (if (Utilities|Enum|Equal(Enum) (Variables|Default|GetSoundChannel) "NewEnumerator2")
    (Audio|Components|Audio|SetVolumeMultiplier (Variables|Default|GetAudio) NewVolume :!class /Script/Engine.AudioComponent)))

(fn SetStereo
  (params (IsStereo :type Boolean))
  (bind _output_get (Variables|Default|SetIsStereo IsStereo))
  (Variables|/Script/Engine.AudioComponent|SetbAllowSpatialization (Variables|Default|GetAudio) _output_get))

(fn SetSoundChannel
  (params (SoundChannel :type SoundChannels_ENum%20Enum :default "NewEnumerator0"))
  (Variables|Default|SetSoundChannel SoundChannel)
  (CallFunction|SetupAudioChannelSettings))

(fn SetupAudioChannelSettings
  (bind _soundmanager (Variables|Default|GetSoundManager))
  (bind _mastervolume (Variables|/Game/Blueprints/Managers/SoundManager_BP.SoundManager_BP_C|GetMasterVolume _soundmanager))
  (Utilities|IsValid _soundmanager
    (:Is%20Valid
      (switch Utilities|FlowControl|Switch|SwitchonSoundChannels_ENum (Variables|Default|GetSoundChannel)
        (:NewEnumerator0
          (CallFunction|OnCharactersVolumeChanged (* _mastervolume (Variables|/Game/Blueprints/Managers/SoundManager_BP.SoundManager_BP_C|GetCharactersVolume _soundmanager))))
        (:NewEnumerator1
          (CallFunction|OnAmbientVolumeChanged (* _mastervolume (Variables|/Game/Blueprints/Managers/SoundManager_BP.SoundManager_BP_C|GetAmbientVolume _soundmanager))))
        (:NewEnumerator2
          (CallFunction|OnMusicVolumeChanged (* _mastervolume (Variables|/Game/Blueprints/Managers/SoundManager_BP.SoundManager_BP_C|GetMusicVolume _soundmanager))))))))

(fn Init
  (bind _audio (Variables|Default|GetAudio))
  (bind (_issuccess _assound_manager_bp) (CallFunction|GetSoundManager))
  (if _issuccess
    (bind _output_get (Variables|Default|SetSoundManager _assound_manager_bp))
    (Utilities|FlowControl|Sequence
      (:then_0
        (EventDispatchers|BindEventtoSoundManageronCharactersVolumeChangedDelegate _output_get (EventDispatchers|CreateEvent :!event OnCharactersVolumeChanged)))
      (:then_1
        (EventDispatchers|BindEventtoSoundManageronAmbientVolumeChangedDelegate _output_get (EventDispatchers|CreateEvent :!event OnAmbientVolumeChanged)))
      (:then_2
        (EventDispatchers|BindEventtoSoundManageronMusicVolumeChangedDelegate _output_get (EventDispatchers|CreateEvent :!event OnMusicVolumeChanged)))
      (:then_3
        (CallFunction|SetupAudioChannelSettings)
        (if (Variables|Default|GetIsSimpleSoundLoop)
          (Audio|Components|Audio|SetSound _audio (Variables|Default|GetSoundForSimpleLoop))
          (Audio|Components|Audio|Play _audio 0.0))))))