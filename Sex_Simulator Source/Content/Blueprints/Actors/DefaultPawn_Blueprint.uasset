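; Player pawn for an adult game, routing mouse, keyboard and VR grip input to the male and female character actors and ObjectManager.
; Q and W switch between the free camera, male POV and female POV with a fade, while the wheel steps a timeline-smoothed, clamped zoom.
; Hotkeys drive character actions, look-at targets and blink rates.
; Gripping near the female's head maps controller distance to her normalized hip angle each tick.
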(event Custom|SetCameraZoom
  (params (Zoom :type Float%20%28single-precision%29))
  (Variables|Default|SetCameraZoom Zoom))

(event EventBeginPlay
  (Utilities|FlowControl|Sequence
    (:then_0
      (Variables|Default|SetSamkaSkeletal (Variables|/Game/Blueprints/Actors/Samka_BP.Samka_BP_C|GetSamkaSkeletalMesh (Variables|/Game/Blueprints/Managers/ObjectsManager.ObjectsManager_C|GetSamkaActor (Variables|Default|GetObjectManager))))
      (Variables|Default|SetCameraNewLocation (Transformation|GetActorLocation)))
    (:then_1
      (Default|OMSetPlayerCamera (Variables|Default|GetObjectManager) self))))

(event Collision|EventActorBeginOverlap
  (params (OtherActor :type Actor%20Object%20Reference)))

(event EventTick
  (params (DeltaSeconds :type Float%20%28single-precision%29))
  (bind _staticmesh (Variables|Default|GetStaticMesh))
  (bind _test1 (Variables|Default|GetTest1))
  (bind _returnvalue (Transformation|GetWorldLocation _staticmesh))
  (bind _distance (CallFunction|GetDistance _returnvalue _test1))
  (bind _returnvalue_2 (Math|Float|Clamp(Float) _distance 0.0 3e+01))
  (bind _returnvalue_3 (Math|Float|NormalizetoRange _returnvalue_2 0.0 3e+01))
  (if (Variables|Default|GetIsVRGrip)
    (Development|PrintString (Utilities|String|ToString(Float) _returnvalue_3))
    (Default|SetNormalizedHipAngle (Variables|Default|GetSamkaActor) false _returnvalue_3 false)))

(event Input|AxisEvents|InputAxisCameraPitch
  (params (AxisValue :type Float%20%28single-precision%29))
  (bind _returnvalue (* AxisValue 1.0))
  (bind _samecactor (Variables|Default|GetSamecActor))
  (if (Variables|Default|GetIsMPOV)
    (Default|EGInputX _samecactor _returnvalue)
    (else
      (Default|EGInputY _samecactor _returnvalue))))

(event Input|AxisEvents|InputAxisCameraYaw
  (params (AxisValue :type Float%20%28single-precision%29))
  (if (not (Variables|Default|GetIsMPOV))
    (if (!= AxisValue 0.0)
      (Default|EGInputX (Variables|Default|GetSamecActor) (* AxisValue 0.7)))))

(event Input|MouseEvents|MouseWheelUp
  (params (Key :type Key%20Structure))
  (:Pressed
    (if (not (Variables|Default|GetIsMPOV))
      (if (not (> (+ (Variables|Default|GetCameraZoom) 5.0) 5e+01))
        (Variables|Default|SetCameraZoom (+ (Variables|Default|GetCameraZoom) 5.0))
        (Variables|Default|SetCameraOldLocation (Transformation|GetActorLocation))
        (Variables|Default|SetCameraNewLocation (+ (* (Transformation|GetActorForwardVector) 5.0) (Variables|Default|GetCameraNewLocation)))
        (bind _newtrack_0 (Timeline|Timeline_0 PlayFromStart)
          (:Update
            (Transformation|SetActorLocation (Math|Vector|Lerp(Vector) (Variables|Default|GetCameraOldLocation) (Variables|Default|GetCameraNewLocation) _newtrack_0) false false)))))))

(event Input|KeyboardEvents|R
  (params (Key :type Key%20Structure))
  (:Pressed
    (Default|SetThroatResistance (Variables|Default|GetSamkaActor) 15.0)))

(event Input|KeyboardEvents|D
  (params (Key :type Key%20Structure))
  (:Pressed
    (Variables|/Game/Blueprints/Actors/Samka_BP.Samka_BP_C|SetTestLookAt (Variables|Default|GetSamkaActor) "default")))

(event Input|KeyboardEvents|F
  (params (Key :type Key%20Structure))
  (:Pressed
    (Default|ToggleHandControl (Variables|Default|GetSamkaActor) false false)))

(event Input|KeyboardEvents|H
  (params (Key :type Key%20Structure))
  (:Pressed
    (Default|ToggleHandjob (Variables|Default|GetSamkaActor) false false)))

(event Input|MouseEvents|LeftMouseButton
  (params (Key :type Key%20Structure))
  (bind _samkaactor (Variables|Default|GetSamkaActor))
  (:Pressed
    (Variables|/Game/Blueprints/Actors/Samka_BP.Samka_BP_C|SetIsLMBPressed _samkaactor true))
  (:Released
    (Variables|/Game/Blueprints/Actors/Samka_BP.Samka_BP_C|SetIsLMBPressed _samkaactor false)))

(event Input|KeyboardEvents|Q
  (params (Key :type Key%20Structure))
  (bind _objectmanager (Variables|Default|GetObjectManager))
  (bind _objectmanager_2 (Variables|Default|GetObjectManager))
  (:Pressed
    (CallFunction|Fadein)
    (if (Variables|Default|GetIsMPOV)
      (Default|OMSetPlayerCamera _objectmanager_2 self)
      (Variables|Default|SetIsMPOV false)
      (else
        (Default|OMSetPlayerCamera _objectmanager_2 (Variables|Default|GetSamecActor))
        (Variables|Default|SetIsMPOV true)
        (if (Variables|Default|GetIsFPOV)
          (Default|OMSetFemalePOV _objectmanager false)
          (Variables|Default|SetIsFPOV false))))
    (Default|OMSetMalePOV _objectmanager (Variables|Default|GetIsMPOV))
    (Default|SetProlongedHand (Variables|Default|GetSamecActor) true)))

(event Input|KeyboardEvents|W
  (params (Key :type Key%20Structure))
  (bind _samecactor (Variables|Default|GetSamecActor))
  (bind _objectmanager (Variables|Default|GetObjectManager))
  (bind _objectmanager_2 (Variables|Default|GetObjectManager))
  (:Pressed
    (CallFunction|Fadein)
    (if (Variables|Default|GetIsFPOV)
      (Variables|Default|SetIsFPOV false)
      (Default|OMSetPlayerCamera _objectmanager self)
      (Default|SetProlongedHand _samecactor true)
      (Default|OMSetFemalePOV _objectmanager_2 false)
      (else
        (Variables|Default|SetIsFPOV true)
        (Default|OMSetPlayerCamera _objectmanager (Variables|Default|GetSamkaActor))
        (if (Variables|Default|GetIsMPOV)
          (Variables|Default|SetIsMPOV false)
          (Default|OMSetMalePOV _objectmanager_2 false))
        (Default|SetProlongedHand _samecactor false)
        (Default|OMSetFemalePOV _objectmanager_2 true)))))

(event Input|KeyboardEvents|MotionControllerLeftGrip1
  (params (Key :type Key%20Structure)))

(event Input|KeyboardEvents|MotionControllerRightGrip1
  (params (Key :type Key%20Structure))
  (bind _staticmesh (Variables|Default|GetStaticMesh))
  (bind _returnvalue (Transformation|GetWorldLocation _staticmesh))
  (:Pressed
    (if (<= (CallFunction|GetDistance (Transformation|GetSocketLocation (Variables|/Game/Blueprints/Actors/Samka_BP.Samka_BP_C|GetSamka (Variables|Default|GetSamkaActor)) "head") _returnvalue) 3e+01)
      (Variables|Default|SetIsVRGrip true)
      (Variables|Default|SetTest1 _returnvalue)
      (else
        (Variables|Default|SetIsVRGrip false :!label _label))))
  (:Released
    (goto _label)))

(event Input|KeyboardEvents|E
  (params (Key :type Key%20Structure))
  (:Pressed
    (Default|OMCreateSalivaCableEffect (Variables|Default|GetObjectManager) 0 "Gen5")))

(event Input|KeyboardEvents|X
  (params (Key :type Key%20Structure))
  (:Pressed
    (Default|SetBlinksPerMinute (Variables|/Game/Blueprints/Actors/Samka_BP.Samka_BP_C|GetBlinkManager (Variables|Default|GetSamkaActor)) "NewEnumerator0")))

(event Input|KeyboardEvents|C
  (params (Key :type Key%20Structure))
  (:Pressed
    (Default|SetBlinksPerMinute (Variables|/Game/Blueprints/Actors/Samka_BP.Samka_BP_C|GetBlinkManager (Variables|Default|GetSamkaActor)) "NewEnumerator1")))

(event Input|KeyboardEvents|V
  (params (Key :type Key%20Structure))
  (:Pressed
    (Default|SetBlinksPerMinute (Variables|/Game/Blueprints/Actors/Samka_BP.Samka_BP_C|GetBlinkManager (Variables|Default|GetSamkaActor)) "NewEnumerator2")))

(event Input|KeyboardEvents|B
  (params (Key :type Key%20Structure))
  (:Pressed
    (Default|SetBlinksPerMinute (Variables|/Game/Blueprints/Actors/Samka_BP.Samka_BP_C|GetBlinkManager (Variables|Default|GetSamkaActor)) "NewEnumerator3")))

(event Input|KeyboardEvents|N
  (params (Key :type Key%20Structure))
  (:Pressed
    (Default|SetBlinksPerMinute (Variables|/Game/Blueprints/Actors/Samka_BP.Samka_BP_C|GetBlinkManager (Variables|Default|GetSamkaActor)) "NewEnumerator4" 60)))

(event Input|MouseEvents|MouseWheelDown
  (params (Key :type Key%20Structure))
  (:Pressed
    (if (not (Variables|Default|GetIsMPOV))
      (if (not (< (+ (Variables|Default|GetCameraZoom) -5.0) -4e+01))
        (Variables|Default|SetCameraZoom (+ (Variables|Default|GetCameraZoom) -5.0))
        (Variables|Default|SetCameraOldLocation (Transformation|GetActorLocation))
        (Variables|Default|SetCameraNewLocation (+ (* (Transformation|GetActorForwardVector) -5.0) (Variables|Default|GetCameraNewLocation)))
        (bind _newtrack_0 (Timeline|Timeline_0 PlayFromStart)
          (:Update
            (Transformation|SetActorLocation (Math|Vector|Lerp(Vector) (Variables|Default|GetCameraOldLocation) (Variables|Default|GetCameraNewLocation) _newtrack_0) false false)))))))

(event Input|KeyboardEvents|A
  (params (Key :type Key%20Structure))
  (:Pressed
    (Variables|/Game/Blueprints/Actors/Samka_BP.Samka_BP_C|SetTestLookAt (Variables|Default|GetSamkaActor) "Gen1")))

(event Input|KeyboardEvents|S
  (params (Key :type Key%20Structure))
  (:Pressed
    (Variables|/Game/Blueprints/Actors/Samka_BP.Samka_BP_C|SetTestLookAt (Variables|Default|GetSamkaActor) "head")))

(fn ConstructionScript)