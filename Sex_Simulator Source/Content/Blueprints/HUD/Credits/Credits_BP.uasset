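; Actor that runs the scrolling credits screen, opening the credits widget on BeginPlay and binding its back-to-menu event.
; A timeline moves the credits vertical box's canvas slot up one unit per update.
; When the box's bottom edge rises above an end-position marker in the widget, it tells the widget to restart the credits.
; The back-to-menu event closes the widget and destroys the actor.
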(event EventBeginPlay
  (bind _widget_reference (CallFunction|OpenWidget "/Game/Blueprints/HUD/Credits/Credits_Widget.Credits_Widget_C" true 3))
  (bind _ascredits_widget (Utilities|Casting|CastToCredits_Widget _widget_reference))
  (EventDispatchers|BindEventtoOnBacktoMenuEvent _ascredits_widget (EventDispatchers|CreateEvent :!event OnBacktoMenuEvent))
  (bind _ascanvas_panel_slot (Utilities|Casting|CastToCanvasPanelSlot (Variables|/Script/UMG.Widget|GetSlot (Variables|/Game/Blueprints/HUD/Credits/Credits_Widget.Credits_Widget_C|GetVerticalBox_25 _ascredits_widget))))
  (Timeline|Timeline_0 Play
    (:Update
      (Class|CanvasPanelSlot|SetPosition _ascanvas_panel_slot (Math|Vector2D|MakeVector2D (.X (Math|Vector2D|BreakVector2D (Class|CanvasPanelSlot|GetPosition _ascanvas_panel_slot))) (+ (.Y (Math|Vector2D|BreakVector2D (Class|CanvasPanelSlot|GetPosition _ascanvas_panel_slot))) -1.0)))
      (if (CallFunction|IsCreditsEnded _ascanvas_panel_slot (Class|WidgetLayoutLibrary|SlotasCanvasSlot (Variables|/Game/Blueprints/HUD/Credits/Credits_Widget.Credits_Widget_C|GetCreditsBottomEndPosition _ascredits_widget)))
        (Default|RestartCredits _ascredits_widget)))))

(event Collision|EventActorBeginOverlap
  (params (OtherActor :type Actor%20Object%20Reference)))

(event EventTick
  (params (DeltaSeconds :type Float%20%28single-precision%29)))

(fn ConstructionScript)

(fn OnBacktoMenuEvent
  (CallFunction|CloseWidget "/Game/Blueprints/HUD/Credits/Credits_Widget.Credits_Widget_C")
  (Actor|DestroyActor))

(fn IsCreditsEnded
  (params (Credits :type Canvas%20Panel%20Slot%20Object%20Reference) (EndPositionSlot :type Canvas%20Panel%20Slot%20Object%20Reference))
  (return (> (.Y (Math|Vector2D|BreakVector2D (Class|CanvasPanelSlot|GetPosition EndPositionSlot))) (+ (.Y (Math|Vector2D|BreakVector2D (Class|CanvasPanelSlot|GetSize Credits))) (.Y (Math|Vector2D|BreakVector2D (Class|CanvasPanelSlot|GetPosition Credits)))))))