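; Main menu HUD that opens the MainMenuWidget_BP screen on BeginPlay and keeps a reference to it.
; It shows the mouse cursor, picks UI-only input in standalone game builds or Game and UI otherwise, and caps the frame rate via console command.
; PlayIntro triggers the widget's intro animation, retrying on a short timer until the widget reference is valid.
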(event Custom|PlayIntro
  (CallFunction|PlayIntroMainMenuAnimation))

(event EventBeginPlay
  (bind _returnvalue (Game|GetPlayerController 0))
  (bind _widget_reference (CallFunction|OpenWidget "/Game/Blueprints/HUD/MainMenu/MainMenuWidget_BP.MainMenuWidget_BP_C" true))
  (bind _asmain_menu_widget_bp (Utilities|Casting|CastToMainMenuWidget_BP _widget_reference))
  (bind _output_get (Variables|Default|SetMainMenuWidget _asmain_menu_widget_bp))
  (Variables|/Script/Engine.PlayerController|SetbShowMouseCursor _returnvalue true)
  (if (Class|HnomerBPLibraryPluginBPLibrary|IsStandaloneGameBuild self)
    (Input|SetInputModeUIOnly _returnvalue _output_get "DoNotLock")
    (else
      (Input|SetInputModeGameandUI _returnvalue _output_get "DoNotLock" false)))
  (Development|ExecuteConsoleCommand "t.maxfps 120" _returnvalue))

(event Collision|EventActorBeginOverlap
  (params (OtherActor :type Actor%20Object%20Reference)))

(event EventTick
  (params (DeltaSeconds :type Float%20%28single-precision%29)))

(fn ConstructionScript)

(fn PlayIntroMainMenuAnimation
  (bind _mainmenuwidget (Variables|Default|GetMainMenuWidget))
  (Utilities|IsValid _mainmenuwidget
    (:Is%20Valid
      (Default|PlayIntroAnimation _mainmenuwidget))
    (:Is%20Not%20Valid
      (Utilities|Time|SetTimerbyFunctionName self "PlayIntro_MainMenuAnimation" 0.05))))